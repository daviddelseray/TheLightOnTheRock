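; BP_Sparks is an effect Blueprint that produces intermittent sparks with sound.
; The custom Activation event, not triggered within this graph, loops by calling itself while IsActive is true.
; Each cycle shows the Sparks component and plays Audio, waits for the sound's duration, then hides the sparks and pauses briefly for a random interval before repeating.
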(event Custom|Activation
  (if (Variables|Default|GetisActive)
    (bind _timetowait (CallFunction|Play))
    (Utilities|FlowControl|Delay _timetowait)
    (CallFunction|Stop)
    (Utilities|FlowControl|Delay (Math|Random|RandomFloatinRange 0.2 0.4))
    (CallFunction|Activation)))

(event EventBeginPlay)

(event Collision|EventActorBeginOverlap
  (params (OtherActor :type Actor%20Object%20Reference)))

(event EventTick
  (params (DeltaSeconds :type Float%20%28single-precision%29)))

(fn ConstructionScript)

(fn Play
  (bind _audio (Variables|Default|GetAudio))
  (Rendering|SetVisibility (Variables|Default|GetSparks) true false)
  (Audio|Components|Audio|Play _audio 0.0)
  (return (Variables|/Script/Engine.SoundBase|GetDuration (Variables|/Script/Engine.AudioComponent|GetSound _audio))))

(fn Stop
  (Rendering|SetVisibility (Variables|Default|GetSparks) false false))