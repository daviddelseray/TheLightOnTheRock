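; BP_WoodBurner is an interactable wood burner that accepts a wood log carried by the player.
; On Interact with the door open, it snaps the player's carried BP_WoodLog to LogAttachPoint and clears the character's carry state.
; It then checks BP_LevelManager's day and problem plus its own Location enum for the first day's first problem, currently only printing a confirmation on a match.
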(event EventBeginPlay)

(event Collision|EventActorBeginOverlap
  (params (OtherActor :type Actor%20Object%20Reference)))

(event EventTick
  (params (DeltaSeconds :type Float%20%28single-precision%29)))

(event EventInteract
  ;[1 1 1] Place the wood log into the woodburner
  (if (Variables|/Game/Blueprints/Bluperints/BP_WoodBurnerDoor.BP_WoodBurnerDoor_C|GetisOpen (Variables|Default|GetDoor))
    (bind _asbp_character (Utilities|Casting|CastToBP_Character (Game|GetPlayerCharacter 0)))
    (Utilities|Casting|CastToBP_WoodLog (Variables|/Game/Blueprints/Bluperints/BP_Character.BP_Character_C|GetCarriedObject _asbp_character))
    (Transformation|AttachComponentToComponent (Variables|/Game/Blueprints/Bluperints/BP_Character.BP_Character_C|GetCarriedObject _asbp_character) (Variables|Default|GetLogAttachPoint) "None" "SnapToTarget" "SnapToTarget" "KeepWorld" true)
    ;[1 1 1] Make Player let go the log
    (Variables|/Game/Blueprints/Bluperints/BP_Character.BP_Character_C|SetCaryObject _asbp_character false)
    (Variables|/Game/Blueprints/Bluperints/BP_Character.BP_Character_C|SetCarriedObject _asbp_character 0)
    ;[1 1 1] Solve the first Problem of the First Day
    (bind _outactors (Actor|GetAllActorsOfClass "/Game/Blueprints/Bluperints/BP_LevelManager.BP_LevelManager_C"))
    (if (Math|Boolean|ANDBoolean (== (Variables|/Game/Blueprints/Bluperints/BP_LevelManager.BP_LevelManager_C|GetCurrentDay (Utilities|Array|Get(acopy) _outactors)) 1) (== (Variables|/Game/Blueprints/Bluperints/BP_LevelManager.BP_LevelManager_C|GetCurrentProblem (Utilities|Array|Get(acopy) _outactors)) 0) (Utilities|Enum|Equal(Enum) (Variables|Default|GetLocation) "NewEnumerator0"))
      (Development|PrintString "OK"))))

(fn ConstructionScript)