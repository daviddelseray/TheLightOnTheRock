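; BP_Rat is an interactable rat the player can pick up, carry and throw.
; Grab frees its trap, then kills the player if electrified; otherwise, unless burning, it disables physics, attaches to the character and clears the generator's rat flag if generator-spawned.
; Interact throws the grabbed rat.
; Ablaze marks it electrified and burning and attaches a spawned BP_Flame, while TurnOff clears only the burning state.
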(event EventBeginPlay)

(event Collision|EventActorBeginOverlap
  (params (OtherActor :type Actor%20Object%20Reference)))

(event EventTick
  (params (DeltaSeconds :type Float%20%28single-precision%29)))

(event EventGrab
  (params (Character :type Skeletal%20Mesh%20Component%20Object%20Reference))
  (if (Variables|Default|GetisCaught)
    (Variables|/Game/Blueprints/Bluperints/BP_RatTraps.BP_RatTraps_C|SetisFull (Variables|Default|GetTrap) false))
  (if (Variables|Default|GetisElectrified)
    (bind _asbp_character (Utilities|Casting|CastToBP_Character (Game|GetPlayerCharacter 0)))
    (Default|Death _asbp_character "NewEnumerator0")
    (elif (not (Variables|Default|GetisBurning))
      (Transformation|AttachComponentToComponent (Variables|Default|GetMesh) (Variables|Default|GetBox) "None" "SnapToTarget" "SnapToTarget" "KeepWorld" true)
      (Physics|SetSimulatePhysics (Variables|Default|GetBox) false)
      (bind _asbp_character_2 (Utilities|Casting|CastToBP_Character (Game|GetPlayerCharacter 0)))
      (Variables|/Game/Blueprints/Bluperints/BP_Character.BP_Character_C|SetCaryObject _asbp_character_2 true)
      (Variables|/Game/Blueprints/Bluperints/BP_Character.BP_Character_C|SetCarriedObject _asbp_character_2 self)
      (Transformation|AttachComponentToComponent Character "AttachPoint" "SnapToTarget" "SnapToTarget" "KeepWorld" false)
      (Variables|/Game/Blueprints/Bluperints/BP_Character.BP_Character_C|SetGrabbedInteraction _asbp_character_2 "Throw away")
      (Variables|Default|SetisGrabbed true)
      (Default|ShowGrabbedInteraction _asbp_character_2)
      (if (Variables|Default|GetisGeneratorSpawned)
        (bind _outactors (Actor|GetAllActorsOfClass "/Game/Blueprints/Bluperints/BP_Generator.BP_Generator_C"))
        (Variables|/Game/Blueprints/Bluperints/BP_Generator.BP_Generator_C|SetisRat (Utilities|Array|Get(acopy) _outactors) false)))))

(event EventInteract
  (if (Variables|Default|GetisGrabbed)
    (bind _asbp_character (Utilities|Casting|CastToBP_Character (Game|GetPlayerCharacter 0)))
    (Default|Throw _asbp_character (Variables|Default|GetBox))))

(event EventAblaze
  (Variables|Default|SetisElectrified true)
  (bind _returnvalue (Game|SpawnActorfromClass "/Game/ParticleSystems/BP_Flame.BP_Flame_C" (Math|Transform|MakeTransform (Transformation|GetWorldLocation (Variables|Default|GetFlameSpawnPoint))) "Undefined" 0 0))
  (Variables|/Game/ParticleSystems/BP_Flame.BP_Flame_C|SetCombustive _returnvalue self)
  (Transformation|AttachComponentToComponent _returnvalue (Variables|Default|GetBox) "None" "SnapToTarget" "SnapToTarget" "KeepWorld" true)
  (Variables|Default|SetisBurning true))

(event EventTurnOff
  (Variables|Default|SetisBurning false))

(fn ConstructionScript)