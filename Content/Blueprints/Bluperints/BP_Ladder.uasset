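; BP_Ladder is an interactable ladder that moves the player character up or down along predefined splines.
; A detection box gates interaction, while top and bottom triggers set whether Interact starts a descent or a climb.
; Timelines scaled by a shared duration drive the capsule along the matching spline, with a camera turn preceding descent.
; Climbing sets a GettingOut guard that this Blueprint never resets.
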(event OnComponentBeginOverlap(BotTrigger)
  (params (OverlappedComponent :type Primitive%20Component%20Object%20Reference) (OtherActor :type Actor%20Object%20Reference) (OtherComp :type Primitive%20Component%20Object%20Reference) (OtherBodyIndex :type Integer) (bFromSweep :type Boolean) (SweepResult :type Hit%20Result%20Structure%20%28by%20ref%29))
  (Utilities|Casting|CastToBP_Character OtherActor)
  (Variables|Default|SetisPlayerTop false))

(event OnComponentBeginOverlap(DetectionBox)
  (params (OverlappedComponent :type Primitive%20Component%20Object%20Reference) (OtherActor :type Actor%20Object%20Reference) (OtherComp :type Primitive%20Component%20Object%20Reference) (OtherBodyIndex :type Integer) (bFromSweep :type Boolean) (SweepResult :type Hit%20Result%20Structure%20%28by%20ref%29))
  (Utilities|Casting|CastToBP_Character OtherActor)
  (Variables|Default|SetIsPlayerIn true))

(event OnComponentEndOverlap(DetectionBox)
  (params (OverlappedComponent :type Primitive%20Component%20Object%20Reference) (OtherActor :type Actor%20Object%20Reference) (OtherComp :type Primitive%20Component%20Object%20Reference) (OtherBodyIndex :type Integer))
  (Utilities|Casting|CastToBP_Character OtherActor)
  (Variables|Default|SetIsPlayerIn false))

(event OnComponentBeginOverlap(TopTrigger)
  (params (OverlappedComponent :type Primitive%20Component%20Object%20Reference) (OtherActor :type Actor%20Object%20Reference) (OtherComp :type Primitive%20Component%20Object%20Reference) (OtherBodyIndex :type Integer) (bFromSweep :type Boolean) (SweepResult :type Hit%20Result%20Structure%20%28by%20ref%29))
  (Utilities|Casting|CastToBP_Character OtherActor)
  (Variables|Default|SetisPlayerTop true))

(event Custom|Climbing
  (if (not (Variables|Default|GetgettingOut))
    (Variables|Default|SetgettingOut true)
    (Components|Timeline|SetPlayRate (Variables|Default|GetClimbOverMovement) (/ 1.0 (Variables|Default|GetClimbOverDuration)))
    (bind _lerpalpha (Timeline|ClimbOverMovement PlayFromStart)
      (:Update
        (CallFunction|ClimbOver _lerpalpha (Variables|Default|GetClimbOverSpline))))))

(event Custom|GoingDown
  (Default|QTECameraControlMove (Variables|Default|GetCharacter) 1.5 (Transformation|GetWorldLocation (Variables|Default|GetLookAtPoint)))
  (Utilities|FlowControl|Delay 1.5)
  (Components|Timeline|SetPlayRate (Variables|Default|GetGoingDownMovement) (/ 1.0 (Variables|Default|GetClimbOverDuration)))
  (bind _lerpalpha (Timeline|GoingDownMovement PlayFromStart)
    (:Update
      (CallFunction|ClimbOver _lerpalpha (Variables|Default|GetGoingDownSpline)))))

(event EventBeginPlay
  (bind _asbp_character (Utilities|Casting|CastToBP_Character (Game|GetPlayerCharacter 0)))
  (Variables|Default|SetCharacter _asbp_character))

(event Collision|EventActorBeginOverlap
  (params (OtherActor :type Actor%20Object%20Reference)))

(event EventTick
  (params (DeltaSeconds :type Float%20%28single-precision%29)))

(event EventInteract
  (if (Variables|Default|GetIsPlayerIn)
    (if (Variables|Default|GetisPlayerTop)
      (CallFunction|GoingDown)
      (else
        (CallFunction|Climbing)))))

(event EventRevealInteractions
  (Default|ShowInteractions (Variables|Default|GetCharacter) "Climb the Ladder" false))

(fn ConstructionScript)

(fn ClimbOver
  (params (LerpAlpha :type Float%20%28single-precision%29) (Spline :type Spline%20Component%20Object%20Reference))
  (Transformation|SetWorldLocation (Variables|/Script/Engine.Character|GetCapsuleComponent (Variables|Default|GetCharacter)) (Spline|GetLocationatDistanceAlongSpline Spline (* LerpAlpha (Spline|GetSplineLength Spline)) "World") false false))