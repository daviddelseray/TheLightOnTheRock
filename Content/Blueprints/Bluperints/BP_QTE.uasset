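; Quick-time event actor that checks player actions against a list of required interactions, with empty Event, Success and Fail events.
; StartStopQTE flags BP_Character, registers itself as its current QTE and swaps the main and QTE HUDs through BP_LevelManager.
; ShowInput displays the current prompt dimmed, and AcceptInput whitens it and opens input.
; ProcessInput then calls Success or Fail; no sequencing or timing logic lives here.
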(event Custom|Event)

(event Custom|Success)

(event Custom|Fail)

(event EventBeginPlay)

(event Collision|EventActorBeginOverlap
  (params (OtherActor :type Actor%20Object%20Reference)))

(event EventTick
  (params (DeltaSeconds :type Float%20%28single-precision%29)))

(fn ConstructionScript)

(fn ProcessInput
  (params (ReceivedAction :type BPE_QTEActions%20Enum :default "NewEnumerator0"))
  (if (Variables|Default|GetAcceptingInputs)
    (if (Utilities|Enum|Equal(Enum) ReceivedAction (Utilities|Array|Get(acopy) (Variables|Default|GetRequiredInteractions) (Variables|Default|GetCurrentInteraction)))
      (CallFunction|Success)
      (else
        (CallFunction|Fail)))))

(fn DisplayQTEHud
  (bind _outactors (Actor|GetAllActorsOfClass "/Game/Blueprints/Bluperints/BP_LevelManager.BP_LevelManager_C"))
  (Widget|SetVisibility (Variables|/Game/Blueprints/Bluperints/BP_LevelManager.BP_LevelManager_C|GetMainHUD (Utilities|Array|Get(acopy) _outactors)) "Hidden")
  (Widget|SetVisibility (Variables|/Game/Blueprints/Bluperints/BP_LevelManager.BP_LevelManager_C|GetQTEHUD (Utilities|Array|Get(acopy) _outactors)) "Visible")
  (Variables|/Game/Widgets/W_QTEHUD.W_QTEHUD_C|SetInputImageVisibility (Variables|/Game/Blueprints/Bluperints/BP_LevelManager.BP_LevelManager_C|GetQTEHUD (Utilities|Array|Get(acopy) _outactors)) "Hidden")
  (Default|MoveBands (Variables|/Game/Blueprints/Bluperints/BP_LevelManager.BP_LevelManager_C|GetQTEHUD (Utilities|Array|Get(acopy) _outactors)) true))

(fn HideQTEhud
  (bind _outactors (Actor|GetAllActorsOfClass "/Game/Blueprints/Bluperints/BP_LevelManager.BP_LevelManager_C"))
  (Widget|SetVisibility (Variables|/Game/Blueprints/Bluperints/BP_LevelManager.BP_LevelManager_C|GetQTEHUD (Utilities|Array|Get(acopy) _outactors)) "Hidden")
  (Variables|/Game/Widgets/W_QTEHUD.W_QTEHUD_C|SetSubtitle (Variables|/Game/Blueprints/Bluperints/BP_LevelManager.BP_LevelManager_C|GetQTEHUD (Utilities|Array|Get(acopy) _outactors)) "")
  (Variables|/Game/Widgets/W_QTEHUD.W_QTEHUD_C|SetSpeakerName (Variables|/Game/Blueprints/Bluperints/BP_LevelManager.BP_LevelManager_C|GetQTEHUD (Utilities|Array|Get(acopy) _outactors)) "")
  (Widget|SetVisibility (Variables|/Game/Blueprints/Bluperints/BP_LevelManager.BP_LevelManager_C|GetMainHUD (Utilities|Array|Get(acopy) _outactors)) "Visible"))

(fn AcceptInput
  (Variables|Default|SetAcceptingInputs true)
  (bind _outactors (Actor|GetAllActorsOfClass "/Game/Blueprints/Bluperints/BP_LevelManager.BP_LevelManager_C"))
  (Variables|/Game/Widgets/W_QTEHUD.W_QTEHUD_C|SetLetterColor (Variables|/Game/Blueprints/Bluperints/BP_LevelManager.BP_LevelManager_C|GetQTEHUD (Utilities|Array|Get(acopy) _outactors)) "(R=1.000000,G=1.000000,B=1.000000,A=1.000000)"))

(fn ShowInput
  (switch Utilities|FlowControl|Switch|SwitchonBPE_QTEActions (Utilities|Array|Get(acopy) (Variables|Default|GetRequiredInteractions) (Variables|Default|GetCurrentInteraction))
    (:NewEnumerator0
      (LocalVariables|SetImageToPass (Variables|Default|GetInputInteract)))
    (:NewEnumerator1
      (LocalVariables|SetImageToPass (Variables|Default|GetInputGoUp)))
    (:NewEnumerator2
      (LocalVariables|SetImageToPass (Variables|Default|GetInputGoDown)))
    (:NewEnumerator3
      (LocalVariables|SetImageToPass (Variables|Default|GetInputGoLeft)))
    (:NewEnumerator4
      (LocalVariables|SetImageToPass (Variables|Default|GetInputGoRight)))
    (:NewEnumerator5
      (LocalVariables|SetImageToPass (Variables|Default|GetInputGrab))))
  (bind _outactors (Actor|GetAllActorsOfClass "/Game/Blueprints/Bluperints/BP_LevelManager.BP_LevelManager_C"))
  (Variables|/Game/Widgets/W_QTEHUD.W_QTEHUD_C|SetInputImage (Variables|/Game/Blueprints/Bluperints/BP_LevelManager.BP_LevelManager_C|GetQTEHUD (Utilities|Array|Get(acopy) _outactors)) (LocalVariables|GetImageToPass))
  (Variables|/Game/Widgets/W_QTEHUD.W_QTEHUD_C|SetLetterColor (Variables|/Game/Blueprints/Bluperints/BP_LevelManager.BP_LevelManager_C|GetQTEHUD (Utilities|Array|Get(acopy) _outactors)) "(R=0.031250,G=0.031250,B=0.031250,A=1.000000)")
  (Variables|/Game/Widgets/W_QTEHUD.W_QTEHUD_C|SetInputImageVisibility (Variables|/Game/Blueprints/Bluperints/BP_LevelManager.BP_LevelManager_C|GetQTEHUD (Utilities|Array|Get(acopy) _outactors)) "Visible"))

(fn StartStopQTE
  (params (isStarting :type Boolean))
  (bind _asbp_character (Utilities|Casting|CastToBP_Character (Game|GetPlayerCharacter 0)))
  (if isStarting
    (Variables|/Game/Blueprints/Bluperints/BP_Character.BP_Character_C|SetisDoingQTE _asbp_character true)
    (Variables|/Game/Blueprints/Bluperints/BP_Character.BP_Character_C|SetCurrentQTE _asbp_character self)
    (CallFunction|DisplayQTEHud)
    (else
      (Variables|/Game/Blueprints/Bluperints/BP_Character.BP_Character_C|SetisDoingQTE _asbp_character false)
      (CallFunction|HideQTEhud))))

(fn HideInput
  (bind _outactors (Actor|GetAllActorsOfClass "/Game/Blueprints/Bluperints/BP_LevelManager.BP_LevelManager_C"))
  (Variables|/Game/Widgets/W_QTEHUD.W_QTEHUD_C|SetInputImageVisibility (Variables|/Game/Blueprints/Bluperints/BP_LevelManager.BP_LevelManager_C|GetQTEHUD (Utilities|Array|Get(acopy) _outactors)) "Hidden"))