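; BP_Medal is a grabbable, throwable medal pickup that advances level progression when first grabbed.
; FirstGrab sets the day on BP_LevelManager and triggers the next problem, while Appear reveals the mesh and enables Sphere query collision.
; Grab disables physics and attaches the actor to the character's AttachPoint socket, updating BP_Character carry state and interaction prompts.
; Release detaches it and restores physics, while Interact passes the held medal to the character's Throw.
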(event Custom|FirstGrab
  (bind _levelmanager (Variables|Default|GetlevelManager))
  (if (Variables|Default|GetisGrabbable)
    (Variables|Default|SethasBeenGrabbed true)
    (Variables|/Game/Blueprints/Bluperints/BP_LevelManager.BP_LevelManager_C|SetCurrentDay _levelmanager 3)
    (Default|ProblemResolution _levelmanager 10 0.0)))

(event Custom|Appear
  (Rendering|SetVisibility (Variables|Default|GetMedal) true false)
  (Collision|SetCollisionEnabled (Variables|Default|GetSphere) "QueryOnly"))

(event EventBeginPlay
  (bind _outactors (Actor|GetAllActorsOfClass "/Game/Blueprints/Bluperints/BP_LevelManager.BP_LevelManager_C"))
  (Variables|Default|SetlevelManager (Utilities|Array|Get(acopy) _outactors)))

(event Collision|EventActorBeginOverlap
  (params (OtherActor :type Actor%20Object%20Reference)))

(event EventTick
  (params (DeltaSeconds :type Float%20%28single-precision%29)))

(event EventInteract
  (if (Variables|Default|GetisGrabbed)
    (bind _asbp_character (Utilities|Casting|CastToBP_Character (Game|GetPlayerCharacter 0)))
    (Default|Throw _asbp_character (Variables|Default|GetMedal))
    (Variables|Default|SetisGrabbed false)))

(event EventRelease
  (Transformation|DetachFromActor "KeepWorld" "KeepWorld" "KeepWorld")
  (bind _asbp_character (Utilities|Casting|CastToBP_Character (Game|GetPlayerCharacter 0)))
  (Variables|/Game/Blueprints/Bluperints/BP_Character.BP_Character_C|SetCaryObject _asbp_character false)
  (Variables|/Game/Blueprints/Bluperints/BP_Character.BP_Character_C|SetCarriedObject _asbp_character 0)
  (Physics|SetSimulatePhysics (Variables|Default|GetMedal) true)
  (Variables|Default|SetisGrabbed false))

(event EventGrab
  (params (Character :type Skeletal%20Mesh%20Component%20Object%20Reference))
  (if (Variables|Default|GetisGrabbable)
    (Transformation|AttachComponentToComponent (Variables|Default|GetMedal) (Variables|Default|GetDefaultSceneRoot) "None" "SnapToTarget" "SnapToTarget" "KeepWorld" true)
    (Physics|SetSimulatePhysics (Variables|Default|GetMedal) false)
    (bind _asbp_character (Utilities|Casting|CastToBP_Character (Game|GetPlayerCharacter 0)))
    (Variables|/Game/Blueprints/Bluperints/BP_Character.BP_Character_C|SetCaryObject _asbp_character true)
    (Variables|/Game/Blueprints/Bluperints/BP_Character.BP_Character_C|SetCarriedObject _asbp_character self)
    (Transformation|AttachComponentToComponent Character "AttachPoint" "SnapToTarget" "SnapToTarget" "KeepWorld" false)
    (Variables|/Game/Blueprints/Bluperints/BP_Character.BP_Character_C|SetGrabbedInteraction _asbp_character "Throw away")
    (Variables|Default|SetisGrabbed true)
    (Default|ShowGrabbedInteraction _asbp_character)))

(event EventShowGrabInteraction
  (if (Variables|Default|GetisGrabbable)
    (bind _asbp_character (Utilities|Casting|CastToBP_Character (Game|GetPlayerCharacter 0)))
    (Default|ChangeGrabHUD _asbp_character "Grab the medal" true)))

(fn ConstructionScript)