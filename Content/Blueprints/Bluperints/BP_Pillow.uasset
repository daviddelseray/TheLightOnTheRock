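; BP_Pillow is a physics pillow actor that the player can pick up, carry and release.
; Grab snaps the pillow back to its root, disables physics, and attaches to the passed character's AttachPoint socket with a fixed relative offset.
; Release detaches it in world space and re-enables physics.
; Both events update the carry flag and carried-object reference on player 0's BP_Character.
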(event EventBeginPlay)

(event Collision|EventActorBeginOverlap
  (params (OtherActor :type Actor%20Object%20Reference)))

(event EventTick
  (params (DeltaSeconds :type Float%20%28single-precision%29)))

(event EventRelease
  (Transformation|DetachFromActor "KeepWorld" "KeepWorld" "KeepWorld")
  (bind _asbp_character (Utilities|Casting|CastToBP_Character (Game|GetPlayerCharacter 0)))
  (Variables|/Game/Blueprints/Bluperints/BP_Character.BP_Character_C|SetCaryObject _asbp_character false)
  (Variables|/Game/Blueprints/Bluperints/BP_Character.BP_Character_C|SetCarriedObject _asbp_character 0)
  (Physics|SetSimulatePhysics (Variables|Default|GetPillow) true))

(event EventGrab
  (params (Character :type Skeletal%20Mesh%20Component%20Object%20Reference))
  (Transformation|AttachComponentToComponent (Variables|Default|GetPillow) (Variables|Default|GetDefaultSceneRoot) "None" "SnapToTarget" "SnapToTarget" "KeepWorld" true)
  (Physics|SetSimulatePhysics (Variables|Default|GetPillow) false)
  (bind _asbp_character (Utilities|Casting|CastToBP_Character (Game|GetPlayerCharacter 0)))
  (Variables|/Game/Blueprints/Bluperints/BP_Character.BP_Character_C|SetCaryObject _asbp_character true)
  (Variables|/Game/Blueprints/Bluperints/BP_Character.BP_Character_C|SetCarriedObject _asbp_character self)
  (Transformation|AttachComponentToComponent Character "AttachPoint" "SnapToTarget" "SnapToTarget" "KeepWorld" false)
  (Transformation|SetRelativeLocationAndRotation (Variables|Default|GetDefaultSceneRoot) "0,11.000000,1.000000" "19.400000,-7.300000,-21.000000" false false))

(fn ConstructionScript)