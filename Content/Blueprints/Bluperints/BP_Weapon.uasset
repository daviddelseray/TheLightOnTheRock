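; BP_Weapon is a weapon actor the player can grab, carry and release.
; Grab disables physics, snaps the mesh to its grip point, attaches to the character's socket and marks BP_Character as armed and carrying; Release reverses this.
; ShowGrabInteraction puts a named grab prompt on the character's HUD.
; Grabbing during one specific day and problem in BP_LevelManager plays a one-time monologue through BP_DialogManager.
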(event Custom|PresentationLine
  (if (not (Variables|Default|GethasBeenGrabbed))
    (Variables|Default|SethasBeenGrabbed true)
    (bind _outactors (Actor|GetAllActorsOfClass "/Game/Blueprints/Bluperints/BP_DialogManager.BP_DialogManager_C"))
    (Default|PlayMonolog (Utilities|Array|Get(acopy) _outactors) (Variables|Default|GetLine))))

(event EventBeginPlay)

(event Collision|EventActorBeginOverlap
  (params (OtherActor :type Actor%20Object%20Reference)))

(event EventTick
  (params (DeltaSeconds :type Float%20%28single-precision%29)))

(event EventRelease
  (Transformation|DetachFromActor "KeepWorld" "KeepWorld" "KeepWorld")
  (Transformation|AttachComponentToComponent (Variables|Default|GetStaticMesh) (Variables|Default|GetGripPoint) "None" "SnapToTarget" "SnapToTarget" "KeepWorld" true)
  (bind _asbp_character (Utilities|Casting|CastToBP_Character (Game|GetPlayerCharacter 0)))
  (Variables|/Game/Blueprints/Bluperints/BP_Character.BP_Character_C|SetCaryObject _asbp_character false)
  (Variables|/Game/Blueprints/Bluperints/BP_Character.BP_Character_C|SetCarriedObject _asbp_character 0)
  (Variables|/Game/Blueprints/Bluperints/BP_Character.BP_Character_C|SetisArmed _asbp_character false)
  (Physics|SetSimulatePhysics (Variables|Default|GetStaticMesh) true)
  (Variables|Default|SetisGrabbed false))

(event EventGrab
  (params (Character :type Skeletal%20Mesh%20Component%20Object%20Reference))
  (Physics|SetSimulatePhysics (Variables|Default|GetStaticMesh) false)
  (Transformation|AttachComponentToComponent (Variables|Default|GetStaticMesh) (Variables|Default|GetGripPoint) "None" "SnapToTarget" "SnapToTarget" "SnapToTarget" true)
  (Transformation|SetRelativeRotation (Variables|Default|GetStaticMesh) (Variables|Default|GetGrabbedRotation) false false)
  (Transformation|SetRelativeLocation (Variables|Default|GetStaticMesh) (Variables|Default|GetGrabbedLocation) false false)
  (Transformation|AttachComponentToComponent Character "AttachPoint" "SnapToTarget" "SnapToTarget" "KeepWorld" true)
  (bind _asbp_character (Utilities|Casting|CastToBP_Character (Game|GetPlayerCharacter 0)))
  (Variables|/Game/Blueprints/Bluperints/BP_Character.BP_Character_C|SetCaryObject _asbp_character true)
  (Variables|/Game/Blueprints/Bluperints/BP_Character.BP_Character_C|SetCarriedObject _asbp_character self)
  (Variables|/Game/Blueprints/Bluperints/BP_Character.BP_Character_C|SetisArmed _asbp_character true)
  (bind _outactors (Actor|GetAllActorsOfClass "/Game/Blueprints/Bluperints/BP_LevelManager.BP_LevelManager_C"))
  (if (and (== (Variables|/Game/Blueprints/Bluperints/BP_LevelManager.BP_LevelManager_C|GetCurrentDay (Utilities|Array|Get(acopy) _outactors)) 2) (== (Variables|/Game/Blueprints/Bluperints/BP_LevelManager.BP_LevelManager_C|GetCurrentProblem (Utilities|Array|Get(acopy) _outactors)) 23))
    (CallFunction|PresentationLine)))

(event EventShowGrabInteraction
  (bind _asbp_character (Utilities|Casting|CastToBP_Character (Game|GetPlayerCharacter 0)))
  (Default|ChangeGrabHUD _asbp_character (Utilities|String|Append "Grab the " (Variables|Default|GetNameOfWeapon)) true))

(fn ConstructionScript)