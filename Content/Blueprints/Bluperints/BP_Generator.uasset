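; Generator actor that spins its wheel while on and controls the level's light flickering through a BP_LightControl found at BeginPlay.
; Activate stops the flicker and can advance a specific LevelManager problem, while Deactivate starts the flicker.
; The Rat event shuts it off and spawns an ablaze rat with sparks.
; Once IsRat is set, Activate and Deactivate instead toggle the sparks and the rat's electrified state.
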(event Custom|Rat
  ;[1 1 1] RAT EVENT : Spawn Rat
  (Variables|Default|SetisRat true)
  (bind _returnvalue (Game|SpawnActorfromClass "/Game/Blueprints/Bluperints/BP_Rat.BP_Rat_C" (Math|Transform|MakeTransform (Transformation|GetWorldLocation (Variables|Default|GetRatSpawnPoint))) "Undefined" 0 0))
  (bind _output_get (Variables|Default|SetSpawnedRat _returnvalue))
  (Default|Ablaze _output_get)
  (Variables|/Game/Blueprints/Bluperints/BP_Rat.BP_Rat_C|SetisGeneratorSpawned _output_get true)
  ;[1 1 1] Spawn the sparks and turn off generator
  (bind _returnvalue_2 (Game|SpawnActorfromClass "/Game/ParticleSystems/BP_Sparks.BP_Sparks_C" (Transformation|GetWorldTransform (Variables|Default|GetSparksSpawnPoint)) "Undefined" 0 0))
  (bind _output_get_2 (Variables|Default|SetSparks _returnvalue_2))
  (Audio|SpawnSoundAttached 0 (Variables|/Script/Engine.Actor|GetRootComponent _output_get_2) "None" "0, 0, 0" "0, 0, 0" "KeepRelativeOffset" false 1.0 1.0 0.0 0 0)
  (Variables|Default|SetisOn false))

(event EventBeginPlay
  (bind _outactors (Actor|GetAllActorsOfClass "/Game/Blueprints/Bluperints/BP_LightControl.BP_LightControl_C"))
  (Variables|Default|SetLightControl (Utilities|Array|Get(acopy) _outactors)))

(event Collision|EventActorBeginOverlap
  (params (OtherActor :type Actor%20Object%20Reference)))

(event EventTick
  (params (DeltaSeconds :type Float%20%28single-precision%29))
  ;[1 1 1] Turn the wheel
  (if (Variables|Default|GetisOn)
    (Transformation|AddRelativeRotation (Variables|Default|GetWheelTrain) (Math|Rotator|MakeRotator (Variables|Default|GetWheelRotationSpeed) 0.0 0.0) false false)))

(event EventActivate
  (bind _levelmanager (Variables|Default|GetLevelManager))
  (if (Variables|Default|GetisRat)
    (bind _returnvalue (Game|SpawnActorfromClass "/Game/ParticleSystems/BP_Sparks.BP_Sparks_C" (Transformation|GetWorldTransform (Variables|Default|GetSparksSpawnPoint)) "Undefined" 0 0))
    (bind _output_get (Variables|Default|SetSparks _returnvalue))
    (Audio|SpawnSoundAttached 0 (Variables|/Script/Engine.Actor|GetRootComponent _output_get) "None" "0, 0, 0" "0, 0, 0" "KeepRelativeOffset" false 1.0 1.0 0.0 0 0)
    (Variables|/Game/Blueprints/Bluperints/BP_Rat.BP_Rat_C|SetisElectrified (Variables|Default|GetSpawnedRat) true)
    (else
      (Default|StopFlickering (Variables|Default|GetLightControl))
      (Variables|Default|SetisOn true)
      (if (and (== (Variables|/Game/Blueprints/Bluperints/BP_LevelManager.BP_LevelManager_C|GetCurrentDay _levelmanager) 1) (== (Variables|/Game/Blueprints/Bluperints/BP_LevelManager.BP_LevelManager_C|GetCurrentProblem _levelmanager) 6))
        (Default|ProblemResolution (Variables|Default|GetLevelManager) 7)))))

(event EventDeactivate
  (bind _lightcontrol (Variables|Default|GetLightControl))
  ;[1 1 1] Turn off the generator, turn off the lights
  (if (Variables|Default|GetisRat)
    (Actor|DestroyActor (Variables|Default|GetSparks))
    (Variables|/Game/Blueprints/Bluperints/BP_Rat.BP_Rat_C|SetisElectrified (Variables|Default|GetSpawnedRat) false)
    (else
      (Variables|/Game/Blueprints/Bluperints/BP_LightControl.BP_LightControl_C|SetFlicker _lightcontrol true)
      (Default|StartFlickering _lightcontrol)
      (Default|Flickering _lightcontrol true)))
  (Variables|Default|SetisOn false))

(fn ConstructionScript)