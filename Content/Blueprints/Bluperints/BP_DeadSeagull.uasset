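; Dead seagull prop that the player can grab, carry and throw.
; Grab disables Box physics, attaches it to the character's AttachPoint socket and registers it as the carried object on BP_Character.
; Interact while held passes Box to the character's Throw; Release detaches, re-snaps Cube to Box, restores physics and clears the carry state.
; It also supplies the grab HUD prompt, and Activate makes Cube visible with optional audio.
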(event Custom|Activate
  (params (ShouldPlaySound :type Boolean))
  (Rendering|SetVisibility (Variables|Default|GetCube) true false)
  (if ShouldPlaySound
    (Audio|Components|Audio|Play (Variables|Default|GetAudio) 0.0)))

(event EventBeginPlay)

(event Collision|EventActorBeginOverlap
  (params (OtherActor :type Actor%20Object%20Reference)))

(event EventTick
  (params (DeltaSeconds :type Float%20%28single-precision%29)))

(event EventGrab
  (params (Character :type Skeletal%20Mesh%20Component%20Object%20Reference))
  (Physics|SetSimulatePhysics (Variables|Default|GetBox) false)
  (Transformation|AttachComponentToComponent (Variables|Default|GetCube) (Variables|Default|GetBox) "None" "SnapToTarget" "SnapToTarget" "KeepWorld" true)
  (bind _asbp_character (Utilities|Casting|CastToBP_Character (Game|GetPlayerCharacter 0)))
  (Variables|/Game/Blueprints/Bluperints/BP_Character.BP_Character_C|SetCaryObject _asbp_character true)
  (Variables|/Game/Blueprints/Bluperints/BP_Character.BP_Character_C|SetCarriedObject _asbp_character self)
  (Transformation|AttachComponentToComponent Character "AttachPoint" "SnapToTarget" "SnapToTarget" "KeepWorld" false)
  (Variables|/Game/Blueprints/Bluperints/BP_Character.BP_Character_C|SetGrabbedInteraction _asbp_character "Throw away")
  (Variables|Default|SetisGrabbed true)
  (Default|ShowGrabbedInteraction _asbp_character))

(event EventRelease
  (Transformation|DetachFromActor "KeepWorld" "KeepWorld" "KeepWorld")
  (Transformation|AttachComponentToComponent (Variables|Default|GetCube) (Variables|Default|GetBox) "None" "SnapToTarget" "SnapToTarget" "KeepWorld" true)
  (bind _asbp_character (Utilities|Casting|CastToBP_Character (Game|GetPlayerCharacter 0)))
  (Variables|/Game/Blueprints/Bluperints/BP_Character.BP_Character_C|SetCaryObject _asbp_character false)
  (Variables|/Game/Blueprints/Bluperints/BP_Character.BP_Character_C|SetCarriedObject _asbp_character 0)
  (Physics|SetSimulatePhysics (Variables|Default|GetBox) true)
  (Variables|Default|SetisGrabbed false))

(event EventInteract
  (if (Variables|Default|GetisGrabbed)
    (bind _asbp_character (Utilities|Casting|CastToBP_Character (Game|GetPlayerCharacter 0)))
    (Default|Throw _asbp_character (Variables|Default|GetBox))))

(event EventShowGrabInteraction
  (bind _asbp_character (Utilities|Casting|CastToBP_Character (Game|GetPlayerCharacter 0)))
  (Default|ChangeGrabHUD _asbp_character "Grab the dead seagull" true))

(fn ConstructionScript)