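; BP_Door is a door actor that swings open and closed when its Interact event fires.
; Interact uses a FlipFlop to alternate between the Open and Close events, which play and reverse the OpenClose timeline.
; The timeline's RotationZ track drives the relative yaw of the PivotPoint component, with roll and pitch held at zero.
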(event Custom|Open
  (bind (_roll _pitch) (Math|Rotator|BreakRotator "0, 0, 0"))
  (bind _rotationz (Timeline|OpenClose Play)
    (:Update
      (Transformation|SetRelativeRotation (Variables|Default|GetPivotPoint) (Math|Rotator|MakeRotator _roll _pitch _rotationz) false false))))

(event Custom|Close
  (bind (_roll _pitch) (Math|Rotator|BreakRotator "0, 0, 0"))
  (bind _rotationz (Timeline|OpenClose Reverse)
    (:Update
      (Transformation|SetRelativeRotation (Variables|Default|GetPivotPoint) (Math|Rotator|MakeRotator _roll _pitch _rotationz) false false))))

(event EventBeginPlay)

(event Collision|EventActorBeginOverlap
  (params (OtherActor :type Actor%20Object%20Reference)))

(event EventTick
  (params (DeltaSeconds :type Float%20%28single-precision%29)))

(event EventInteract
  (Utilities|FlowControl|FlipFlop
    (:A
      (CallFunction|Open))
    (:B
      (CallFunction|Close))))

(fn ConstructionScript)