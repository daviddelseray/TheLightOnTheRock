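; Interactable fuse box lever that toggles between up and down and reports its Id and state to its FuseBox.
; Interact plays a player animation unless the system triggered the flip, then a Rotation timeline swings the switch pivot, delayed only when moving down.
; When rotation finishes, it notifies the FuseBox and refreshes the Activate/Deactivate prompt if the interaction collision check passes.
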(event EventBeginPlay)

(event Collision|EventActorBeginOverlap
  (params (OtherActor :type Actor%20Object%20Reference)))

(event EventTick
  (params (DeltaSeconds :type Float%20%28single-precision%29)))

(event EventInteract
  (bind _switchpivotpoint (Variables|Default|GetSwitchPivotPoint))
  (bind _returnvalue (Transformation|GetWorldRotation _switchpivotpoint))
  (bind (_roll _pitch _yaw) (Math|Rotator|BreakRotator _returnvalue))
  (if (Variables|Default|GetIsUp)
    (Variables|Default|SetIsUp false)
    (if (Variables|Default|GetisSystemTriggered)
      _
      (else
        (bind _asbp_character (Utilities|Casting|CastToBP_Character (Game|GetPlayerCharacter 0)))
        (Default|ObjectInteractAnimationin _asbp_character "NewEnumerator6")))
    (else
      (Variables|Default|SetIsUp true)
      (if (Variables|Default|GetisSystemTriggered)
        _
        (else
          (bind _asbp_character_2 (Utilities|Casting|CastToBP_Character (Game|GetPlayerCharacter 0)))
          (Default|ObjectInteractAnimationin _asbp_character_2 "NewEnumerator5")))))
  (Utilities|FlowControl|Sequence
    (:then_0
      (Utilities|FlowControl|Delay 0.2)
      (if (not (Variables|Default|GetisSystemTriggered))
        (if (Variables|Default|GetIsUp)
          (bind _asbp_character_3 (Utilities|Casting|CastToBP_Character (Game|GetPlayerCharacter 0)))
          (Variables|/Game/DefaultContent/FirstPerson/Animations/ABP_Character.ABP_Character_C|SetActivatingLever (Variables|/Game/Blueprints/Bluperints/BP_Character.BP_Character_C|GetABP_Character _asbp_character_3) false)
          (else
            (bind _asbp_character_4 (Utilities|Casting|CastToBP_Character (Game|GetPlayerCharacter 0)))
            (Variables|/Game/DefaultContent/FirstPerson/Animations/ABP_Character.ABP_Character_C|SetDeactivatingLever (Variables|/Game/Blueprints/Bluperints/BP_Character.BP_Character_C|GetABP_Character _asbp_character_4) false)))))
    (:then_1
      (Variables|Default|SetisSystemTriggered false)
      (if (Variables|Default|GetIsUp)
        (bind _xrot (Timeline|Rotation ReverseFromEnd)
          (:Update
            (Transformation|SetWorldRotation (Variables|Default|GetSwitchPivotPoint) (Math|Rotator|MakeRotator _xrot _pitch _yaw) false false))
          (:Finished
            (Default|ReceiveInput (Variables|Default|GetFuseBox) (Variables|Default|GetId) (Variables|Default|GetIsUp))
            (bind _interactionconepresent (CallFunction|CheckInteractionCollision))
            (if _interactionconepresent
              (CallFunction|RevealInteractions))))
        (else
          (Utilities|FlowControl|Delay 1.0)
          (Timeline|Rotation PlayFromStart))))))

(event EventRevealInteractions
  (bind _asbp_character (Utilities|Casting|CastToBP_Character (Game|GetPlayerCharacter 0)))
  (if (Variables|Default|GetIsUp)
    (Default|ShowInteractions _asbp_character "Deactivate" false)
    (else
      (Default|ShowInteractions _asbp_character "Activate" false))))

(fn ConstructionScript)

(fn CheckInteractionCollision
  (for _array_element (Class|PrimitiveComponent|GetOverlappingComponents (Variables|Default|GetBox))
    _)
  (return (Components|ComponentHasTag _array_element "InteractionCone")))