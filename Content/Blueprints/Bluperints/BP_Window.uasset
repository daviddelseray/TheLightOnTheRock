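; BP_Window is a window that can break and be boarded up by the player with carried planks.
; Break swaps the frame meshes and spawns BP_WindowDebris at the debris point.
; While broken, it shows a repair prompt if BP_Character carries BP_Planks, and each interaction reveals one of three planks and destroys the carried one.
; The final plank clears the broken state and resolves a specific day's problem in BP_LevelManager.
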(event Custom|Break
  (Rendering|SetVisibility (Variables|Default|GetWindowFrame) false true)
  (Rendering|SetVisibility (Variables|Default|GetBrokenWindowFrame) true true)
  (Game|SpawnActorfromClass "/Game/Blueprints/Bluperints/BP_WindowDebris.BP_WindowDebris_C" (Math|Transform|MakeTransform (Transformation|GetWorldLocation (Variables|Default|GetDebrisSpawnPoint)) "0, 0, 0" "1,1,1") "Undefined" 0 0)
  (Variables|Default|SetIsBroken true))

(event EventBeginPlay)

(event Collision|EventActorBeginOverlap
  (params (OtherActor :type Actor%20Object%20Reference)))

(event EventTick
  (params (DeltaSeconds :type Float%20%28single-precision%29)))

(event EventRevealInteractions
  (if (Variables|Default|GetIsBroken)
    (bind _asbp_character (Utilities|Casting|CastToBP_Character (Game|GetPlayerCharacter 0)))
    (Utilities|Casting|CastToBP_Planks (Variables|/Game/Blueprints/Bluperints/BP_Character.BP_Character_C|GetCarriedObject _asbp_character))
    (Default|ShowInteractions _asbp_character "Repair Window" false)))

(event EventInteract
  (if (Variables|Default|GetIsBroken)
    (bind _asbp_character (Utilities|Casting|CastToBP_Character (Game|GetPlayerCharacter 0)))
    (Utilities|Casting|CastToBP_Planks (Variables|/Game/Blueprints/Bluperints/BP_Character.BP_Character_C|GetCarriedObject _asbp_character))
    (if (< (Variables|Default|GetRepairStage) 3)
      (bind _result (Math|Integer|IncrementInt (Variables|Default|GetRepairStage))
        (:%20%20
          (switch int _result
            (:1
              (Rendering|SetVisibility (Variables|Default|GetPlank1) true false))
            (:2
              (Rendering|SetVisibility (Variables|Default|GetPlank2) true false))
            (:3
              (Rendering|SetVisibility (Variables|Default|GetPlank3) true false)
              (Variables|Default|SetIsBroken false)))
          (bind _asbp_character_2 (Utilities|Casting|CastToBP_Character (Game|GetPlayerCharacter 0)))
          (Actor|DestroyActor (Variables|/Game/Blueprints/Bluperints/BP_Character.BP_Character_C|GetCarriedObject _asbp_character_2))
          (Variables|/Game/Blueprints/Bluperints/BP_Character.BP_Character_C|SetCaryObject _asbp_character_2 false)
          (if (== (Variables|Default|GetRepairStage) 3)
            (bind _outactors (Actor|GetAllActorsOfClass "/Game/Blueprints/Bluperints/BP_LevelManager.BP_LevelManager_C"))
            (if (and (== (Variables|/Game/Blueprints/Bluperints/BP_LevelManager.BP_LevelManager_C|GetCurrentDay (Utilities|Array|Get(acopy) _outactors)) 2) (== (Variables|/Game/Blueprints/Bluperints/BP_LevelManager.BP_LevelManager_C|GetCurrentProblem (Utilities|Array|Get(acopy) _outactors)) 1))
              (Default|ProblemResolution (Utilities|Array|Get(acopy) _outactors) 2 0.0))))))))

(fn ConstructionScript)