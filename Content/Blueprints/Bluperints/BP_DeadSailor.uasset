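; BP_DeadSailor is a dead sailor actor that can be shown or hidden, set fighting, and killed.
; On BeginPlay it caches its mesh's ABP_DeadSailor animation instance.
; Activate and Deactivate toggle the visibility of the mesh and its children.
; StartFighting and Die only set the attacking and dead flags on the animation Blueprint, with no combat or damage logic here.
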(event Custom|Activate
  (Rendering|SetVisibility (Variables|Character|GetMesh) true true))

(event Custom|Deactivate
  (Rendering|SetVisibility (Variables|Character|GetMesh) false true))

(event Custom|StartFighting
  (Variables|/Game/Animations/DeadSailor/ABP_DeadSailor.ABP_DeadSailor_C|SetisAttacking (Variables|Default|GetABP_DeadSailor) true))

(event Custom|Die
  (Variables|/Game/Animations/DeadSailor/ABP_DeadSailor.ABP_DeadSailor_C|SetisDead (Variables|Default|GetABP_DeadSailor) true))

(event EventBeginPlay
  (bind _asabp_dead_sailor (Utilities|Casting|CastToABP_DeadSailor (Components|SkeletalMesh|GetAnimInstance (Variables|Character|GetMesh))))
  (Variables|Default|SetABP_DeadSailor _asabp_dead_sailor))

(fn ConstructionScript)