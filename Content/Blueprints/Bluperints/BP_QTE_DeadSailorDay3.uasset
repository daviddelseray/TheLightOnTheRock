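; Day 3 quick-time event where the player crouches by the "dead" sailor to take a medal and he starts fighting.
; Timelines and delays script movement, camera look-ats, hand animations and monologues before opening a timed input window.
; Success has the player strike him with a rock, then walk a rail and change sanity; on timeout, he dies without that blow.
; Both outcomes grab the medal, advance BP_LevelManager's problem and record whether the player killed him.
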(event Custom|MovePlayer
  (params (Duration :type Float%20%28single-precision%29) (MovePoint :type Scene%20Component%20Object%20Reference) (InterestPoint :type Scene%20Component%20Object%20Reference))
  (Components|Timeline|SetPlayRate (Variables|Default|GetPlayerMoving) (/ 1.0 Duration))
  (Variables|Default|SettempPlayerLoc (Transformation|GetWorldLocation (Variables|/Script/Engine.Character|GetCapsuleComponent (Variables|Default|GetCharacter))))
  (bind _lerpalpha (Timeline|PlayerMoving PlayFromStart)
    (:Update
      (Transformation|SetWorldLocation (Variables|/Script/Engine.Character|GetCapsuleComponent (Variables|Default|GetCharacter)) (Math|Vector|Lerp(Vector) (Variables|Default|GettempPlayerLoc) (Transformation|GetWorldLocation MovePoint) _lerpalpha) false false)
      (CallFunction|MoveCam InterestPoint))))

(event Custom|BreakMoving
  (bind _lerpalpha (Timeline|PlayerMoving Stop)
    (:Update
      (Transformation|SetWorldLocation (Variables|/Script/Engine.Character|GetCapsuleComponent (Variables|Default|GetCharacter)) (Math|Vector|Lerp(Vector) (Variables|Default|GettempPlayerLoc) (Transformation|GetWorldLocation (stale Custom|MovePlayer MovePoint)) _lerpalpha) false false)
      (CallFunction|MoveCam (stale Custom|MovePlayer InterestPoint)))))

(event Custom|AfterBreak
  (bind _character (Variables|Default|GetCharacter))
  (bind _character_2 (Variables|Default|GetCharacter))
  (Default|CamCrouch _character 3.2 true)
  (Components|Timeline|SetPlayRate (Variables|Default|GetCamCrouch) (/ 1.0 3.2))
  (Utilities|FlowControl|Sequence
    (:then_0
      (Timeline|CamCrouch PlayFromStart
        (:Update
          (CallFunction|MoveCam (Variables|Default|GetInterestPoint2)))))
    (:then_1
      (Utilities|FlowControl|Delay 0.2)
      (Default|ObjectInteractAnimationin _character "NewEnumerator15"))
    (:then_2
      (Utilities|FlowControl|Delay 2.5)
      (CallFunction|BreakCamCrouch)
      (Transformation|DetachFromComponent (Variables|/Game/Blueprints/Bluperints/BP_Character.BP_Character_C|GetMesh2P (Variables|Default|GetCharacter)) "KeepWorld" "KeepWorld" "KeepWorld" true)
      (Transformation|AttachComponentToComponent (Variables|/Game/Blueprints/Bluperints/BP_Character.BP_Character_C|GetMesh2P _character_2) (Variables|/Script/Engine.Character|GetCapsuleComponent _character_2) "None" "KeepWorld" "KeepWorld" "KeepWorld" true)
      (Default|StartFighting (Variables|Default|GetDeadSailor))
      (Utilities|FlowControl|Delay 0.15)
      (Default|PlayMonolog (Variables|Default|GetdialogManager) 33 0.0)
      (CallFunction|MovePlayer 0.1 (Variables|Default|GetPositionPoint2) (Variables|Default|GetInterestPoint3))
      (CallFunction|ShowInput)
      (CallFunction|AcceptInput)
      (bind _returnvalue (Utilities|Time|SetTimerbyFunctionName 0 "Fail" (Utilities|Array|Get(acopy) (Variables|Default|GetInteractionsDurations) (Variables|Default|GetCurrentInteraction)))))))

(event Custom|MoveCam
  (params (InterestPoint :type Scene%20Component%20Object%20Reference))
  (Pawn|SetControlRotation (Pawn|GetController (Variables|Default|GetCharacter)) (Math|Rotator|FindLookatRotation (Transformation|GetWorldLocation (Variables|/Game/Blueprints/Bluperints/BP_Character.BP_Character_C|GetFirstPersonCamera (Variables|Default|GetCharacter))) (Transformation|GetWorldLocation InterestPoint))))

(event Custom|BreakCamCrouch
  (Timeline|CamCrouch Stop
    (:Update
      (CallFunction|MoveCam (Variables|Default|GetInterestPoint2)))))

(event Custom|Barf
  (params (goDown :type Boolean))
  (bind _character (Variables|Default|GetCharacter))
  (if goDown
    (Components|Timeline|SetPlayRate (Variables|Default|GetBarfing) (/ 1.0 0.5))
    (bind _lerpalpha (Timeline|Barfing PlayFromStart)
      (:Update
        (Transformation|SetRelativeLocation (Variables|/Game/Blueprints/Bluperints/BP_Character.BP_Character_C|GetFirstPersonCamera (Variables|Default|GetCharacter)) (Math|Vector|Lerp(Vector) (Variables|/Script/Engine.SceneComponent|GetRelativeLocation (Variables|/Game/Blueprints/Bluperints/BP_Character.BP_Character_C|GetDefaultCamPos _character)) (Variables|/Script/Engine.SceneComponent|GetRelativeLocation (Variables|/Game/Blueprints/Bluperints/BP_Character.BP_Character_C|GetWatchPointZoomPos _character)) _lerpalpha) false false)))
    (else
      (Components|Timeline|SetPlayRate (Variables|Default|GetBarfing) (/ 1.0 1.0))
      (Timeline|Barfing ReverseFromEnd))))

(event EventBeginPlay
  (|CallParentFunction)
  (bind _asbp_character (Utilities|Casting|CastToBP_Character (Game|GetPlayerCharacter 0)))
  (Variables|Default|SetCharacter _asbp_character)
  (bind _outactors (Actor|GetAllActorsOfClass "/Game/Blueprints/Bluperints/BP_DialogManager.BP_DialogManager_C"))
  (Variables|Default|SetdialogManager (Utilities|Array|Get(acopy) _outactors)))

(event Collision|EventActorBeginOverlap
  (params (OtherActor :type Actor%20Object%20Reference))
  (|CallParentFunction OtherActor) ; This node is disabled and will not be called.\nDrag off pins to build functionality.
)

(event EventTick
  (params (DeltaSeconds :type Float%20%28single-precision%29))
  (|CallParentFunction DeltaSeconds) ; This node is disabled and will not be called.\nDrag off pins to build functionality.
)

(event EventEvent
  (bind _character (Variables|Default|GetCharacter))
  (bind _character_2 (Variables|Default|GetCharacter))
  (switch int (Variables|Default|GetCurrentInteraction)
    (:0
      (CallFunction|StartStopQTE true)
      (Default|PlayMonolog (Variables|Default|GetdialogManager) 32 0.0)
      (CallFunction|MovePlayer (Variables|Default|GetMoveDuration) (Variables|Default|GetPositionPoint) (Variables|Default|GetInterestPoint))
      (Utilities|FlowControl|Delay (* (Variables|Default|GetMoveDuration) 0.8))
      (Default|CamCrouch _character 3.2 true)
      (Components|Timeline|SetPlayRate (Variables|Default|GetCamCrouch) (/ 1.0 3.2))
      (Utilities|FlowControl|Sequence
        (:then_0
          (Timeline|CamCrouch PlayFromStart
            (:Update
              (CallFunction|MoveCam (Variables|Default|GetInterestPoint2)))))
        (:then_1
          (Utilities|FlowControl|Delay 0.2)
          (Default|ObjectInteractAnimationin _character "NewEnumerator15"))
        (:then_2
          (Utilities|FlowControl|Delay 2.5)
          (CallFunction|BreakCamCrouch)
          (Transformation|DetachFromComponent (Variables|/Game/Blueprints/Bluperints/BP_Character.BP_Character_C|GetMesh2P (Variables|Default|GetCharacter)) "KeepWorld" "KeepWorld" "KeepWorld" true)
          (Transformation|AttachComponentToComponent (Variables|/Game/Blueprints/Bluperints/BP_Character.BP_Character_C|GetMesh2P _character_2) (Variables|/Script/Engine.Character|GetCapsuleComponent _character_2) "None" "KeepWorld" "KeepWorld" "KeepWorld" true)
          (Default|StartFighting (Variables|Default|GetDeadSailor))
          (Utilities|FlowControl|Delay 0.15)
          (Default|PlayMonolog (Variables|Default|GetdialogManager) 33 0.0)
          (CallFunction|MovePlayer 0.1 (Variables|Default|GetPositionPoint2) (Variables|Default|GetInterestPoint3))
          (CallFunction|ShowInput)
          (CallFunction|AcceptInput)
          (bind _returnvalue (Utilities|Time|SetTimerbyFunctionName 0 "Fail" (Utilities|Array|Get(acopy) (Variables|Default|GetInteractionsDurations) (Variables|Default|GetCurrentInteraction)))))))))

(event EventSuccess
  (bind _character (Variables|Default|GetCharacter))
  (bind _dialogmanager (Variables|Default|GetdialogManager))
  (bind _dialogmanager_2 (Variables|Default|GetdialogManager))
  (bind _character_2 (Variables|Default|GetCharacter))
  (bind _character_3 (Variables|Default|GetCharacter))
  (bind _abp_character (Variables|/Game/Blueprints/Bluperints/BP_Character.BP_Character_C|GetABP_Character _character))
  (Utilities|Time|ClearandInvalidateTimerbyHandle (stale Custom|AfterBreak _returnvalue))
  (switch int (Variables|Default|GetCurrentInteraction)
    (:0
      (CallFunction|HideInput)
      (Transformation|DetachFromComponent (Variables|/Game/Blueprints/Bluperints/BP_Character.BP_Character_C|GetMesh2P (Variables|Default|GetCharacter)) "KeepWorld" "KeepWorld" "KeepWorld" true)
      (Default|QTECameraControlMove (Variables|Default|GetCharacter) 0.3 (Transformation|GetWorldLocation (Variables|Default|GetInterestPoint4)))
      (Utilities|FlowControl|Delay 0.5)
      (Default|QTECameraControlMove (Variables|Default|GetCharacter) 0.3 (Transformation|GetWorldLocation (Variables|Default|GetInterestPoint5)))
      (Utilities|FlowControl|Delay 0.3)
      (Default|ObjectInteractAnimationin (Variables|Default|GetCharacter) "NewEnumerator17")
      (Utilities|FlowControl|Delay 0.1)
      (Transformation|AttachComponentToComponent (Variables|Default|GetRock) (Variables|/Game/Blueprints/Bluperints/BP_Character.BP_Character_C|GetMesh2P (Variables|Default|GetCharacter)) "RightAttachPoint" "SnapToTarget" "SnapToTarget" "KeepWorld" true)
      (Transformation|SetRelativeLocation (Variables|/Game/Blueprints/Bluperints/BP_Rock.BP_Rock_C|GetRock (Variables|Default|GetRock)) "0,7.500000, 0" false false)
      (Default|QTECameraControlMove (Variables|Default|GetCharacter) 0.5 (Transformation|GetWorldLocation (Variables|Default|GetInterestPoint3)))
      (Utilities|FlowControl|Delay 0.5)
      (Default|TakeHit (Variables|Default|GetDeadSailor))
      (Variables|/Game/DefaultContent/FirstPerson/Animations/ABP_Character.ABP_Character_C|SetisGrabbingMedal _abp_character false)
      (Variables|/Game/DefaultContent/FirstPerson/Animations/ABP_Character.ABP_Character_C|SetisGrabbingRock _abp_character false)
      (Default|Grab (Variables|Default|GetMedal) (Variables|/Game/Blueprints/Bluperints/BP_Character.BP_Character_C|GetMesh2P (Variables|Default|GetCharacter)))
      (Utilities|FlowControl|Delay 1.0)
      (Default|PlayMonolog _dialogmanager_2 36 0.0)
      (Utilities|FlowControl|Delay (+ (Variables|/Script/Engine.SoundBase|GetDuration (.lineaudio (Utilities|Array|Get(acopy) (Variables|/Game/Blueprints/Bluperints/BP_DialogManager.BP_DialogManager_C|GetDialogsDay3 _dialogmanager_2) 36))) 3.0))
      (Default|CamCrouch (Variables|Default|GetCharacter) 0.5 false)
      (Default|QTECameraControlMove (Variables|Default|GetCharacter) 0.2 (Transformation|GetWorldLocation (Variables|Default|GetInterestPoint6)))
      (Utilities|FlowControl|Delay 0.1)
      (Default|WalktheRail (Variables|Default|GetSuccessRail))
      (Utilities|FlowControl|Delay 1.0)
      (Transformation|AttachComponentToComponent (Variables|/Game/Blueprints/Bluperints/BP_Character.BP_Character_C|GetMesh2P _character_3) (Variables|/Game/Blueprints/Bluperints/BP_Character.BP_Character_C|GetFirstPersonCamera _character_3) "None" "KeepWorld" "KeepWorld" "KeepWorld" true)
      (Default|QTECameraControlMove (Variables|Default|GetCharacter) 0.3 (Transformation|GetWorldLocation (Variables|Default|GetInterestPoint7)))
      (Default|PlayMonolog _dialogmanager 38 0.0)
      (Utilities|FlowControl|Delay (+ (Variables|/Script/Engine.SoundBase|GetDuration (.lineaudio (Utilities|Array|Get(acopy) (Variables|/Game/Blueprints/Bluperints/BP_DialogManager.BP_DialogManager_C|GetDialogsDay3 _dialogmanager) 38))) 1.0))
      (Actor|DestroyActor (Variables|Default|GetRock))
      (Default|FinishCamFall (Variables|Default|GetCharacter))
      (Default|ObjectZoomin _character_2)
      (Utilities|FlowControl|Delay 3.0)
      (Default|ObjectZoomOut _character_2)
      (CallFunction|StartStopQTE false)
      (Default|ChangeSanity (Variables|Default|GetCharacter) false)
      (bind _outactors (Actor|GetAllActorsOfClass "/Game/Blueprints/Bluperints/BP_LevelManager.BP_LevelManager_C"))
      (Default|ProblemResolution (Utilities|Array|Get(acopy) _outactors) 22 0.0)
      (Variables|/Game/Blueprints/Bluperints/BP_LevelManager.BP_LevelManager_C|SethasKilledTheSailor (Utilities|Array|Get(acopy) _outactors) true))))

(event EventFail
  (bind _dialogmanager (Variables|Default|GetdialogManager))
  (switch int (Variables|Default|GetCurrentInteraction)
    (:0
      (CallFunction|HideInput)
      (Default|Grab (Variables|Default|GetMedal) (Variables|/Game/Blueprints/Bluperints/BP_Character.BP_Character_C|GetMesh2P (Variables|Default|GetCharacter)))
      (Variables|/Game/DefaultContent/FirstPerson/Animations/ABP_Character.ABP_Character_C|SetisGrabbingMedal (Variables|/Game/Blueprints/Bluperints/BP_Character.BP_Character_C|GetABP_Character (Variables|Default|GetCharacter)) false)
      (Default|Die (Variables|Default|GetDeadSailor))
      (CallFunction|MovePlayer 0.5 (Variables|Default|GetFailPositionPoint) (Variables|Default|GetInterestPoint))
      (Utilities|FlowControl|Delay 1.5)
      (Default|PlayMonolog _dialogmanager 34 0.0)
      (Utilities|FlowControl|Delay (+ (Variables|/Script/Engine.SoundBase|GetDuration (.lineaudio (Utilities|Array|Get(acopy) (Variables|/Game/Blueprints/Bluperints/BP_DialogManager.BP_DialogManager_C|GetDialogsDay3 _dialogmanager) 34))) 1.0))
      (Default|CamCrouch (Variables|Default|GetCharacter) 2.0 false)
      (Utilities|FlowControl|Delay 2.0)
      (Default|ObjectZoomin (Variables|Default|GetCharacter))
      (Utilities|FlowControl|Delay 2.0)
      (Default|ObjectZoomOut (Variables|Default|GetCharacter))
      (CallFunction|StartStopQTE false)
      (bind _outactors (Actor|GetAllActorsOfClass "/Game/Blueprints/Bluperints/BP_LevelManager.BP_LevelManager_C"))
      (Default|ProblemResolution (Utilities|Array|Get(acopy) _outactors) 22 0.0)
      (Variables|/Game/Blueprints/Bluperints/BP_LevelManager.BP_LevelManager_C|SethasKilledTheSailor (Utilities|Array|Get(acopy) _outactors) false))))

(fn ConstructionScript
  (|CallParentFunction))