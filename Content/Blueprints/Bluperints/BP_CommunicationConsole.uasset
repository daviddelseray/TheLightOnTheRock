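; Communication console that rings with a blinking light and sound until the player answers or SystemAnswer picks up without the interact animation.
; StartCall opens a Gate that Ring passes through, re-calling itself to loop until AnswerCall closes it.
; Answering branches on LevelManager's current day: day 1 starts an Archibald dialog through DialogManager, later days drive the FuseBox (activation with problem resolution, then looping Morse).
; As interlocutor, it plays line audio and sets HUD subtitles.
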(event Custom|SystemAnswer
  (bind _fusebox (Variables|Default|GetFuseBox))
  (bind _character (Variables|Default|GetCharacter))
  (bind _dialogmanager (Variables|Default|GetDialogManager))
  (CallFunction|AnswerCall)
  (Variables|/Game/Blueprints/Bluperints/BP_Character.BP_Character_C|SetisDialoging _character true)
  (Variables|/Game/Blueprints/Bluperints/BP_Character.BP_Character_C|SetLookAtPoint _character (Transformation|GetWorldLocation (Variables|Default|GetLookAtPoint)))
  (switch int (Variables|/Game/Blueprints/Bluperints/BP_LevelManager.BP_LevelManager_C|GetCurrentDay (Variables|Default|GetLevelManager))
    (:1
      (Variables|/Game/Blueprints/Bluperints/BP_DialogManager.BP_DialogManager_C|SetCurrentDialog _dialogmanager (Variables|/Game/Blueprints/Bluperints/BP_DialogManager.BP_DialogManager_C|GetDay1ArchibaldConsoleDialog _dialogmanager))
      (Variables|/Game/Blueprints/Bluperints/BP_DialogManager.BP_DialogManager_C|SetCurrentQuestion _dialogmanager (Variables|/Game/Blueprints/Bluperints/BP_DialogManager.BP_DialogManager_C|GetDay1ArchibaldConsoleQuestions _dialogmanager))
      (Variables|/Game/Blueprints/Bluperints/BP_DialogManager.BP_DialogManager_C|SetInterlocutor _dialogmanager self)
      (Default|DefineLine _dialogmanager))
    (:2
      (Variables|/Game/Blueprints/Bluperints/BP_Character.BP_Character_C|SetisDialoging (Variables|Default|GetCharacter) false)
      (Default|Activate (Variables|Default|GetFuseBox))
      (Default|ProblemResolution (Variables|Default|GetLevelManager) 15 0.0))
    (:3
      (Variables|/Game/Blueprints/Bluperints/BP_Character.BP_Character_C|SetisDialoging (Variables|Default|GetCharacter) false)
      (Variables|/Game/Blueprints/Bluperints/BP_Fusebox.BP_Fusebox_C|SetshouldLoop? _fusebox true)
      (Default|LoopPlayMorse _fusebox))))

(event Custom|Ring
  (params (ConsoleFirst :type Boolean))
  (bind _speaker (Variables|Default|GetSpeaker))
  (bind _output_get (Variables|Default|SetConsoleTalksFirst ConsoleFirst))
  (Utilities|FlowControl|Gate true
    (:Exit
      (Rendering|SetVisibility (Variables|Default|GetBlinker) true false)
      (Audio|Components|Audio|SetSound _speaker "/Game/StarterContent/Audio/Explosion_Cue.Explosion_Cue")
      (Audio|Components|Audio|Play _speaker 0.0)
      (Utilities|FlowControl|Delay (Variables|Default|GetBlinkingDelay))
      (Rendering|SetVisibility (Variables|Default|GetBlinker) false false)
      (Utilities|FlowControl|Delay (Variables|Default|GetBlinkingDelay))
      (CallFunction|Ring _output_get))))

(event Custom|AnswerCall
  (bind _speaker (Variables|Default|GetSpeaker))
  (Audio|Components|Audio|Stop (Variables|Default|GetSpeaker))
  (Rendering|SetVisibility (Variables|Default|GetBlinker) false false)
  (if (Variables|Default|GetisRinging)
    (Variables|Default|SetisRinging false)
    (Default|HideInteractions (Variables|Default|GetCharacter) false true)
    (Utilities|FlowControl|Gate true) ; enters at Close
  ))

(event Custom|StartCall
  (bind _speaker (Variables|Default|GetSpeaker))
  (if (not (Variables|Default|GetisRinging))
    (Variables|Default|SetisRinging true)
    (Utilities|FlowControl|Gate true) ; enters at Open
  ))

(event EventBeginPlay
  (bind _asbp_character (Utilities|Casting|CastToBP_Character (Game|GetPlayerCharacter 0)))
  (Variables|Default|SetCharacter _asbp_character)
  (bind _outactors (Actor|GetAllActorsOfClass "/Game/Blueprints/Bluperints/BP_DialogManager.BP_DialogManager_C"))
  (Variables|Default|SetDialogManager (Utilities|Array|Get(acopy) _outactors)))

(event Collision|EventActorBeginOverlap
  (params (OtherActor :type Actor%20Object%20Reference)))

(event EventTick
  (params (DeltaSeconds :type Float%20%28single-precision%29)))

(event EventInteract
  (bind _character (Variables|Default|GetCharacter))
  (bind _fusebox (Variables|Default|GetFuseBox))
  (bind _character_2 (Variables|Default|GetCharacter))
  (bind _dialogmanager (Variables|Default|GetDialogManager))
  (if (Variables|Default|GetisRinging)
    (Default|ObjectInteractAnimationin _character "NewEnumerator7")
    (bind _duration (Default|GetAnimDuration (Variables|/Game/Blueprints/Bluperints/BP_Character.BP_Character_C|GetAnimationContainer _character) "NewEnumerator7"))
    (Utilities|FlowControl|Delay (* _duration 0.8))
    (Variables|/Game/DefaultContent/FirstPerson/Animations/ABP_Character.ABP_Character_C|SetAnsweringCall (Variables|/Game/Blueprints/Bluperints/BP_Character.BP_Character_C|GetABP_Character (Variables|Default|GetCharacter)) false)
    (CallFunction|AnswerCall)
    (Variables|/Game/Blueprints/Bluperints/BP_Character.BP_Character_C|SetisDialoging _character_2 true)
    (Variables|/Game/Blueprints/Bluperints/BP_Character.BP_Character_C|SetLookAtPoint _character_2 (Transformation|GetWorldLocation (Variables|Default|GetLookAtPoint)))
    (switch int (Variables|/Game/Blueprints/Bluperints/BP_LevelManager.BP_LevelManager_C|GetCurrentDay (Variables|Default|GetLevelManager))
      (:1
        (Variables|/Game/Blueprints/Bluperints/BP_DialogManager.BP_DialogManager_C|SetCurrentDialog _dialogmanager (Variables|/Game/Blueprints/Bluperints/BP_DialogManager.BP_DialogManager_C|GetDay1ArchibaldConsoleDialog _dialogmanager))
        (Variables|/Game/Blueprints/Bluperints/BP_DialogManager.BP_DialogManager_C|SetCurrentQuestion _dialogmanager (Variables|/Game/Blueprints/Bluperints/BP_DialogManager.BP_DialogManager_C|GetDay1ArchibaldConsoleQuestions _dialogmanager))
        (Variables|/Game/Blueprints/Bluperints/BP_DialogManager.BP_DialogManager_C|SetInterlocutor _dialogmanager self)
        (Default|DefineLine _dialogmanager))
      (:2
        (Variables|/Game/Blueprints/Bluperints/BP_Character.BP_Character_C|SetisDialoging (Variables|Default|GetCharacter) false)
        (Default|Activate (Variables|Default|GetFuseBox))
        (Default|ProblemResolution (Variables|Default|GetLevelManager) 15 0.0))
      (:3
        (Variables|/Game/Blueprints/Bluperints/BP_Character.BP_Character_C|SetisDialoging (Variables|Default|GetCharacter) false)
        (Variables|/Game/Blueprints/Bluperints/BP_Fusebox.BP_Fusebox_C|SetshouldLoop? _fusebox true)
        (Default|LoopPlayMorse _fusebox)))))

(event EventRevealInteractions
  (if (Variables|Default|GetisRinging)
    (Default|ShowInteractions (Variables|Default|GetCharacter) "Answer" false)))

(event EventPlaySound
  (params (Sound :type Sound%20Cue%20Object%20Reference))
  (CallFunction|PlayLineSound Sound))

(fn ConstructionScript)

(fn PlayLineSound
  (params (Sound :type Sound%20Cue%20Object%20Reference))
  (Utilities|IsValid Sound
    (:Is%20Valid
      (Audio|Components|Audio|SetSound (Variables|Default|GetSpeaker) Sound)
      (Audio|Components|Audio|Play (Variables|Default|GetSpeaker) 0.0))))

(fn DisplayLineSubtitle
  (params (Subtitle :type String))
  (bind _asbp_character (Utilities|Casting|CastToBP_Character (Game|GetPlayerCharacter 0)))
  (Widget|SetVisibility (Variables|/Game/Blueprints/Bluperints/BP_Character.BP_Character_C|GetMainHUD _asbp_character) "Visible")
  (Variables|/Game/Widgets/W_MainHUD.W_MainHUD_C|SetSubtitle (Variables|/Game/Blueprints/Bluperints/BP_Character.BP_Character_C|GetMainHUD _asbp_character) Subtitle))