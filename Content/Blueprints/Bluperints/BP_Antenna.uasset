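; Breakable antenna that the player repairs through a button-mashing QTE shown on the level manager's QTE HUD.
; Each Interact adds progress, by a separate increment when the character is hurt, while Tick drains it.
; Progress thresholds advance one-way stages, each restarting a timeline that lerps the pivot further over.
; The final stage detaches the pivot, enables antenna physics, restores the main HUD and can resolve a day-specific level problem.
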(event Custom|Break
  (Transformation|SetRelativeRotation (Variables|Default|GetAntennaPivotPoint) "0, 0, 0" false false)
  (Variables|Default|SetisBroken true))

(event Custom|Repairing
  (if (Variables|/Game/Blueprints/Bluperints/BP_Character.BP_Character_C|GetisHurt (Variables|Default|GetCharacter))
    (Variables|Default|SetRepairPercent (+ (Variables|Default|GetRepairPercent) (Variables|Default|GethurtRepairIncrement)))
    (else
      (Variables|Default|SetRepairPercent (+ (Variables|Default|GetRepairPercent) (Variables|Default|GetRepairIncrement)))))
  (if (>= (Variables|Default|GetRepairPercent) 3e+01)
    (if (>= (Variables|Default|GetRepairingStage) 1)
      _
      (else
        (Variables|Default|SetRepairingStage 1)
        (CallFunction|MoveAntenna)))
    (if (>= (Variables|Default|GetRepairPercent) 6e+01)
      (if (>= (Variables|Default|GetRepairingStage) 2)
        _
        (else
          (Variables|Default|SetRepairingStage 2)
          (CallFunction|MoveAntenna)))
      (if (>= (Variables|Default|GetRepairPercent) 9e+01)
        (if (>= (Variables|Default|GetRepairingStage) 3)
          _
          (else
            (Variables|Default|SetRepairingStage 3)
            (CallFunction|MoveAntenna)))
        (if (>= (Variables|Default|GetRepairPercent) 1e+02)
          (Variables|Default|SetRepairingStage 4)
          (CallFunction|MoveAntenna)
          (Variables|Default|SetisBroken false)
          (Variables|/Game/Widgets/W_QTEHUD.W_QTEHUD_C|SetInputImageVisibility (Variables|/Game/Blueprints/Bluperints/BP_LevelManager.BP_LevelManager_C|GetQTEHUD (Variables|Default|GetlevelManager)) "Hidden"))))))

(event Custom|MoveAntenna
  (bind _levelmanager (Variables|Default|GetlevelManager))
  (bind _levelmanager_2 (Variables|Default|GetlevelManager))
  (bind _qtehud (Variables|/Game/Blueprints/Bluperints/BP_LevelManager.BP_LevelManager_C|GetQTEHUD _levelmanager))
  (Variables|Default|SetTempRot (Variables|/Script/Engine.SceneComponent|GetRelativeRotation (Variables|Default|GetAntennaPivotPoint)))
  (CallFunction|StopPrevRot)
  (switch int (Variables|Default|GetRepairingStage)
    (:1
      (Variables|Default|SetTargetRotation "15.000000, 0, 0")
      (bind _lerpalpha (Timeline|Rotation PlayFromStart)
        (:Update
          (Transformation|SetRelativeRotation (Variables|Default|GetAntennaPivotPoint) (Math|Rotator|Lerp(Rotator) (Variables|Default|GetTempRot) (Variables|Default|GetTargetRotation) _lerpalpha true) false false))
        (:Finished
          (if (== (Variables|Default|GetRepairingStage) 4)
            (Transformation|DetachFromComponent (Variables|Default|GetAntennaPivotPoint) "KeepWorld" "KeepWorld" "KeepWorld" true)
            (Physics|SetSimulatePhysics (Variables|Default|GetAntenna) true)
            (Variables|Default|SetisGettingRepaired false)
            (Variables|/Game/Widgets/W_QTEHUD.W_QTEHUD_C|SetisPowerInteracting _qtehud false)
            (Widget|SetVisibility _qtehud "Hidden")
            (Widget|SetVisibility (Variables|/Game/Blueprints/Bluperints/BP_LevelManager.BP_LevelManager_C|GetMainHUD _levelmanager) "Visible")
            (if (and (== (Variables|/Game/Blueprints/Bluperints/BP_LevelManager.BP_LevelManager_C|GetCurrentDay _levelmanager_2) 3) (== (Variables|/Game/Blueprints/Bluperints/BP_LevelManager.BP_LevelManager_C|GetCurrentProblem _levelmanager_2) 3))
              (Default|ProblemResolution (Variables|Default|GetlevelManager) 4 0.0))))))
    (:2
      (Variables|Default|SetTargetRotation "30.000000, 0, 0")
      (Timeline|Rotation PlayFromStart))
    (:3
      (Variables|Default|SetTargetRotation "50.000000, 0, 0")
      (Timeline|Rotation PlayFromStart))
    (:4
      (Variables|Default|SetTargetRotation "90.000000, 0, 0")
      (Timeline|Rotation PlayFromStart))))

(event Custom|StopPrevRot
  (bind _levelmanager (Variables|Default|GetlevelManager))
  (bind _levelmanager_2 (Variables|Default|GetlevelManager))
  (bind _qtehud (Variables|/Game/Blueprints/Bluperints/BP_LevelManager.BP_LevelManager_C|GetQTEHUD _levelmanager))
  (bind _lerpalpha (Timeline|Rotation Stop)
    (:Update
      (Transformation|SetRelativeRotation (Variables|Default|GetAntennaPivotPoint) (Math|Rotator|Lerp(Rotator) (Variables|Default|GetTempRot) (Variables|Default|GetTargetRotation) _lerpalpha true) false false))
    (:Finished
      (if (== (Variables|Default|GetRepairingStage) 4)
        (Transformation|DetachFromComponent (Variables|Default|GetAntennaPivotPoint) "KeepWorld" "KeepWorld" "KeepWorld" true)
        (Physics|SetSimulatePhysics (Variables|Default|GetAntenna) true)
        (Variables|Default|SetisGettingRepaired false)
        (Variables|/Game/Widgets/W_QTEHUD.W_QTEHUD_C|SetisPowerInteracting _qtehud false)
        (Widget|SetVisibility _qtehud "Hidden")
        (Widget|SetVisibility (Variables|/Game/Blueprints/Bluperints/BP_LevelManager.BP_LevelManager_C|GetMainHUD _levelmanager) "Visible")
        (if (and (== (Variables|/Game/Blueprints/Bluperints/BP_LevelManager.BP_LevelManager_C|GetCurrentDay _levelmanager_2) 3) (== (Variables|/Game/Blueprints/Bluperints/BP_LevelManager.BP_LevelManager_C|GetCurrentProblem _levelmanager_2) 3))
          (Default|ProblemResolution (Variables|Default|GetlevelManager) 4 0.0))))))

(event EventBeginPlay
  (bind _asbp_character (Utilities|Casting|CastToBP_Character (Game|GetPlayerCharacter 0)))
  (Variables|Default|SetCharacter _asbp_character)
  (bind _outactors (Actor|GetAllActorsOfClass "/Game/Blueprints/Bluperints/BP_LevelManager.BP_LevelManager_C"))
  (Variables|Default|SetlevelManager (Utilities|Array|Get(acopy) _outactors)))

(event Collision|EventActorBeginOverlap
  (params (OtherActor :type Actor%20Object%20Reference)))

(event EventTick
  (params (DeltaSeconds :type Float%20%28single-precision%29))
  (if (Variables|Default|GetisGettingRepaired)
    (Variables|Default|SetRepairPercent (Math|Float|Clamp(Float) (- (Variables|Default|GetRepairPercent) (Variables|Default|GetRepairDecrease)) 0.0 1e+02))))

(event EventInteract
  (bind _levelmanager (Variables|Default|GetlevelManager))
  (bind _qtehud (Variables|/Game/Blueprints/Bluperints/BP_LevelManager.BP_LevelManager_C|GetQTEHUD _levelmanager))
  (if (Variables|Default|GetisBroken)
    (if (Variables|Default|GetisGettingRepaired)
      (CallFunction|Repairing)
      (else
        (Variables|Default|SetisGettingRepaired true)
        (Widget|SetVisibility (Variables|/Game/Blueprints/Bluperints/BP_Character.BP_Character_C|GetMainHUD (Variables|Default|GetCharacter)) "Hidden")
        (Widget|SetVisibility _qtehud "Visible")
        (Default|MoveBands _qtehud true)
        (Utilities|FlowControl|Delay 1.0)
        (Variables|/Game/Widgets/W_QTEHUD.W_QTEHUD_C|SetInputImage _qtehud "/Game/David2DAssets/HUD/QTE_E.QTE_E")
        (Variables|/Game/Widgets/W_QTEHUD.W_QTEHUD_C|SetInputImageVisibility _qtehud "Visible")
        (Variables|/Game/Widgets/W_QTEHUD.W_QTEHUD_C|SetisPowerInteracting _qtehud true)
        (Default|PowerInteract _qtehud)))))

(event EventRevealInteractions
  (if (Variables|Default|GetisBroken)
    (Default|ShowInteractions (Variables|Default|GetCharacter) "Repair the antenna" false)))

(fn ConstructionScript)