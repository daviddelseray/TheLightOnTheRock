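; BP_InterestPoint is a gaze target that reports to the level manager when the player looks toward it.
; While IsTracking is set, Tick measures the angle between the first-person camera's forward vector and the direction from the character's capsule to the Sphere.
; Every frame that angle is under Tolerance, it calls ProblemResolution on the first BP_LevelManager found, passing ParentTrigger's EventRequired.
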(event EventBeginPlay)

(event Collision|EventActorBeginOverlap
  (params (OtherActor :type Actor%20Object%20Reference)))

(event EventTick
  (params (DeltaSeconds :type Float%20%28single-precision%29))
  (if (Variables|Default|GetisTracking)
    (bind _asbp_character (Utilities|Casting|CastToBP_Character (Game|GetPlayerCharacter 0)))
    (if (< (Utilities|AngleBetweenVector (Math|Vector|GetForwardVector (Variables|/Game/Blueprints/Bluperints/BP_Character.BP_Character_C|GetFirstPersonCamera _asbp_character)) (- (Transformation|GetWorldLocation (Variables|Default|GetSphere)) (Transformation|GetWorldLocation (Variables|/Script/Engine.Character|GetCapsuleComponent _asbp_character)))) (Variables|Default|GetTolerance))
      (bind _outactors (Actor|GetAllActorsOfClass "/Game/Blueprints/Bluperints/BP_LevelManager.BP_LevelManager_C"))
      (Default|ProblemResolution (Utilities|Array|Get(acopy) _outactors) (Variables|/Game/Blueprints/Bluperints/BP_Triger.BP_Triger_C|GetEventRequired (Variables|Default|GetParentTrigger)) 0.0))))

(fn ConstructionScript)