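; BP_CharacterRailWalk moves the player's BP_Character along a spline rail for scripted walks.
; GetToRail runs a timeline that lerps the capsule from its current location toward the first spline point, switching to WalkTheRail once within tolerance.
; A second timeline maps progress to spline distance, with events to pause, resume or walk back from the end over a given duration.
; Walk events also drive the character's IsMoving flag and footsteps.
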(event Custom|WalkTheRail
  (bind _character (Variables|Default|GetCharacter))
  (Components|Timeline|SetPlayRate (Variables|Default|GetGoAlongRail) (/ 1.0 (Variables|Default|GetMoveAlongRailTime)))
  (Variables|/Game/Blueprints/Bluperints/BP_Character.BP_Character_C|SetisMoving _character true)
  (Default|PlayFootsteps _character)
  (bind _positionalongrail (Timeline|GoAlongRail PlayFromStart)
    (:Update
      (CallFunction|MoveAlongRail _positionalongrail))
    (:Finished
      (Variables|/Game/Blueprints/Bluperints/BP_Character.BP_Character_C|SetisMoving (Variables|Default|GetCharacter) false))))

(event Custom|GetToRail
  (Components|Timeline|SetPlayRate (Variables|Default|GetGoToRail) (/ 1.0 (Variables|Default|GetGetToRailTime)))
  (bind _lerpalpha (Timeline|GoToRail PlayFromStart)
    (:Update
      (CallFunction|MovePlayertoRail _lerpalpha))))

(event Custom|BreakGetToRail
  (Utilities|FlowControl|Sequence
    (:then_0
      (bind _lerpalpha (Timeline|GoToRail Stop)
        (:Update
          (CallFunction|MovePlayertoRail _lerpalpha))))
    (:then_1
      (CallFunction|WalktheRail))))

(event Custom|PauseInWalk
  (Variables|/Game/Blueprints/Bluperints/BP_Character.BP_Character_C|SetisMoving (Variables|Default|GetCharacter) false)
  (bind _positionalongrail (Timeline|GoAlongRail Stop)
    (:Update
      (CallFunction|MoveAlongRail _positionalongrail))
    (:Finished
      (Variables|/Game/Blueprints/Bluperints/BP_Character.BP_Character_C|SetisMoving (Variables|Default|GetCharacter) false))))

(event Custom|ResumeWalk
  (bind _character (Variables|Default|GetCharacter))
  (Variables|/Game/Blueprints/Bluperints/BP_Character.BP_Character_C|SetisMoving _character true)
  (Default|PlayFootsteps _character)
  (bind _positionalongrail (Timeline|GoAlongRail Play)
    (:Update
      (CallFunction|MoveAlongRail _positionalongrail))
    (:Finished
      (Variables|/Game/Blueprints/Bluperints/BP_Character.BP_Character_C|SetisMoving (Variables|Default|GetCharacter) false))))

(event Custom|WalkBackTheRail
  (params (MoveBackDuration :type Float%20%28single-precision%29))
  (bind _character (Variables|Default|GetCharacter))
  (Components|Timeline|SetPlayRate (Variables|Default|GetGoAlongRail) (/ 1.0 MoveBackDuration))
  (Variables|/Game/Blueprints/Bluperints/BP_Character.BP_Character_C|SetisMoving _character true)
  (Default|PlayFootsteps _character)
  (bind _positionalongrail (Timeline|GoAlongRail ReverseFromEnd)
    (:Update
      (CallFunction|MoveAlongRail _positionalongrail))
    (:Finished
      (Variables|/Game/Blueprints/Bluperints/BP_Character.BP_Character_C|SetisMoving (Variables|Default|GetCharacter) false))))

(event EventBeginPlay
  (bind _asbp_character (Utilities|Casting|CastToBP_Character (Game|GetPlayerCharacter 0)))
  (Variables|Default|SetCharacter _asbp_character))

(event Collision|EventActorBeginOverlap
  (params (OtherActor :type Actor%20Object%20Reference)))

(event EventTick
  (params (DeltaSeconds :type Float%20%28single-precision%29)))

(fn ConstructionScript)

(fn MovePlayertoRail
  (params (LerpAlpha :type Float%20%28single-precision%29))
  (Transformation|SetWorldLocation (Variables|/Script/Engine.Character|GetCapsuleComponent (Variables|Default|GetCharacter)) (Math|Vector|Lerp(Vector) (Transformation|GetWorldLocation (Variables|/Script/Engine.Character|GetCapsuleComponent (Variables|Default|GetCharacter))) (Spline|GetLocationatSplinePoint (Variables|Default|GetSpline) 0 "World") LerpAlpha) false false)
  (if (< (Math|Float|Absolute(Float) (Math|Vector|VectorLength (- (Spline|GetLocationatSplinePoint (Variables|Default|GetSpline) 0 "World") (Transformation|GetWorldLocation (Variables|/Script/Engine.Character|GetCapsuleComponent (Variables|Default|GetCharacter)))))) (Variables|Default|GetGetToRailApprox))
    (CallFunction|BreakGettoRail)))

(fn MoveAlongRail
  (params (PercentAlongSpline :type Float%20%28single-precision%29))
  (bind _spline (Variables|Default|GetSpline))
  (Transformation|SetWorldLocation (Variables|/Script/Engine.Character|GetCapsuleComponent (Variables|Default|GetCharacter)) (Spline|GetLocationatDistanceAlongSpline _spline (* PercentAlongSpline (Spline|GetSplineLength _spline)) "World") false false))