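; A spotlight mount that a character can watch from, interact with, or take the spotlight off.
; On BeginPlay it attaches itself to its Spotlight, initializes it and marks itself loaded.
; Its Box overlap sets the character's watch-point flag and reference on entry and clears the flag on exit.
; Grab hands over a loaded spotlight and empties the mount, Interact activates it while loaded, and Watch and GetOff toggle its tracking.
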(event OnComponentBeginOverlap(Box)
  (params (OverlappedComponent :type Primitive%20Component%20Object%20Reference) (OtherActor :type Actor%20Object%20Reference) (OtherComp :type Primitive%20Component%20Object%20Reference) (OtherBodyIndex :type Integer) (bFromSweep :type Boolean) (SweepResult :type Hit%20Result%20Structure%20%28by%20ref%29))
  (bind _asbp_character (Utilities|Casting|CastToBP_Character OtherActor))
  (Variables|/Game/Blueprints/Bluperints/BP_Character.BP_Character_C|SetatWatchPoint _asbp_character true)
  (Variables|/Game/Blueprints/Bluperints/BP_Character.BP_Character_C|SetWatchPoint _asbp_character self))

(event OnComponentEndOverlap(Box)
  (params (OverlappedComponent :type Primitive%20Component%20Object%20Reference) (OtherActor :type Actor%20Object%20Reference) (OtherComp :type Primitive%20Component%20Object%20Reference) (OtherBodyIndex :type Integer))
  (bind _asbp_character (Utilities|Casting|CastToBP_Character OtherActor))
  (Variables|/Game/Blueprints/Bluperints/BP_Character.BP_Character_C|SetatWatchPoint _asbp_character false))

(event EventBeginPlay
  (Variables|/Game/Blueprints/Bluperints/BP_WallWalkSpotlight.BP_WallWalkSpotlight_C|SetAttach (Variables|Default|GetSpotlight) self)
  (Default|Init (Variables|Default|GetSpotlight))
  (Variables|Default|SetisLoaded true))

(event Collision|EventActorBeginOverlap
  (params (OtherActor :type Actor%20Object%20Reference)))

(event EventTick
  (params (DeltaSeconds :type Float%20%28single-precision%29)))

(event EventWatch
  (Variables|/Game/Blueprints/Bluperints/BP_WallWalkSpotlight.BP_WallWalkSpotlight_C|SetisTracking (Variables|Default|GetSpotlight) true))

(event EventInteract
  (if (Variables|Default|GetisLoaded)
    (Default|Activate (Variables|Default|GetSpotlight))))

(event EventGetOff
  (Variables|/Game/Blueprints/Bluperints/BP_WallWalkSpotlight.BP_WallWalkSpotlight_C|SetisTracking (Variables|Default|GetSpotlight) false))

(event EventGrab
  (params (Character :type Skeletal%20Mesh%20Component%20Object%20Reference))
  (if (Variables|Default|GetisLoaded)
    (Default|Grab (Variables|Default|GetSpotlight) Character)
    (Variables|Default|SetisLoaded false)))

(fn ConstructionScript)