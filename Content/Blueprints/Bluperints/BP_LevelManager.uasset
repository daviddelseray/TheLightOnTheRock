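; BP_LevelManager runs the day-by-day story progression of a narrative game, with only Day 1 scripted.
; ProblemResolution feeds step indices into the Day1 switch, which fires monologues, objectives and world events, while DialogEvents maps dialogue events to following steps.
; BeginPlay loads SG_LevelManager save data and creates the HUDs shared with the character and DialogManager.
; Ellipse handles fade transitions, optional teleports and the between-days screen used by ChangeDay.
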(event Custom|Problem
  (params (Delay :type Float%20%28single-precision%29))
  (Utilities|FlowControl|Delay Delay)
  (switch int (Variables|ProgressionStates|GetCurrentDay)
    (:1
      (CallFunction|Day1))))

(event Custom|Ellipse
  (params (MoveAway :type Boolean) (NewLocation :type Vector) (NewRotation :type Rotator) (isBetweenDays :type Boolean) (Date :type String) (EventTrigerrer :type Boolean) (TimeToWait :type Float%20%28single-precision%29) (EventIndex :type Integer))
  ;[1 1 1] Ellipse between levels and during level
  (CameraFades|StartCameraFade :self (Game|GetPlayerCameraManager 0) :ToAlpha 1.0 :Duration 0.5 :bShouldFadeAudio true :bHoldWhenFinished true)
  (Utilities|FlowControl|Delay 0.5)
  (if MoveAway
    (Transformation|SetWorldLocationAndRotation (Variables|/Script/Engine.Character|GetCapsuleComponent (Variables|Default|GetCharacter)) NewLocation NewRotation false false))
  (if isBetweenDays
    (CallFunction|SetBetweenDaysUI Date)
    (bind _alpha (Timeline|AlphaTextLerp PlayFromStart)
      (:Update
        (Variables|/Game/Widgets/W_BetweenDaysUI.W_BetweenDaysUI_C|SetAlphaText (Variables|UI|GetBetweenDaysHUD) _alpha))
      (:Finished
        (Widget|SetVisibility (Variables|UI|GetBetweenDaysHUD) "Hidden")
        (CameraFades|StartCameraFade :self (Game|GetPlayerCameraManager 0) :FromAlpha 1.0 :Duration 0.5 :bShouldFadeAudio true :bHoldWhenFinished true :!label _label)
        (if EventTrigerrer
          (Utilities|FlowControl|Delay TimeToWait)
          (CallFunction|ProblemResolution EventIndex 0.0))))
    (else
      (Utilities|FlowControl|Delay 2.0)
      (goto _label))))

(event Custom|DisplayObjective
  (params (Delay :type Float%20%28single-precision%29))
  (bind _mainhud (Variables|UI|GetMainHUD))
  ;[1 1 1] GiveNewObjective
  (Utilities|FlowControl|Delay Delay)
  (Widget|SetVisibility _mainhud "Visible")
  (Default|DisplayObjective _mainhud (Variables|ProgressionStates|GetCurrentObjective)))

(event Custom|ProblemResolution
  (params (NextProblem :type Integer) (Delay :type Float%20%28single-precision%29))
  (Variables|ProgressionStates|SetCurrentProblem NextProblem)
  (CallFunction|Problem Delay))

(event EventBeginPlay
  ;[1 1 1] Create the HUDs, assign them and hide them
  (bind _asbp_character (Utilities|Casting|CastToBP_Character (Game|GetPlayerCharacter 0)))
  (Variables|Default|SetCharacter _asbp_character)
  (CallFunction|Load)
  (bind _returnvalue (UserInterface|CreateWidget "/Game/Widgets/W_MainHUD.W_MainHUD_C" (Game|GetPlayerController 0)))
  (bind _output_get (Variables|UI|SetMainHUD _returnvalue))
  (Variables|/Game/Blueprints/Bluperints/BP_DialogManager.BP_DialogManager_C|SetMainHUD (Variables|Actors|GetDialogManager) _returnvalue)
  (UserInterface|Viewport|AddtoViewport _output_get 0)
  (Variables|/Game/Blueprints/Bluperints/BP_Character.BP_Character_C|SetMainHUD (Variables|Default|GetCharacter) _output_get)
  (CallFunction|HideMainHUD)
  (bind _returnvalue_2 (UserInterface|CreateWidget "/Game/Widgets/W_DialogHUD.W_DialogHUD_C" (Game|GetPlayerController 0)))
  (bind _output_get_2 (Variables|UI|SetDialogHUD _returnvalue_2))
  (UserInterface|Viewport|AddtoViewport _output_get_2 0)
  (Variables|/Game/Blueprints/Bluperints/BP_DialogManager.BP_DialogManager_C|SetDialogueHUD (Variables|Actors|GetDialogManager) _returnvalue_2)
  (bind _output_get_3 (Variables|/Game/Blueprints/Bluperints/BP_Character.BP_Character_C|SetDialogHUD (Variables|Default|GetCharacter) _returnvalue_2))
  (Widget|SetVisibility _output_get_3 "Hidden")
  (bind _returnvalue_3 (UserInterface|CreateWidget "/Game/Widgets/W_BetweenDaysUI.W_BetweenDaysUI_C" (Game|GetPlayerController 0)))
  (bind _output_get_4 (Variables|UI|SetBetweenDaysHUD _returnvalue_3))
  (UserInterface|Viewport|AddtoViewport _output_get_4 0)
  (bind _output_get_5 (Variables|/Game/Blueprints/Bluperints/BP_Character.BP_Character_C|SetBetweenDaysHUD (Variables|Default|GetCharacter) _output_get_4))
  (Widget|SetVisibility _output_get_5 "Hidden")
  (bind _outactors (Actor|GetAllActorsOfClass "/Game/Blueprints/Bluperints/BP_LivingRat.BP_LivingRat_C"))
  (Variables|Actors|SetRodents _outactors))

(fn ConstructionScript)

(fn HideMainHUD
  (bind _mainhud (Variables|UI|GetMainHUD))
  (Widget|SetVisibility _mainhud "Visible")
  (Utilities|FlowControl|Sequence
    (:then_0
      (Variables|/Game/Widgets/W_MainHUD.W_MainHUD_C|SetAVisibility _mainhud "Hidden"))
    (:then_1
      (Variables|/Game/Widgets/W_MainHUD.W_MainHUD_C|SetInteractionAVisibility _mainhud "Hidden"))
    (:then_2
      (Variables|/Game/Widgets/W_MainHUD.W_MainHUD_C|SetEVisibility _mainhud "Hidden"))
    (:then_3
      (Variables|/Game/Widgets/W_MainHUD.W_MainHUD_C|SetEInteractionVisibility _mainhud "Hidden"))
    (:then_4
      (Variables|/Game/Widgets/W_MainHUD.W_MainHUD_C|SetRInteractionVisibility _mainhud "Hidden"))
    (:then_5
      (Variables|/Game/Widgets/W_MainHUD.W_MainHUD_C|SetRVisibility _mainhud "Hidden"))
    (:then_6
      (if (Variables|ProgressionStates|GetisCountdownVisible)
        (Variables|/Game/Widgets/W_MainHUD.W_MainHUD_C|SetCountdownDaysVisibility _mainhud "Visible")
        (Variables|/Game/Widgets/W_MainHUD.W_MainHUD_C|SetCountdownDays _mainhud (Utilities|String|ToString(Integer) (Variables|ProgressionStates|GetCountdownDays)))
        (else
          (Variables|/Game/Widgets/W_MainHUD.W_MainHUD_C|SetCountdownDaysVisibility _mainhud "Hidden"))))
    (:then_7
      (if (Variables|ProgressionStates|GetisSanityVisible)
        (Variables|/Game/Widgets/W_MainHUD.W_MainHUD_C|SetInsanityLevelVisibility _mainhud "Visible")
        (else
          (Variables|/Game/Widgets/W_MainHUD.W_MainHUD_C|SetInsanityLevelVisibility _mainhud "Visible"))))))

(fn Day1
  (bind _dialogmanager (Variables|Actors|GetDialogManager))
  (bind _generator (Variables|Actors|GetGenerator))
  (bind _triggers (Variables|Actors|GetTriggers))
  (bind _mainhud (Variables|UI|GetMainHUD))
  (bind _communicationconsole (Variables|Actors|GetCommunicationConsole))
  (switch int (Variables|ProgressionStates|GetCurrentProblem)
    (:0
      ;[1 1 1] 0-Started at the beginning of the day
      (Default|PlayMonolog (Variables|Actors|GetDialogManager)))
    (:1
      ;[1 1 1] 1-Started by the end of the intro monolog
      (Variables|ProgressionStates|SetCurrentObjective "Put a log in the wood burner of the lightroom")
      (CallFunction|DisplayObjective 0.0))
    (:2
      ;[1 1 1] 2-Started by placing a wood log in the wood burner
      (Default|PlayMonolog (Variables|Actors|GetDialogManager) 6))
    (:3
      ;[1 1 1] 3-Started by the ending of the previous event/monolog
      (Default|StartCall _communicationconsole)
      (Default|Ring _communicationconsole false))
    (:4
      ;[1 1 1] 4-Started by the ending of the call on the console
      (Default|Deactivate _generator)
      (Default|Rat _generator)
      (Variables|/Game/Blueprints/Bluperints/BP_Triger.BP_Triger_C|SetisOn (Utilities|Array|Get(acopy) (Variables|Actors|GetTriggers)) true)
      (for _array_element (Variables|Actors|GetRodents)
        (Default|Appear _array_element))
      (Default|Interact (Variables|Actors|GetLanternLever))
      (CallFunction|ProblemResolution 5 1.0))
    (:5
      ;[1 1 1] 5 - Triggered by the end of the previous Event (Shut down of the generator)
      (Default|PlayMonolog (Variables|Actors|GetDialogManager) 7)
      (Variables|ProgressionStates|SetCurrentObjective "Get the lantern in the bedroom")
      (CallFunction|DisplayObjective 2.0))
    (:6
      ;[1 1 1] 6-Triggered by grabbing the Lantern in the bedroom
      (Default|PlayMonolog (Variables|Actors|GetDialogManager) 8))
    (:7
      ;[1 1 1] 7-Started by the trigger in the stairs
      (Default|PlayMonolog (Variables|Actors|GetDialogManager) 9))
    (:8
      ;[1 1 1] 8-Triggered by the line of dialog said in previous event
      (Variables|ProgressionStates|SetCurrentObjective "Restart the generator")
      (CallFunction|DisplayObjective 0.0)
      (Default|PlayMonolog (Variables|Actors|GetDialogManager) 29))
    (:9
      ;[1 1 1] 9- Triggered when the player opens the door of the closet
      (Default|PlayMonolog (Variables|Actors|GetDialogManager) 10))
    (:10
      ;[1 1 1] 10-Triggered by reactivating the generator
      (Audio|SpawnSoundatLocation "/Game/StarterContent/Audio/Collapse_Cue.Collapse_Cue" "-345.000000,434.000000,2463.000000" "0, 0, 0" 1.0 1.0 0.0 0 0)
      (Default|PlayMonolog (Variables|Actors|GetDialogManager) 12)
      (Game|SpawnActorfromClass "/Game/Blueprints/Bluperints/BP_Countdown.BP_Countdown_C" (Math|Transform|MakeTransform "-318.351746,403.471100,2524.992676" "-90.000000,33.000000, 0" "1,1,1") "Undefined" 0 0)
      (bind _outactors (Actor|GetAllActorsOfClass "/Game/Blueprints/Bluperints/BP_Door.BP_Door_C"))
      (for _array_element_2 _outactors
        (if (Utilities|Enum|Equal(Enum) (Utilities|GetDisplayName _array_element_2) "BP_DoorToWallWalk")
          (Default|Open _array_element_2)
          (Variables|/Game/Blueprints/Bluperints/BP_Triger.BP_Triger_C|SetisOn (Utilities|Array|Get(acopy) _triggers 1) true)
          (Variables|/Game/Blueprints/Bluperints/BP_Triger.BP_Triger_C|SetisOn (Utilities|Array|Get(acopy) _triggers 2) true)
          (Variables|/Game/Blueprints/Bluperints/BP_Triger.BP_Triger_C|SetisOn (Utilities|Array|Get(acopy) _triggers 3) true)
          (Game|SpawnActorfromClass "/Game/Blueprints/Bluperints/BP_Rat.BP_Rat_C" (Math|Transform|MakeTransform "-412.400146,530.760559,17.041714" "0, 0,91.099808" "1,1,1") "Undefined" 0 0))))
    (:11
      ;[1 1 1] 11 - Triggered by finding the half eaten rat
      (Default|PlayMonolog (Variables|Actors|GetDialogManager) 14)
      (Variables|Day1Variables|SetHasSeenRat true))
    (:12
      ;[1 1 1] 12-Triggered by placing all the rat traps
      (Default|PlayMonolog (Variables|Actors|GetDialogManager) 28))
    (:13
      ;[1 1 1] 13-Triggered by reaching the lightroom
      (Default|PlayMonolog (Variables|Actors|GetDialogManager) 15))
    (:14
      ;[1 1 1] 14-Triggered by getting to the countdown
      (Default|PlayMonolog (Variables|Actors|GetDialogManager) 16))
    (:15
      ;[1 1 1] 15-Triggered by grabbing the countdown for the first time
      (Default|PlayMonolog (Variables|Actors|GetDialogManager) 17)
      (Variables|ProgressionStates|SetisCountdownVisible true)
      (Variables|/Game/Widgets/W_MainHUD.W_MainHUD_C|SetCountdownDaysVisibility _mainhud "Visible")
      (bind _output_get (Variables|ProgressionStates|SetCountdownDays 10))
      (Variables|/Game/Widgets/W_MainHUD.W_MainHUD_C|SetCountdownDays _mainhud (Utilities|String|ToString(Integer) _output_get))
      (bind _assg_level_manager (Utilities|Casting|CastToSG_LevelManager (Variables|Default|GetSaverSubClass)))
      (Variables|/Game/Blueprints/SaveGames/SG_LevelManager.SG_LevelManager_C|SetisCountDownVisible _assg_level_manager true)
      (Variables|/Game/Blueprints/SaveGames/SG_LevelManager.SG_LevelManager_C|SetCountdownDays _assg_level_manager 10))
    (:16
      ;[1 1 1] 16 - Triggered by the end of the previous event/ monolog
      (Audio|SpawnSoundatLocation "/Game/DAvid3DAssets/DavidTestSounds/Bells_Cue.Bells_Cue" "2782.103027,-5868.364258,-1606.452515" "0, 0, 0" 1.0 1.0 0.0 0 0)
      (CallFunction|ProblemResolution 17 3.0))
    (:17
      ;[1 1 1] 17- Triggered by restarting the lantern
      (Default|PlayMonolog (Variables|Actors|GetDialogManager) 18)
      (Variables|ProgressionStates|SetCurrentObjective "Restart the lantern")
      (CallFunction|DisplayObjective 0.0))
    (:18
      ;[1 1 1] 18- Triggered by the end of the last event/ Monolog
      (CallFunction|Ellipse false "1056.341919,-656.513062,2723.978760" "0,-20.552649, 0" false "" true 0.0 19))
    (:19
      ;[1 1 1] 19- Triggered by the end of the ellipse
      (Default|PlayMonolog (Variables|Actors|GetDialogManager) 19))
    (:20
      (if (Variables|Day1Variables|GetHasSeenRat)
        (Default|PlayMonolog _dialogmanager 25)
        (else
          (Default|PlayMonolog _dialogmanager 27))))
    (:21
      ;[1 1 1] 20- Triggered by the end of the outro monolog
      (CallFunction|ChangeDay "1056.341919,-656.513062,2723.978760" "0,-20.552649, 0"))))

(fn DialogEvents
  (params (EventIndex :type Integer))
  (switch int (Variables|ProgressionStates|GetCurrentDay)
    (:1
      (CallFunction|Day1DialogEvent EventIndex))))

(fn SetBetweenDaysUI
  (params (Date :type String))
  (bind _betweendayshud (Variables|UI|GetBetweenDaysHUD))
  (bind _betweendayshud_2 (Variables|UI|GetBetweenDaysHUD))
  (bind _betweendayshud_3 (Variables|UI|GetBetweenDaysHUD))
  (Widget|SetVisibility _betweendayshud "Visible")
  (if (Variables|ProgressionStates|GetisSanityVisible)
    (Variables|/Game/Widgets/W_BetweenDaysUI.W_BetweenDaysUI_C|SetSanityVisibility _betweendayshud "Visible")
    (Variables|/Game/Widgets/W_BetweenDaysUI.W_BetweenDaysUI_C|SetSanity (Variables|UI|GetBetweenDaysHUD) (Utilities|String|ToString(Integer) (Variables|/Game/Blueprints/Bluperints/BP_Character.BP_Character_C|GetSanityPoints (Variables|Default|GetCharacter))))
    (else
      (Variables|/Game/Widgets/W_BetweenDaysUI.W_BetweenDaysUI_C|SetSanityVisibility _betweendayshud "Hidden")))
  (if (Variables|ProgressionStates|GetisCountdownVisible)
    (Variables|/Game/Widgets/W_BetweenDaysUI.W_BetweenDaysUI_C|SetVisibilityCountdown _betweendayshud_2 "Visible")
    (Variables|/Game/Widgets/W_BetweenDaysUI.W_BetweenDaysUI_C|SetDaysLeft _betweendayshud_3 (Utilities|String|ToString(Integer) (Variables|ProgressionStates|GetCountdownDays)))
    (else
      (Variables|/Game/Widgets/W_BetweenDaysUI.W_BetweenDaysUI_C|SetVisibilityCountdown _betweendayshud_2 "Hidden")))
  (Variables|/Game/Widgets/W_BetweenDaysUI.W_BetweenDaysUI_C|SetDayDate _betweendayshud_3 Date)
  (Variables|/Game/Widgets/W_BetweenDaysUI.W_BetweenDaysUI_C|SetDayNumber _betweendayshud_3 (Utilities|String|ToString(Integer) (Variables|ProgressionStates|GetCurrentDay))))

(fn Load
  (bind _returnvalue (SaveGame|DoesSaveGameExist "SlotName"))
  (if _returnvalue
    ;[1 1 1] Executed everytime but the first time.
    (bind _returnvalue_2 (SaveGame|LoadGamefromSlot "SlotName"))
    (bind _output_get (Variables|Default|SetSaverSubClass _returnvalue_2))
    (bind _assg_level_manager (Utilities|Casting|CastToSG_LevelManager _output_get))
    (Variables|ProgressionStates|SetCountdownDays (Variables|/Game/Blueprints/SaveGames/SG_LevelManager.SG_LevelManager_C|GetCountdownDays _assg_level_manager))
    (Variables|ProgressionStates|SetCurrentDay (Variables|/Game/Blueprints/SaveGames/SG_LevelManager.SG_LevelManager_C|GetChapter _assg_level_manager))
    (Variables|/Game/Blueprints/Bluperints/BP_Character.BP_Character_C|SetSanityPoints (Variables|Default|GetCharacter) (Variables|/Game/Blueprints/SaveGames/SG_LevelManager.SG_LevelManager_C|GetSanityPoints _assg_level_manager))
    (Variables|ProgressionStates|SetisCountdownVisible (Variables|/Game/Blueprints/SaveGames/SG_LevelManager.SG_LevelManager_C|GetisCountDownVisible _assg_level_manager))
    (Variables|ProgressionStates|SetisSanityVisible (Variables|/Game/Blueprints/SaveGames/SG_LevelManager.SG_LevelManager_C|GetisSanityVisible _assg_level_manager))
    (else
      ;[1 1 1] Executed on the first game on this save. After that the Save Game object is kept all along
      (bind _returnvalue_3 (SaveGame|CreateSaveGameObject "/Game/Blueprints/SaveGames/SG_LevelManager.SG_LevelManager_C"))
      (bind _output_get_2 (Variables|Default|SetSaverSubClass _returnvalue_3))
      (bind _assg_level_manager_2 (Utilities|Casting|CastToSG_LevelManager _output_get_2))
      (Variables|/Game/Blueprints/SaveGames/SG_LevelManager.SG_LevelManager_C|SetCountdownDays _assg_level_manager_2 10)
      (Variables|/Game/Blueprints/SaveGames/SG_LevelManager.SG_LevelManager_C|SetChapter _assg_level_manager_2 0)
      (Variables|/Game/Blueprints/SaveGames/SG_LevelManager.SG_LevelManager_C|SetSanityPoints _assg_level_manager_2 6)
      (Variables|/Game/Blueprints/SaveGames/SG_LevelManager.SG_LevelManager_C|SetisCountDownVisible _assg_level_manager_2 false)
      (Variables|/Game/Blueprints/SaveGames/SG_LevelManager.SG_LevelManager_C|SetisSanityVisible _assg_level_manager_2 false)
      (SaveGame|SaveGametoSlot (Variables|Default|GetSaverSubClass) "SlotName"))))

(fn ChangeDay
  (params (NewLocation :type Vector) (NewRotation :type Rotator) (NewDate :type String))
  (Math|Integer|IncrementInt (Variables|ProgressionStates|GetCurrentDay)
    (:%20%20
      (CallFunction|Ellipse true NewLocation NewRotation true NewDate true 0.0)
      (Math|Integer|DecrementInt (Variables|ProgressionStates|GetCountdownDays)
        (:%20%20
          (SaveGame|SaveGametoSlot (Variables|Default|GetSaverSubClass) "SlotName"))))))

(fn Day1DialogEvent
  (params (Event :type Integer))
  (switch int Event
    (:0
      (CallFunction|ProblemResolution 1 0.0))
    (:1
      (CallFunction|ProblemResolution 3 0.0))
    (:2
      (CallFunction|ProblemResolution 4 0.0))
    (:3
      (CallFunction|ProblemResolution 8 0.0))
    (:4
      (CallFunction|ProblemResolution 16 0.0))
    (:5
      (CallFunction|ProblemResolution 18 0.0))
    (:6
      (CallFunction|ProblemResolution 20 0.0))
    (:7
      (CallFunction|ProblemResolution 21 0.0))))

(fn ResetSaveSlot
  (bind _assg_level_manager (Utilities|Casting|CastToSG_LevelManager (Variables|Default|GetSaverSubClass)))
  (Utilities|FlowControl|Sequence
    (:then_0
      (Variables|/Game/Blueprints/SaveGames/SG_LevelManager.SG_LevelManager_C|SetChapter _assg_level_manager 1))
    (:then_1
      (Variables|/Game/Blueprints/SaveGames/SG_LevelManager.SG_LevelManager_C|SetCountdownDays _assg_level_manager 10))
    (:then_2
      (Variables|/Game/Blueprints/SaveGames/SG_LevelManager.SG_LevelManager_C|SetSanityPoints _assg_level_manager 6))
    (:then_3
      (Variables|/Game/Blueprints/SaveGames/SG_LevelManager.SG_LevelManager_C|SetisCountDownVisible _assg_level_manager false))
    (:then_4
      (Variables|/Game/Blueprints/SaveGames/SG_LevelManager.SG_LevelManager_C|SetisSanityVisible _assg_level_manager false))
    (:then_5
      (SaveGame|SaveGametoSlot (Variables|Default|GetSaverSubClass) "SlotName"))))