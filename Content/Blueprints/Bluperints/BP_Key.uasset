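; BP_Key is a key actor that the player can pick up, carry and drop.
; Grab turns off physics, re-seats the Key component, attaches the actor to the passed Character's AttachPoint and records it as the player BP_Character's carried object.
; Release detaches it, clears that carry state and restores physics.
; Activate makes the key visible, while ShoePrintActivate reveals every DecalActor in the level, not just shoe prints.
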(event Custom|ShoePrintActivate
  (bind _outactors (Actor|GetAllActorsOfClass "/Script/Engine.DecalActor"))
  (for _array_element _outactors
    (Rendering|SetVisibility (Variables|/Script/Engine.DecalActor|GetDecal _array_element) true false)))

(event Custom|Activate
  (Rendering|SetVisibility (Variables|Default|GetKey) true false))

(event EventBeginPlay)

(event Collision|EventActorBeginOverlap
  (params (OtherActor :type Actor%20Object%20Reference)))

(event EventTick
  (params (DeltaSeconds :type Float%20%28single-precision%29)))

(event EventRelease
  (Transformation|SetRelativeLocation (Variables|Default|GetKey) "0, 0, 0" false false)
  (Transformation|DetachFromActor "KeepWorld" "KeepWorld" "KeepWorld")
  (bind _asbp_character (Utilities|Casting|CastToBP_Character (Game|GetPlayerCharacter 0)))
  (Variables|/Game/Blueprints/Bluperints/BP_Character.BP_Character_C|SetCaryObject _asbp_character false)
  (Variables|/Game/Blueprints/Bluperints/BP_Character.BP_Character_C|SetCarriedObject _asbp_character 0)
  (Physics|SetSimulatePhysics (Variables|Default|GetKey) true))

(event EventGrab
  (params (Character :type Skeletal%20Mesh%20Component%20Object%20Reference))
  (Transformation|AttachComponentToComponent (Variables|Default|GetKey) (Variables|Default|GetDefaultSceneRoot) "None" "SnapToTarget" "SnapToTarget" "KeepWorld" true)
  (Transformation|SetRelativeLocationAndRotation (Variables|Default|GetKey) "0.000000, 0,-1.000000" "-11.000000,55.000000,-15.000000" false false)
  (Physics|SetSimulatePhysics (Variables|Default|GetKey) false)
  (bind _asbp_character (Utilities|Casting|CastToBP_Character (Game|GetPlayerCharacter 0)))
  (Variables|/Game/Blueprints/Bluperints/BP_Character.BP_Character_C|SetCaryObject _asbp_character true)
  (Variables|/Game/Blueprints/Bluperints/BP_Character.BP_Character_C|SetCarriedObject _asbp_character self)
  (Transformation|AttachComponentToComponent Character "AttachPoint" "SnapToTarget" "SnapToTarget" "KeepWorld" false))

(fn ConstructionScript)