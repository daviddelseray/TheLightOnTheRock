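; BP_Planks is a planks pickup that the player character can grab, carry and throw away.
; Grab snaps the Cube back to the root, disables its physics, attaches to the character's AttachPoint socket, and registers itself as the carried object with a "Throw away" prompt.
; Interact hands the Cube to the character's Throw, only while grabbed and not Repairing.
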(event EventBeginPlay
  (bind _asbp_character (Utilities|Casting|CastToBP_Character (Game|GetPlayerCharacter 0)))
  (Variables|Default|SetCharacter _asbp_character))

(event Collision|EventActorBeginOverlap
  (params (OtherActor :type Actor%20Object%20Reference)))

(event EventTick
  (params (DeltaSeconds :type Float%20%28single-precision%29)))

(event EventInteract
  (if (Variables|Default|GetisGrabbed)
    (if (not (Variables|Default|GetRepairing))
      (Default|Throw (Variables|Default|GetCharacter) (Variables|Default|GetCube)))))

(event EventGrab
  (params (Character :type Skeletal%20Mesh%20Component%20Object%20Reference))
  (Transformation|AttachComponentToComponent (Variables|Default|GetCube) (Variables|Default|GetDefaultSceneRoot) "None" "SnapToTarget" "SnapToTarget" "KeepWorld" true)
  (Physics|SetSimulatePhysics (Variables|Default|GetCube) false)
  (Variables|/Game/Blueprints/Bluperints/BP_Character.BP_Character_C|SetCaryObject (Variables|Default|GetCharacter) true)
  (Variables|/Game/Blueprints/Bluperints/BP_Character.BP_Character_C|SetCarriedObject (Variables|Default|GetCharacter) self)
  (Transformation|AttachComponentToComponent Character "AttachPoint" "SnapToTarget" "SnapToTarget" "KeepWorld" false)
  (Variables|Default|SetisGrabbed true)
  (Variables|/Game/Blueprints/Bluperints/BP_Character.BP_Character_C|SetGrabbedInteraction (Variables|Default|GetCharacter) "Throw away")
  (Default|ShowGrabbedInteraction (Variables|Default|GetCharacter)))

(fn ConstructionScript)