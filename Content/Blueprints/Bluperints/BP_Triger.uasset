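; BP_Triger is a box trigger that starts a level problem when a Character enters it on a specific day.
; It caches the level manager on BeginPlay, and on overlap compares the manager's CurrentDay with DayOfAction.
; On a match, the Event Starter type passes EventRequired to ProblemResolution without delay, then switches the trigger off.
; A Character overlap on any other day also switches it off, and nothing here re-enables it.
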(event OnComponentBeginOverlap(Box)
  (params (OverlappedComponent :type Primitive%20Component%20Object%20Reference) (OtherActor :type Actor%20Object%20Reference) (OtherComp :type Primitive%20Component%20Object%20Reference) (OtherBodyIndex :type Integer) (bFromSweep :type Boolean) (SweepResult :type Hit%20Result%20Structure%20%28by%20ref%29))
  (if (Variables|Default|GetisOn)
    (Utilities|Casting|CastToCharacter OtherActor)
    (if (== (Variables|/Game/Blueprints/Bluperints/BP_LevelManager.BP_LevelManager_C|GetCurrentDay (Variables|Default|GetLevelManager)) (Variables|Default|GetDayOfAction))
      (switch Utilities|FlowControl|Switch|SwitchonBPE_TriggerType (Variables|Default|GetType)
        (:NewEnumerator1
          (Default|ProblemResolution (Variables|Default|GetLevelManager) (Variables|Default|GetEventRequired) 0.0)
          (Variables|Default|SetisOn false)))
      (else
        (Variables|Default|SetisOn false)))))

(event EventBeginPlay
  (bind _outactors (Actor|GetAllActorsOfClass "/Game/Blueprints/Bluperints/BP_LevelManager.BP_LevelManager_C"))
  (Variables|Default|SetLevelManager (Utilities|Array|Get(acopy) _outactors)))

(event EventTick
  (params (DeltaSeconds :type Float%20%28single-precision%29)))

(fn ConstructionScript)