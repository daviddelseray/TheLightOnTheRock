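; Carryable rat trap the player places on walkable surfaces and that catches rats when set on a rat nest.
; Grab carries the trap or hands off its caught rat, while Interact places it via camera line trace, or defuses it when not held.
; A trap overlapping a nest becomes effective, advancing the level manager's day-one trap objective.
; CatchRat spawns a caught rat in effective, empty traps.
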(event Custom|CatchRat
  (bind _ratspawnplace (Variables|Default|GetRatSpawnPlace))
  (if (Variables|Default|GetisEffective)
    (if (not (Variables|Default|GetisFull))
      (Variables|Default|SetisSet false)
      (Variables|Default|SetisEffective false)
      (bind _returnvalue (Game|SpawnActorfromClass "/Game/Blueprints/Bluperints/BP_Rat.BP_Rat_C" (Math|Transform|MakeTransform (Transformation|GetWorldLocation _ratspawnplace) (Transformation|GetWorldRotation _ratspawnplace) "1,1,1") "Undefined" 0 0))
      (bind _output_get (Variables|Default|SetRat _returnvalue))
      (Variables|/Game/Blueprints/Bluperints/BP_Rat.BP_Rat_C|SetTrap _output_get self)
      (Variables|/Game/Blueprints/Bluperints/BP_Rat.BP_Rat_C|SetisCaught _output_get true)
      (Variables|Default|SetisFull true))))

(event EventBeginPlay)

(event Collision|EventActorBeginOverlap
  (params (OtherActor :type Actor%20Object%20Reference)))

(event EventTick
  (params (DeltaSeconds :type Float%20%28single-precision%29)))

(event EventInteract
  (if (Variables|Default|GetisGrabbed)
    (bind _asbp_character (Utilities|Casting|CastToBP_Character (Game|GetPlayerCharacter 0)))
    (bind _outhit (Collision|LineTraceByChannel (Transformation|GetWorldLocation (Variables|/Game/Blueprints/Bluperints/BP_Character.BP_Character_C|GetFirstPersonCamera _asbp_character)) (+ (Transformation|GetWorldLocation (Variables|/Game/Blueprints/Bluperints/BP_Character.BP_Character_C|GetFirstPersonCamera _asbp_character)) (* (Math|Vector|GetForwardVector (Variables|/Game/Blueprints/Bluperints/BP_Character.BP_Character_C|GetFirstPersonCamera _asbp_character)) (Variables|/Game/Blueprints/Bluperints/BP_Character.BP_Character_C|GetInteractRayLength _asbp_character))) "TraceTypeQuery1" false 0 "ForDuration" true "(R=1.000000,G=0.101989,B=0.161720,A=1.000000)" "(R=0.801595,G=0.765915,B=1.000000,A=1.000000)" 2e+02))
    (Utilities|Casting|CastToBP_WalkableSurface (.hitactor _outhit))
    (Transformation|DetachFromActor "KeepWorld" "KeepWorld" "KeepWorld")
    (bind _asbp_character_2 (Utilities|Casting|CastToBP_Character (Game|GetPlayerCharacter 0)))
    (Variables|/Game/Blueprints/Bluperints/BP_Character.BP_Character_C|SetCaryObject _asbp_character_2 false)
    (Variables|/Game/Blueprints/Bluperints/BP_Character.BP_Character_C|SetCarriedObject _asbp_character_2 0)
    (Variables|Default|SetisGrabbed false)
    (Transformation|SetWorldLocation (Variables|Default|GetDefaultSceneRoot) (.location _outhit) false false)
    (Transformation|SetWorldRotation (Variables|Default|GetDefaultSceneRoot) "0, 0, 0" false false)
    (Variables|Default|SetisSet true)
    (bind _asbp_character_3 (Utilities|Casting|CastToBP_Character (Game|GetPlayerCharacter 0)))
    (Default|HideGrabbedInteraction _asbp_character_3)
    (if (> (Utilities|Array|Length (Collision|GetOverlappingActors (Variables|Default|GetLighthouseRatTrap) "/Game/Blueprints/Bluperints/BP_RatNest.BP_RatNest_C" :!class /Script/Engine.PrimitiveComponent)) 0)
      (Variables|Default|SetisEffective true)
      (bind _outactors (Actor|GetAllActorsOfClass "/Game/Blueprints/Bluperints/BP_LevelManager.BP_LevelManager_C"))
      (if (and (== (Variables|/Game/Blueprints/Bluperints/BP_LevelManager.BP_LevelManager_C|GetCurrentDay (Utilities|Array|Get(acopy) _outactors)) 1) (or (== (Variables|/Game/Blueprints/Bluperints/BP_LevelManager.BP_LevelManager_C|GetCurrentProblem (Utilities|Array|Get(acopy) _outactors)) 11) (== (Variables|/Game/Blueprints/Bluperints/BP_LevelManager.BP_LevelManager_C|GetCurrentProblem (Utilities|Array|Get(acopy) _outactors)) 10)))
        (bind _result (Math|Integer|IncrementInt (Variables|/Game/Blueprints/Bluperints/BP_LevelManager.BP_LevelManager_C|GetDay1SetRatTraps (Utilities|Array|Get(acopy) _outactors)))
          (:%20%20
            (if (== _result 3)
              (Default|ProblemResolution (Utilities|Array|Get(acopy) _outactors) 12))))))
    (else
      (Variables|Default|SetisSet false))))

(event EventRelease
  (Transformation|DetachFromActor "KeepWorld" "KeepWorld" "KeepWorld")
  (bind _asbp_character (Utilities|Casting|CastToBP_Character (Game|GetPlayerCharacter 0)))
  (Variables|/Game/Blueprints/Bluperints/BP_Character.BP_Character_C|SetCaryObject _asbp_character false)
  (Variables|/Game/Blueprints/Bluperints/BP_Character.BP_Character_C|SetCarriedObject _asbp_character 0)
  (Physics|SetSimulatePhysics (Variables|Default|GetLighthouseRatTrap) true)
  (Variables|Default|SetisGrabbed false))

(event EventGrab
  (params (Character :type Skeletal%20Mesh%20Component%20Object%20Reference))
  (if (Variables|Default|GetisFull)
    (Default|Grab (Variables|Default|GetRat) Character)
    (Variables|Default|SetisFull false)
    (elif (not (Variables|Default|GetisSet))
      (Transformation|AttachComponentToComponent (Variables|Default|GetLighthouseRatTrap) (Variables|Default|GetDefaultSceneRoot) "None" "SnapToTarget" "SnapToTarget" "KeepWorld" true)
      (Physics|SetSimulatePhysics (Variables|Default|GetLighthouseRatTrap) false)
      (bind _asbp_character (Utilities|Casting|CastToBP_Character (Game|GetPlayerCharacter 0)))
      (Variables|/Game/Blueprints/Bluperints/BP_Character.BP_Character_C|SetCaryObject _asbp_character true)
      (Variables|/Game/Blueprints/Bluperints/BP_Character.BP_Character_C|SetCarriedObject _asbp_character self)
      (Transformation|AttachComponentToComponent Character "AttachPoint" "SnapToTarget" "SnapToTarget" "KeepWorld" false)
      (Variables|/Game/Blueprints/Bluperints/BP_Character.BP_Character_C|SetGrabbedInteraction _asbp_character "Set Trap")
      (Variables|Default|SetisGrabbed true)
      (Default|ShowGrabbedInteraction _asbp_character))))

(event EventRevealInteractions
  (if (Variables|Default|GetisSet)
    (bind _asbp_character (Utilities|Casting|CastToBP_Character (Game|GetPlayerCharacter 0)))
    (Default|ShowInteractions _asbp_character "Defuse Trap" false)))

(fn ConstructionScript)