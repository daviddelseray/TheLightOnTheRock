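; BP_RightClosetDoor is an interactable right closet door that swings open and closed.
; Interact alternates Open and Close through a FlipFlop, playing or reversing a timeline that drives the yaw of PivotPoint.
; RevealInteractions has BP_Character show the matching open or close prompt on the E interaction.
; The player cast happens only on the closed branch; the open branch reuses that cast's result.
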(event Custom|Open
  ;[1 1 1] Rotate the door
  (bind _rotationz (Timeline|Timeline_0 Play)
    (:Update
      (Transformation|SetRelativeRotation (Variables|Default|GetPivotPoint) (Math|Rotator|MakeRotator 0.0 0.0 _rotationz) false false))))

(event Custom|Close
  ;[1 1 1] Rotate the door
  (bind _rotationz (Timeline|Timeline_0 Reverse)
    (:Update
      (Transformation|SetRelativeRotation (Variables|Default|GetPivotPoint) (Math|Rotator|MakeRotator 0.0 0.0 _rotationz) false false))))

(event EventBeginPlay)

(event Collision|EventActorBeginOverlap
  (params (OtherActor :type Actor%20Object%20Reference)))

(event EventTick
  (params (DeltaSeconds :type Float%20%28single-precision%29)))

(event EventInteract
  (bind _isa (Utilities|FlowControl|FlipFlop)
    (:A
      (CallFunction|Open))
    (:B
      (CallFunction|Close)))
  (Variables|Default|SetisOpen _isa)
  (CallFunction|RevealInteractions))

(event EventRevealInteractions
  (if (Variables|Default|GetisOpen)
    (Default|ShowInteractions (stale _asbp_character) "CloseDoor" false)
    (else
      (bind _asbp_character (Utilities|Casting|CastToBP_Character (Game|GetPlayerCharacter 0)))
      (Default|ShowInteractions _asbp_character "Open Door" false))))

(fn ConstructionScript)