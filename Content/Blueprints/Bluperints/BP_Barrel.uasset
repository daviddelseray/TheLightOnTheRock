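; BP_Barrel is an interactable barrel that lets the player fill a carried bucket.
; It caches the player's BP_Character on BeginPlay and reads its CarriedObject to find a BP_Bucket.
; RevealInteractions shows a "Fill the Bucket" prompt only when that bucket is not full.
; Interact calls Fill on the carried bucket and then hides the interaction prompt.
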(event EventBeginPlay
  (bind _asbp_character (Utilities|Casting|CastToBP_Character (Game|GetPlayerCharacter 0)))
  (Variables|Default|SetCharacter _asbp_character))

(event Collision|EventActorBeginOverlap
  (params (OtherActor :type Actor%20Object%20Reference)))

(event EventTick
  (params (DeltaSeconds :type Float%20%28single-precision%29)))

(event EventInteract
  (bind _character (Variables|Default|GetCharacter))
  (bind _asbp_bucket (Utilities|Casting|CastToBP_Bucket (Variables|/Game/Blueprints/Bluperints/BP_Character.BP_Character_C|GetCarriedObject _character)))
  (Default|Fill _asbp_bucket)
  (Default|HideInteractions _character false true))

(event EventRevealInteractions
  (bind _character (Variables|Default|GetCharacter))
  (bind _asbp_bucket (Utilities|Casting|CastToBP_Bucket (Variables|/Game/Blueprints/Bluperints/BP_Character.BP_Character_C|GetCarriedObject _character)))
  (if (not (Variables|/Game/Blueprints/Bluperints/BP_Bucket.BP_Bucket_C|GetisFull _asbp_bucket))
    (Default|ShowInteractions _character "Fill the Bucket" false)))

(fn ConstructionScript)