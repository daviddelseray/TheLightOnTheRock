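; Living rat actor that can be revealed, run to a given point, then scatter.
; RunToPoint lerps it there on a timeline whose play rate comes from the point's TimeToAccess, while Tick turns it toward the goal.
; On arrival at a non-destroyer point, or when Scatter is called, it navigates via SimpleMoveToActor to a random destroyer-flagged BP_RatsScatterPoints, relying on the nav mesh.
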(event Custom|Scatter
  ;[1 1 1] In case of rat not moving after reaching the first scatter point, rebuild the nav mesh.
  (if (not (Variables|Default|GetisScattering))
    (Variables|Default|SetisScattering true)
    (CallFunction|StopRunning)
    (Variables|Default|SetisRunning true)
    (bind _outactors (Actor|GetAllActorsOfClass "/Game/Blueprints/Bluperints/BP_RatsScatterPoints.BP_RatsScatterPoints_C"))
    (for _array_element _outactors
      (if (Variables|/Game/Blueprints/Bluperints/BP_RatsScatterPoints.BP_RatsScatterPoints_C|GetisDestroyer _array_element)
        (Utilities|Array|Add (Variables|Default|GetScatterPoints) _array_element)))
    (bind _output_get (Variables|Default|SetGoalActor (Utilities|Array|Get(acopy) (Variables|Default|GetScatterPoints) (Math|Random|RandomIntegerinRange 0 (Utilities|Array|LastIndex (Variables|Default|GetScatterPoints))))))
    (AI|Navigation|SimpleMovetoActor (Pawn|GetController) _output_get)
    (Variables|Default|SetisScattering false)))

(event Custom|RunToPoint
  (Variables|Default|SetGoalActor (Variables|Default|GetPointToRun))
  (Variables|Default|SetisRunning true)
  (Variables|Default|SetPositionBeforeRun (Transformation|GetWorldLocation (Variables|Default|GetCollisionComponent)))
  (Components|Timeline|SetPlayRate (Variables|Default|GetRunTime) (Variables|/Game/Blueprints/Bluperints/BP_RatsScatterPoints.BP_RatsScatterPoints_C|GetTimeToAccess (Variables|Default|GetPointToRun)))
  (bind _lerpprogress (Timeline|RunTime PlayFromStart)
    (:Update
      (Transformation|SetWorldLocation (Variables|Default|GetCollisionComponent) (Math|Vector|Lerp(Vector) (Variables|Default|GetPositionBeforeRun) (Transformation|GetActorLocation (Variables|Default|GetGoalActor)) _lerpprogress) false false))
    (:Finished
      (if (not (Variables|/Game/Blueprints/Bluperints/BP_RatsScatterPoints.BP_RatsScatterPoints_C|GetisDestroyer (Variables|Default|GetPointToRun)))
        (CallFunction|Scatter)))))

(event Custom|Appear
  (Rendering|SetVisibility (Variables|Default|GetRat) true false))

(event Custom|StopRunning
  (bind _lerpprogress (Timeline|RunTime Stop)
    (:Update
      (Transformation|SetWorldLocation (Variables|Default|GetCollisionComponent) (Math|Vector|Lerp(Vector) (Variables|Default|GetPositionBeforeRun) (Transformation|GetActorLocation (Variables|Default|GetGoalActor)) _lerpprogress) false false))
    (:Finished
      (if (not (Variables|/Game/Blueprints/Bluperints/BP_RatsScatterPoints.BP_RatsScatterPoints_C|GetisDestroyer (Variables|Default|GetPointToRun)))
        (CallFunction|Scatter)))))

(event EventBeginPlay)

(event Collision|EventActorBeginOverlap
  (params (OtherActor :type Actor%20Object%20Reference)))

(event EventTick
  (params (DeltaSeconds :type Float%20%28single-precision%29))
  (bind _goalactor (Variables|Default|GetGoalActor))
  (bind _collisioncomponent (Variables|Default|GetCollisionComponent))
  (bind _returnvalue (Transformation|GetActorLocation _goalactor))
  (bind _returnvalue_2 (Transformation|GetWorldLocation _collisioncomponent))
  (bind _returnvalue_3 (Math|Rotator|FindLookatRotation _returnvalue_2 _returnvalue))
  (if (Variables|Default|GetisRunning)
    (Transformation|SetWorldRotation (Variables|Default|GetCollisionComponent) (Math|Rotator|MakeRotator (.roll _returnvalue_3) 0.0 (.yaw _returnvalue_3)) false false)))

(fn ConstructionScript)