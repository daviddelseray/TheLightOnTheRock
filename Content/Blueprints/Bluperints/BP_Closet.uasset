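; Interactable closet whose double doors open and close, and which can release rats during a scripted level problem.
; Interact toggles the open state, triggers the character's animation and, after a short delay, plays or reverses a timeline that rotates both door pivots.
; When the timeline finishes, the prompt refreshes if an interaction cone overlaps.
; If opened with rats inside on the matching day and problem, BP_LevelManager's rodents flee, then are destroyed, and the problem advances.
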(event Custom|DoorOpening
  (Utilities|FlowControl|Delay 0.5)
  (Variables|/Game/DefaultContent/FirstPerson/Animations/ABP_Character.ABP_Character_C|SetOpeningCloset (Variables|/Game/Blueprints/Bluperints/BP_Character.BP_Character_C|GetABP_Character (Variables|Default|GetCharacter)) false)
  (bind _newtrack_0 (Timeline|OpenDoors Play)
    (:Update
      (Transformation|SetRelativeRotation (Variables|Default|GetPivotPointLeft) (Math|Rotator|MakeRotator 0.0 0.0 _newtrack_0) false false)
      (bind _result (Math|Float|NegateFloat _newtrack_0)
        (:%20%20
          (Transformation|SetRelativeRotation (Variables|Default|GetPivotPointRight) (Math|Rotator|MakeRotator 0.0 0.0 _result) false false))))
    (:Finished
      (CallFunction|RevealInteractions)
      (if (Variables|Default|GetisOpen)
        (if (Variables|Default|GetratsInside)
          (bind _outactors (Actor|GetAllActorsOfClass "/Game/Blueprints/Bluperints/BP_LevelManager.BP_LevelManager_C"))
          (if (and (== (Variables|/Game/Blueprints/Bluperints/BP_LevelManager.BP_LevelManager_C|GetCurrentDay (Utilities|Array|Get(acopy) _outactors)) 1) (== (Variables|/Game/Blueprints/Bluperints/BP_LevelManager.BP_LevelManager_C|GetCurrentProblem (Utilities|Array|Get(acopy) _outactors)) 8))
            (CallFunction|RatSpread true)
            (Utilities|FlowControl|Delay 0.5)
            (Default|ProblemResolution (Utilities|Array|Get(acopy) _outactors) 9 0.0)))))))

(event Custom|DoorClosing
  (Utilities|FlowControl|Delay 0.5)
  (Variables|/Game/DefaultContent/FirstPerson/Animations/ABP_Character.ABP_Character_C|SetClosingCloset (Variables|/Game/Blueprints/Bluperints/BP_Character.BP_Character_C|GetABP_Character (Variables|Default|GetCharacter)) false)
  (bind _newtrack_0 (Timeline|OpenDoors Reverse)
    (:Update
      (Transformation|SetRelativeRotation (Variables|Default|GetPivotPointLeft) (Math|Rotator|MakeRotator 0.0 0.0 _newtrack_0) false false)
      (bind _result (Math|Float|NegateFloat _newtrack_0)
        (:%20%20
          (Transformation|SetRelativeRotation (Variables|Default|GetPivotPointRight) (Math|Rotator|MakeRotator 0.0 0.0 _result) false false))))
    (:Finished
      (CallFunction|RevealInteractions)
      (if (Variables|Default|GetisOpen)
        (if (Variables|Default|GetratsInside)
          (bind _outactors (Actor|GetAllActorsOfClass "/Game/Blueprints/Bluperints/BP_LevelManager.BP_LevelManager_C"))
          (if (and (== (Variables|/Game/Blueprints/Bluperints/BP_LevelManager.BP_LevelManager_C|GetCurrentDay (Utilities|Array|Get(acopy) _outactors)) 1) (== (Variables|/Game/Blueprints/Bluperints/BP_LevelManager.BP_LevelManager_C|GetCurrentProblem (Utilities|Array|Get(acopy) _outactors)) 8))
            (CallFunction|RatSpread true)
            (Utilities|FlowControl|Delay 0.5)
            (Default|ProblemResolution (Utilities|Array|Get(acopy) _outactors) 9 0.0)))))))

(event Custom|RatSpread
  (params (hasDelay :type Boolean))
  (Variables|Default|SetratsInside false)
  (if hasDelay
    (Utilities|FlowControl|Delay 1.0)
    (bind _outactors (Actor|GetAllActorsOfClass "/Game/Blueprints/Bluperints/BP_LevelManager.BP_LevelManager_C"))
    (for _array_element (Variables|/Game/Blueprints/Bluperints/BP_LevelManager.BP_LevelManager_C|GetRodents (Utilities|Array|Get(acopy) _outactors))
      (Default|RuntoPoint _array_element))
    (Utilities|FlowControl|Delay 2.0)
    (bind _outactors_2 (Actor|GetAllActorsOfClass "/Game/Blueprints/Bluperints/BP_LevelManager.BP_LevelManager_C"))
    (for _array_element_2 (Variables|/Game/Blueprints/Bluperints/BP_LevelManager.BP_LevelManager_C|GetRodents (Utilities|Array|Get(acopy) _outactors_2))
      (Utilities|IsValid _array_element_2
        (:Is%20Valid
          (Actor|DestroyActor _array_element_2))))))

(event EventBeginPlay
  (bind _asbp_character (Utilities|Casting|CastToBP_Character (Game|GetPlayerCharacter 0)))
  (Variables|Default|SetCharacter _asbp_character))

(event Collision|EventActorBeginOverlap
  (params (OtherActor :type Actor%20Object%20Reference)))

(event EventTick
  (params (DeltaSeconds :type Float%20%28single-precision%29)))

(event EventInteract
  (bind _character (Variables|Default|GetCharacter))
  (if (Variables|Default|GetisOpen)
    (CallFunction|DoorClosing)
    (Variables|Default|SetisOpen false)
    (Default|ObjectInteractAnimationin _character "NewEnumerator4")
    (else
      (CallFunction|DoorOpening)
      (Variables|Default|SetisOpen true)
      (Default|ObjectInteractAnimationin _character "NewEnumerator3"))))

(event EventRevealInteractions
  (bind _character (Variables|Default|GetCharacter))
  (bind _interactionconepresent (CallFunction|InteractionConeDetection))
  (if _interactionconepresent
    (if (Variables|Default|GetisOpen)
      (Default|ShowInteractions _character "Close Doors" false)
      (else
        (Default|ShowInteractions _character "Open Doors" false)))))

(fn ConstructionScript)

(fn InteractionConeDetection
  (for _array_element (Class|PrimitiveComponent|GetOverlappingComponents (Variables|Default|GetBox))
    _)
  (return (Components|ComponentHasTag _array_element "InteractionCone")))