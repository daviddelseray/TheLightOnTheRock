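; BP_Movable is an interactable world object that the player character can grab and move around when it is flagged as movable.
; Interacting triggers StartMoving, which attaches the actor to BP_Character while keeping its world transform; StopMoving detaches it the same way.
; ShowInteraction has the character's grab HUD display a "Move the" prompt with the object's name.
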(event Custom|StartMoving
  (if (Variables|Default|GetisMovable)
    (Variables|Default|SetisMoving true)
    (bind _asbp_character (Utilities|Casting|CastToBP_Character (Game|GetPlayerCharacter 0)))
    (Transformation|AttachActorToActor _asbp_character "None" "KeepWorld" "KeepWorld" "KeepWorld" true)))

(event Custom|StopMoving
  (Variables|Default|SetisMoving false)
  (Transformation|DetachFromActor "KeepWorld" "KeepWorld" "KeepWorld"))

(event Custom|ShowInteraction
  (if (Variables|Default|GetisMovable)
    (bind _asbp_character (Utilities|Casting|CastToBP_Character (Game|GetPlayerCharacter 0)))
    (Default|ChangeGrabHUD _asbp_character (Utilities|String|Append "Move the" (Variables|Default|GetName)) true)))

(event EventBeginPlay)

(event Collision|EventActorBeginOverlap
  (params (OtherActor :type Actor%20Object%20Reference)))

(event EventTick
  (params (DeltaSeconds :type Float%20%28single-precision%29)))

(event EventInteract
  (CallFunction|StartMoving))

(fn ConstructionScript)