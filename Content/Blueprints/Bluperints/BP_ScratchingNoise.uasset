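; BP_ScratchingNoise is an actor that repeats a scratching sound until the player character comes near.
; Activate enables the proximity trigger and starts a self-calling loop that replays the audio after a random delay based on the clip's length.
; A BP_Character overlap stops the sound and disables the trigger.
; If BP_LevelManager reports day 3 and problem 0, the overlap also plays a delayed monologue through DialogManager.
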(event OnComponentBeginOverlap(ProximityDetection)
  (params (OverlappedComponent :type Primitive%20Component%20Object%20Reference) (OtherActor :type Actor%20Object%20Reference) (OtherComp :type Primitive%20Component%20Object%20Reference) (OtherBodyIndex :type Integer) (bFromSweep :type Boolean) (SweepResult :type Hit%20Result%20Structure%20%28by%20ref%29))
  (Utilities|Casting|CastToBP_Character OtherActor)
  (Variables|Default|SetisPlaying false)
  (Audio|Components|Audio|Stop (Variables|Default|GetAudio))
  (Collision|SetCollisionEnabled (Variables|Default|GetProximityDetection) "NoCollision")
  (bind _outactors (Actor|GetAllActorsOfClass "/Game/Blueprints/Bluperints/BP_LevelManager.BP_LevelManager_C"))
  (if (and (== (Variables|/Game/Blueprints/Bluperints/BP_LevelManager.BP_LevelManager_C|GetCurrentDay (Utilities|Array|Get(acopy) _outactors)) 3) (== (Variables|/Game/Blueprints/Bluperints/BP_LevelManager.BP_LevelManager_C|GetCurrentProblem (Utilities|Array|Get(acopy) _outactors)) 0))
    (Default|PlayMonolog (Variables|Default|GetdialogManager) 1 1.5)))

(event Custom|Activate
  (Collision|SetCollisionEnabled (Variables|Default|GetProximityDetection) "QueryOnly")
  (Variables|Default|SetisPlaying true)
  (CallFunction|LoopPlay))

(event Custom|LoopPlay
  (if (Variables|Default|GetisPlaying)
    (Audio|Components|Audio|Play (Variables|Default|GetAudio) 0.0)
    (bind _output_get (Variables|Default|SetDelay (Math|Random|RandomFloatinRange (Variables|/Script/Engine.SoundBase|GetDuration (Variables|/Script/Engine.AudioComponent|GetSound (Variables|Default|GetAudio))) 3.0)))
    (Utilities|FlowControl|Delay _output_get)
    (CallFunction|LoopPlay)))

(event EventBeginPlay)

(event Collision|EventActorBeginOverlap
  (params (OtherActor :type Actor%20Object%20Reference)))

(event EventTick
  (params (DeltaSeconds :type Float%20%28single-precision%29)))

(fn ConstructionScript)