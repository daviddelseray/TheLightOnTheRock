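; Wall-walk trigger actor that marks a BP_Character as being at a watch point when it begins overlapping.
; On overlap it sets the character's AtWatchPoint flag and registers itself as WatchPoint; it never clears either.
; GiveLookAtPoint scales the root-to-player capsule offset by DistanceLookAtPoint for X and Y, without adding the root position back, and takes Z from the root's world height.
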(event EventBeginPlay)

(event EventTick
  (params (DeltaSeconds :type Float%20%28single-precision%29)))

(event Collision|EventActorBeginOverlap
  (params (OtherActor :type Actor%20Object%20Reference))
  (bind _asbp_character (Utilities|Casting|CastToBP_Character OtherActor))
  (Variables|/Game/Blueprints/Bluperints/BP_Character.BP_Character_C|SetatWatchPoint _asbp_character true)
  (Variables|/Game/Blueprints/Bluperints/BP_Character.BP_Character_C|SetWatchPoint _asbp_character self))

(fn ConstructionScript)

(fn GiveLookatPoint
  (bind _returnvalue (Game|GetPlayerCharacter 0))
  (bind _defaultsceneroot (Variables|Default|GetDefaultSceneRoot))
  (bind _distancelookatpoint (LocalVariables|GetDistanceLookAtPoint))
  (bind _returnvalue_2 (Transformation|GetWorldLocation _defaultsceneroot))
  (bind _capsulecomponent (Variables|/Script/Engine.Character|GetCapsuleComponent _returnvalue))
  (bind _returnvalue_3 (Transformation|GetWorldLocation _capsulecomponent))
  (bind _returnvalue_4 (Math|Vector|MakeVector (.x _returnvalue_2) (.y _returnvalue_2) (.z _returnvalue_2)))
  (bind _returnvalue_5 (- _returnvalue_3 _returnvalue_4))
  (bind _returnvalue_6 (* _returnvalue_5 _distancelookatpoint))
  (return (Math|Vector|MakeVector (.x _returnvalue_6) (.y _returnvalue_6) (.z _returnvalue_2))))