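; Day 2 seagull quick-time event: three scripted attacks in sequence, closed by Archibald monologues before LevelManager moves to the next problem.
; Each stage moves the player along rails, steers the camera between interest points, activates a seagull and opens a timed input window.
; Success knocks the bird away; failure plays a knock-back and marks the player hurt.
; Both outcomes advance the sequence, with closing lines depending on injury and a carried frying pan.
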(event EventBeginPlay
  (|CallParentFunction)
  (bind _asbp_character (Utilities|Casting|CastToBP_Character (Game|GetPlayerCharacter 0)))
  (Variables|Default|SetCharacter _asbp_character)
  (bind _outactors (Actor|GetAllActorsOfClass "/Game/Blueprints/Bluperints/BP_LevelManager.BP_LevelManager_C"))
  (Variables|Default|SetLevelManager (Utilities|Array|Get(acopy) _outactors))
  (bind _outactors_2 (Actor|GetAllActorsOfClass "/Game/Blueprints/Bluperints/BP_DialogManager.BP_DialogManager_C"))
  (Variables|Default|SetdialogManager (Utilities|Array|Get(acopy) _outactors_2)))

(event Collision|EventActorBeginOverlap
  (params (OtherActor :type Actor%20Object%20Reference))
  (|CallParentFunction OtherActor) ; This node is disabled and will not be called.\nDrag off pins to build functionality.
)

(event EventTick
  (params (DeltaSeconds :type Float%20%28single-precision%29))
  (|CallParentFunction DeltaSeconds)
  (if (Variables|Default|GetTracking)
    (Default|QTECamDirectControl (Variables|Default|GetCharacter) (Transformation|GetWorldLocation (Variables|/Game/Blueprints/Bluperints/BP_Seagull.BP_Seagull_C|GetCube (Variables|Default|GetSeagul1))))))

(event EventEvent
  (bind _dialogmanager (Variables|Default|GetdialogManager))
  (switch int (Variables|Default|GetCurrentInteraction)
    (:0
      (CallFunction|StartStopQTE true)
      (Default|QTECameraControlMove (Variables|Default|GetCharacter) 0.6 (Transformation|GetWorldLocation (Variables|Default|GetInterestPoint)))
      (Default|PlayMonolog _dialogmanager 34)
      (Utilities|FlowControl|Delay (Variables|/Script/Engine.SoundBase|GetDuration (.lineaudio (Utilities|Array|Get(acopy) (Variables|/Game/Blueprints/Bluperints/BP_DialogManager.BP_DialogManager_C|GetDay2ArchibaldMonolog _dialogmanager) 34))))
      (Default|QTECameraControlMove (Variables|Default|GetCharacter) 0.6 (Transformation|GetWorldLocation (Variables|Default|GetInterestPoint1)))
      (Default|WalktheRail (Variables|Default|GetFirstRail))
      (Utilities|FlowControl|Delay 3.0)
      (Default|Activate (Variables|Default|GetSeagul1) 0.0)
      (Default|QTECameraControlMove (Variables|Default|GetCharacter) 0.4 (Transformation|GetWorldLocation (Variables|Default|GetInterestPoint2)))
      (Utilities|FlowControl|Delay 0.6)
      (Default|QTECameraControlMove (Variables|Default|GetCharacter) 1.0 (Transformation|GetWorldLocation (Variables|Default|GetInterestPoint3)))
      (CallFunction|ShowInput)
      (Utilities|FlowControl|Delay 0.2))
    (:1
      (Default|WalktheRail (Variables|Default|GetSecondRail))
      (Default|QTECameraControlMove (Variables|Default|GetCharacter) 1.5 (Transformation|GetWorldLocation (Variables|Default|GetInterestPoint4)))
      (Utilities|FlowControl|Delay 1.0)
      (Default|Activate (Variables|Default|GetSeagull2) 0.0)
      (Utilities|FlowControl|Delay 1.0)
      (Default|QTECameraControlMove (Variables|Default|GetCharacter) 1.0 (Transformation|GetWorldLocation (Variables|Default|GetInterestPoint5)))
      (Utilities|FlowControl|Delay 0.4)
      (CallFunction|ShowInput)
      (Utilities|FlowControl|Delay 0.2))
    (:2
      (Default|WalktheRail (Variables|Default|GetThirdRail))
      (Default|QTECameraControlMove (Variables|Default|GetCharacter) 2.0 (Transformation|GetWorldLocation (Variables|Default|GetInterestPoint6)))
      (Utilities|FlowControl|Delay 2.0)
      (Default|QTECameraControlMove (Variables|Default|GetCharacter) 0.3 (Transformation|GetWorldLocation (Variables|Default|GetInterestPoint7)))
      (Default|Activate (Variables|Default|GetSeagull3) 0.0)
      (CallFunction|ShowInput)
      (Utilities|FlowControl|Delay 0.3)))
  (CallFunction|AcceptInput)
  (bind _returnvalue (Utilities|Time|SetTimerbyFunctionName 0 "Fail" (Utilities|Array|Get(acopy) (Variables|Default|GetInteractionsDurations) (Variables|Default|GetCurrentInteraction)))))

(event EventSuccess
  (bind _dialogmanager (Variables|Default|GetdialogManager))
  (bind _dialogmanager_2 (Variables|Default|GetdialogManager))
  (bind _character (Variables|Default|GetCharacter))
  (bind _character_2 (Variables|Default|GetCharacter))
  (bind _dialogmanager_3 (Variables|Default|GetdialogManager))
  (Variables|Default|SetAcceptingInputs false)
  (Utilities|Time|ClearandInvalidateTimerbyHandle (stale EventEvent _returnvalue))
  (switch int (Variables|Default|GetCurrentInteraction)
    (:0
      (CallFunction|HideInput)
      (Default|GetHit (Variables|Default|GetSeagul1) "300.000000,-1300.000000,100.000000")
      (Utilities|FlowControl|Delay 0.3)
      (Default|QTECameraControlMove (Variables|Default|GetCharacter) 0.5 (Transformation|GetWorldLocation (Variables|Default|GetInterestPoint1)))
      (Utilities|FlowControl|Delay 1.0)
      (Math|Integer|IncrementInt (Variables|Default|GetCurrentInteraction)
        (:%20%20
          (CallFunction|Event)
          (if (not (Variables|/Game/Blueprints/Bluperints/BP_Character.BP_Character_C|GetisArmed _character))
            (Variables|/Game/Blueprints/Bluperints/BP_Character.BP_Character_C|SetisHurt _character true)))))
    (:1
      (CallFunction|HideInput)
      (Default|GetHit (Variables|Default|GetSeagull2) "300.000000,1300.000000,-80.000000")
      (Default|QTECameraControlMove (Variables|Default|GetCharacter) 0.5 (Transformation|GetWorldLocation (Variables|Default|GetInterestPoint4)))
      (Math|Integer|IncrementInt (Variables|Default|GetCurrentInteraction)
        (:%20%20
          (CallFunction|Event))))
    (:2
      (CallFunction|HideInput)
      (Default|GetHit (Variables|Default|GetSeagull3) "300.000000,1300.000000,-80.000000")
      (Utilities|FlowControl|Delay 0.8)
      (Default|QTECameraControlMove (Variables|Default|GetCharacter) 0.8 (Transformation|GetWorldLocation (Variables|Default|GetInterestPoint10)))
      (Default|PlayMonolog _dialogmanager_3 35)
      (Utilities|FlowControl|Delay (Variables|/Script/Engine.SoundBase|GetDuration (.lineaudio (Utilities|Array|Get(acopy) (Variables|/Game/Blueprints/Bluperints/BP_DialogManager.BP_DialogManager_C|GetDay2ArchibaldMonolog _dialogmanager_3) 35))))
      (if (Variables|/Game/Blueprints/Bluperints/BP_Character.BP_Character_C|GetisHurt _character_2)
        (Default|PlayMonolog _dialogmanager 36)
        (Utilities|FlowControl|Delay (Variables|/Script/Engine.SoundBase|GetDuration (.lineaudio (Utilities|Array|Get(acopy) (Variables|/Game/Blueprints/Bluperints/BP_DialogManager.BP_DialogManager_C|GetDay2ArchibaldMonolog _dialogmanager) 36)))))
      (Utilities|Casting|CastToBP_FryingPan (Variables|/Game/Blueprints/Bluperints/BP_Character.BP_Character_C|GetCarriedObject _character_2)
        (:then
          (Default|PlayMonolog _dialogmanager_2 37)
          (Utilities|FlowControl|Delay (Variables|/Script/Engine.SoundBase|GetDuration (.lineaudio (Utilities|Array|Get(acopy) (Variables|/Game/Blueprints/Bluperints/BP_DialogManager.BP_DialogManager_C|GetDay2ArchibaldMonolog _dialogmanager_2) 37)))))
        (:CastFailed
          _))
      (CallFunction|StartStopQTE false)
      (Default|ProblemResolution (Variables|Default|GetLevelManager) 25 0.0))))

(event EventFail
  (bind _character (Variables|Default|GetCharacter))
  (bind _dialogmanager (Variables|Default|GetdialogManager))
  (bind _dialogmanager_2 (Variables|Default|GetdialogManager))
  (bind _dialogmanager_3 (Variables|Default|GetdialogManager))
  (Variables|Default|SetAcceptingInputs false)
  (switch int (Variables|Default|GetCurrentInteraction)
    (:0
      (Variables|/Game/Blueprints/Bluperints/BP_Character.BP_Character_C|SetisHurt (Variables|Default|GetCharacter) true)
      (CallFunction|HideInput)
      (Default|QTECameraControlMove (Variables|Default|GetCharacter) 0.1 (Transformation|GetWorldLocation (Variables|Default|GetKOPoint)))
      (Default|WalktheRail (Variables|Default|GetFirstFailRail))
      (Utilities|FlowControl|Delay 0.2)
      (Default|QTECameraControlMove (Variables|Default|GetCharacter) 0.4 (Transformation|GetWorldLocation (Variables|Default|GetInterestPoint1)))
      (Utilities|FlowControl|Delay 1.0)
      (Default|WalkBacktheRail (Variables|Default|GetFirstFailRail) 0.3)
      (Utilities|FlowControl|Delay 0.3)
      (Math|Integer|IncrementInt (Variables|Default|GetCurrentInteraction)
        (:%20%20
          (CallFunction|Event))))
    (:1
      (Variables|/Game/Blueprints/Bluperints/BP_Character.BP_Character_C|SetisHurt (Variables|Default|GetCharacter) true)
      (CallFunction|HideInput)
      (Default|QTECameraControlMove (Variables|Default|GetCharacter) 0.1 (Transformation|GetWorldLocation (Variables|Default|GetKOPoint2)))
      (Default|WalktheRail (Variables|Default|GetSecondFailRail))
      (Utilities|FlowControl|Delay 0.1)
      (Default|QTECameraControlMove (Variables|Default|GetCharacter) 0.1 (Transformation|GetWorldLocation (Variables|Default|GetKOPoint3)))
      (Default|Tumble (Variables|Default|GetHandRail))
      (Utilities|FlowControl|Delay 0.1)
      (Default|WalkBacktheRail (Variables|Default|GetSecondFailRail) 0.2)
      (Utilities|FlowControl|Delay 0.2)
      (Default|QTECameraControlMove (Variables|Default|GetCharacter) 0.1 (Transformation|GetWorldLocation (Variables|Default|GetKOPoint2)))
      (Utilities|FlowControl|Delay 0.5)
      (Default|QTECameraControlMove (Variables|Default|GetCharacter) 0.5 (Transformation|GetWorldLocation (Variables|Default|GetInterestPoint4)))
      (Utilities|FlowControl|Delay 0.5)
      (Math|Integer|IncrementInt (Variables|Default|GetCurrentInteraction)
        (:%20%20
          (CallFunction|Event))))
    (:2
      (Variables|/Game/Blueprints/Bluperints/BP_Character.BP_Character_C|SetisHurt (Variables|Default|GetCharacter) true)
      (CallFunction|HideInput)
      (Default|WalktheRail (Variables|Default|GetThirdFailRail))
      (Default|CamFall (Variables|Default|GetCharacter) 0.3 true)
      (Utilities|FlowControl|Delay 0.1)
      (Default|QTECameraControlMove (Variables|Default|GetCharacter) 0.2 (Transformation|GetWorldLocation (Variables|Default|GetKOPoint4)))
      (Utilities|FlowControl|Delay 1.2)
      (Default|CamFall (Variables|Default|GetCharacter) 1.5 false)
      (Default|QTECameraControlMove (Variables|Default|GetCharacter) 1.0 (Transformation|GetWorldLocation (Variables|Default|GetKOPoint5)))
      (Default|PlayMonolog _dialogmanager_2 35)
      (Utilities|FlowControl|Delay (Variables|/Script/Engine.SoundBase|GetDuration (.lineaudio (Utilities|Array|Get(acopy) (Variables|/Game/Blueprints/Bluperints/BP_DialogManager.BP_DialogManager_C|GetDay2ArchibaldMonolog _dialogmanager_2) 35))))
      (if (Variables|/Game/Blueprints/Bluperints/BP_Character.BP_Character_C|GetisHurt _character)
        (Default|PlayMonolog _dialogmanager_3 36)
        (Utilities|FlowControl|Delay (Variables|/Script/Engine.SoundBase|GetDuration (.lineaudio (Utilities|Array|Get(acopy) (Variables|/Game/Blueprints/Bluperints/BP_DialogManager.BP_DialogManager_C|GetDay2ArchibaldMonolog _dialogmanager_3) 36)))))
      (Utilities|Casting|CastToBP_FryingPan (Variables|/Game/Blueprints/Bluperints/BP_Character.BP_Character_C|GetCarriedObject _character)
        (:then
          (Default|PlayMonolog _dialogmanager 37)
          (Utilities|FlowControl|Delay (Variables|/Script/Engine.SoundBase|GetDuration (.lineaudio (Utilities|Array|Get(acopy) (Variables|/Game/Blueprints/Bluperints/BP_DialogManager.BP_DialogManager_C|GetDay2ArchibaldMonolog _dialogmanager) 37)))))
        (:CastFailed
          _))
      (CallFunction|StartStopQTE false)
      (Default|ProblemResolution (Variables|Default|GetLevelManager) 25 0.0))))

(fn ConstructionScript
  (|CallParentFunction))