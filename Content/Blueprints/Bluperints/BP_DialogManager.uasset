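; BP_DialogManager is an actor that runs branching, voiced conversations between the player character and a stored interlocutor.
; PlayLine plays audio and subtitles, waits out the clip, fires optional BP_LevelManager events, then chains by index to another line or question, or ends the dialog.
; PlayQuestion voices the question, then shows four answers (A/Z/E/R) on the dialog HUD.
; PlayAnswer resumes at the chosen line and restores the main HUD.
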(event Custom|PlayQuestion
  (params (Index :type Integer))
  (bind _character (Variables|Default|GetCharacter))
  (bind _character_2 (Variables|Default|GetCharacter))
  (bind _currentquestion (Variables|Default|GetCurrentQuestion))
  (bind _interlocutor (Variables|Default|GetInterlocutor))
  (bind _output (Utilities|Array|Get(acopy) _currentquestion Index))
  (bind _dialoghud (Variables|/Game/Blueprints/Bluperints/BP_Character.BP_Character_C|GetDialogHUD _character))
  (Variables|Default|SetCurrentQuestionIndex Index)
  (if (.isarchibaldquestion _output)
    (Class|BPIInterlocutor|PlaySound(Message) _interlocutor (.audio _output))
    (Class|BPIInterlocutor|DisplaySubtitle(Message) _interlocutor (.text _output))
    (else
      (Class|BPIInterlocutor|PlaySound(Message) _character_2 (.audio _output))
      (Class|BPIInterlocutor|DisplaySubtitle(Message) _character_2 (.text _output))))
  (Variables|Default|SetCurrentLineText (.text _output))
  (Utilities|FlowControl|Delay (Variables|/Script/Engine.SoundBase|GetDuration (.audio _output)))
  (Widget|SetVisibility _dialoghud "Visible")
  (Variables|/Game/Widgets/W_DialogHUD.W_DialogHUD_C|SetQuestionText _dialoghud (Variables|Default|GetCurrentLineText))
  (Default|SetAnswers _dialoghud (.linetext (Utilities|Array|Get(acopy) (Variables|Default|GetCurrentDialog) (.answeraindex _output))) (.linetext (Utilities|Array|Get(acopy) (Variables|Default|GetCurrentDialog) (.answerzindex _output))) (.linetext (Utilities|Array|Get(acopy) (Variables|Default|GetCurrentDialog) (.answereindex _output))) (.linetext (Utilities|Array|Get(acopy) (Variables|Default|GetCurrentDialog) (.answerrindex _output))))
  (Widget|SetVisibility (Variables|/Game/Blueprints/Bluperints/BP_Character.BP_Character_C|GetMainHUD _character) "Hidden")
  (Variables|/Game/Blueprints/Bluperints/BP_Character.BP_Character_C|SetisAnswering (Variables|Default|GetCharacter) true))

(event Custom|StartDialog
  (params (Interlocutor :type Actor%20Object%20Reference))
  (if (Utilities|DoesObjectImplementInterface Interlocutor "/Game/Blueprints/Interfaces/BPI_Interlocutor.BPI_Interlocutor_C")
    (Variables|Default|SetInterlocutor Interlocutor)))

(event Custom|PlayLine
  (params (Index :type Integer))
  (bind _mainhud (Variables|Default|GetMainHUD))
  (bind _currentdialog (Variables|Default|GetCurrentDialog))
  (bind _output (Utilities|Array|Get(acopy) _currentdialog Index))
  ;[1 1 1] Play Line
  (if (.isarchibaldline _output)
    (Class|BPIInterlocutor|PlaySound(Message) (Variables|Default|GetCharacter) (.lineaudio _output))
    (else
      (Class|BPIInterlocutor|PlaySound(Message) (Variables|Default|GetInterlocutor) (.lineaudio _output))))
  (Widget|SetVisibility _mainhud "Visible")
  (Variables|/Game/Widgets/W_MainHUD.W_MainHUD_C|SetSubtitle _mainhud (.linetext _output))
  (Utilities|FlowControl|Delay (Variables|/Script/Engine.SoundBase|GetDuration (.lineaudio _output)))
  (Variables|/Game/Widgets/W_MainHUD.W_MainHUD_C|SetSubtitle (Variables|/Game/Blueprints/Bluperints/BP_Character.BP_Character_C|GetMainHUD (Variables|Default|GetCharacter)) "")
  (if (.iseventtrigger _output)
    (Default|DialogEvents (Variables|Default|GetLevelManager) (.eventindex _output)))
  (if (.isfinisher _output)
    (Variables|/Game/Blueprints/Bluperints/BP_Character.BP_Character_C|SetisDialoging (Variables|Default|GetCharacter) false)
    (else
      ;;[0.1211 0.0913 1] If the line calls for another line from me, replay event
      (if (.leadstoquestion _output)
        (CallFunction|PlayQuestion (.leadsto _output))
        (else
          ;;[0.2183 0.1567 1] if Line calls for an answer, ask interlocutor
          (CallFunction|PlayLine (.leadsto _output)))))))

(event Custom|PlayAnswer
  (params (Answer :type BPE_Answer%20Enum :default "NewEnumerator0"))
  (bind _currentquestionindex (Variables|Default|GetCurrentQuestionIndex))
  (bind _currentquestion (Variables|Default|GetCurrentQuestion))
  (bind _character (Variables|Default|GetCharacter))
  (bind _output (Utilities|Array|Get(acopy) _currentquestion _currentquestionindex))
  (Variables|/Game/Blueprints/Bluperints/BP_Character.BP_Character_C|SetisAnswering (Variables|Default|GetCharacter) false)
  (switch Utilities|FlowControl|Switch|SwitchonBPE_Answer Answer
    (:NewEnumerator0
      (CallFunction|PlayLine (.answeraindex _output)))
    (:NewEnumerator1
      (CallFunction|PlayLine (.answerzindex _output)))
    (:NewEnumerator2
      (CallFunction|PlayLine (.answereindex _output)))
    (:NewEnumerator3
      (CallFunction|PlayLine (.answerrindex _output))))
  (Widget|SetVisibility (Variables|/Game/Blueprints/Bluperints/BP_Character.BP_Character_C|GetDialogHUD _character) "Hidden")
  (Widget|SetVisibility (Variables|/Game/Blueprints/Bluperints/BP_Character.BP_Character_C|GetMainHUD _character) "Visible"))

(event EventBeginPlay
  (bind _asbp_character (Utilities|Casting|CastToBP_Character (Game|GetPlayerCharacter 0)))
  (bind _output_get (Variables|Default|SetCharacter _asbp_character))
  (Variables|Default|SetMainHUD (Variables|/Game/Blueprints/Bluperints/BP_Character.BP_Character_C|GetMainHUD _output_get))
  (bind _outactors (Actor|GetAllActorsOfClass "/Game/Blueprints/Bluperints/BP_LevelManager.BP_LevelManager_C"))
  (Variables|Default|SetLevelManager (Utilities|Array|Get(acopy) _outactors)))

(event Collision|EventActorBeginOverlap
  (params (OtherActor :type Actor%20Object%20Reference)))

(event EventTick
  (params (DeltaSeconds :type Float%20%28single-precision%29)))

(fn ConstructionScript)