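; BP_Bible is a grabbable, physics-driven Bible prop that the player carries and that advances a level objective.
; Grab disables physics, snaps the mesh to the root with an offset, attaches to the character's AttachPoint socket and sets the carry state, which Release undoes.
; Grabbing it on day 3 during problem 23 tells BP_LevelManager to resolve to problem 24, stores the Bible there and clears the HUD objective.
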(event EventBeginPlay)

(event Collision|EventActorBeginOverlap
  (params (OtherActor :type Actor%20Object%20Reference)))

(event EventTick
  (params (DeltaSeconds :type Float%20%28single-precision%29)))

(event EventRelease
  (Transformation|SetRelativeLocationAndRotation (Variables|Default|GetBible) "0, 0, 0" "0, 0, 0" false false)
  (Transformation|DetachFromActor "KeepWorld" "KeepWorld" "KeepWorld")
  (bind _asbp_character (Utilities|Casting|CastToBP_Character (Game|GetPlayerCharacter 0)))
  (Variables|/Game/Blueprints/Bluperints/BP_Character.BP_Character_C|SetCaryObject _asbp_character false)
  (Variables|/Game/Blueprints/Bluperints/BP_Character.BP_Character_C|SetCarriedObject _asbp_character 0)
  (Physics|SetSimulatePhysics (Variables|Default|GetBible) true))

(event EventGrab
  (params (Character :type Skeletal%20Mesh%20Component%20Object%20Reference))
  (Transformation|AttachComponentToComponent (Variables|Default|GetBible) (Variables|Default|GetDefaultSceneRoot) "None" "SnapToTarget" "SnapToTarget" "KeepWorld" true)
  (Transformation|SetRelativeLocationAndRotation (Variables|Default|GetBible) "5.400000,7.230000,1.600000" "-14.000000,-219.000000,17.500000" false false)
  (Physics|SetSimulatePhysics (Variables|Default|GetBible) false)
  (bind _asbp_character (Utilities|Casting|CastToBP_Character (Game|GetPlayerCharacter 0)))
  (Variables|/Game/Blueprints/Bluperints/BP_Character.BP_Character_C|SetCaryObject _asbp_character true)
  (Variables|/Game/Blueprints/Bluperints/BP_Character.BP_Character_C|SetCarriedObject _asbp_character self)
  (Transformation|AttachComponentToComponent Character "AttachPoint" "SnapToTarget" "SnapToTarget" "KeepWorld" false)
  (bind _outactors (Actor|GetAllActorsOfClass "/Game/Blueprints/Bluperints/BP_LevelManager.BP_LevelManager_C"))
  (if (and (== (Variables|/Game/Blueprints/Bluperints/BP_LevelManager.BP_LevelManager_C|GetCurrentDay (Utilities|Array|Get(acopy) _outactors)) 3) (== (Variables|/Game/Blueprints/Bluperints/BP_LevelManager.BP_LevelManager_C|GetCurrentProblem (Utilities|Array|Get(acopy) _outactors)) 23))
    (Default|ProblemResolution (Utilities|Array|Get(acopy) _outactors) 24 0.0)
    (Variables|/Game/Blueprints/Bluperints/BP_LevelManager.BP_LevelManager_C|SetBible (Utilities|Array|Get(acopy) _outactors) self)
    (Variables|/Game/Widgets/W_MainHUD.W_MainHUD_C|SetCurrentObjective (Variables|/Game/Blueprints/Bluperints/BP_LevelManager.BP_LevelManager_C|GetMainHUD (Utilities|Array|Get(acopy) _outactors)) "")))

(event EventShowGrabInteraction
  (bind _asbp_character (Utilities|Casting|CastToBP_Character (Game|GetPlayerCharacter 0)))
  (Default|ChangeGrabHUD _asbp_character "Grab the Bible" true))

(fn ConstructionScript)