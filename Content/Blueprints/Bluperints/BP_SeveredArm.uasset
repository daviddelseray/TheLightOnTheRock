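; Severed arm prop that the player can grab, carry and throw as part of a Day 2 story sequence.
; Activate reveals the arm and enables its trigger sphere, whose player overlap can advance BP_LevelManager's current problem.
; Grab disables capsule physics and attaches to the character's AttachPoint; Release reverses this.
; Interact while held calls the character's Throw and flags the throw on the level manager at the matching story step.
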(event OnComponentBeginOverlap(Sphere)
  (params (OverlappedComponent :type Primitive%20Component%20Object%20Reference) (OtherActor :type Actor%20Object%20Reference) (OtherComp :type Primitive%20Component%20Object%20Reference) (OtherBodyIndex :type Integer) (bFromSweep :type Boolean) (SweepResult :type Hit%20Result%20Structure%20%28by%20ref%29))
  (Utilities|Casting|CastToBP_Character OtherActor)
  (bind _outactors (Actor|GetAllActorsOfClass "/Game/Blueprints/Bluperints/BP_LevelManager.BP_LevelManager_C"))
  (if (and (== (Variables|/Game/Blueprints/Bluperints/BP_LevelManager.BP_LevelManager_C|GetCurrentDay (Utilities|Array|Get(acopy) _outactors)) 2) (== (Variables|/Game/Blueprints/Bluperints/BP_LevelManager.BP_LevelManager_C|GetCurrentProblem (Utilities|Array|Get(acopy) _outactors)) 25))
    (Default|ProblemResolution (Utilities|Array|Get(acopy) _outactors) 26 0.0)))

(event Custom|Activate
  (bind _sphere (Variables|Default|GetSphere))
  (Rendering|SetVisibility (Variables|Default|Getarm) true false)
  (Collision|SetCollisionEnabled _sphere "QueryOnly")
  (Class|PrimitiveComponent|WakeRigidBody _sphere "None"))

(event EventBeginPlay)

(event Collision|EventActorBeginOverlap
  (params (OtherActor :type Actor%20Object%20Reference)))

(event EventTick
  (params (DeltaSeconds :type Float%20%28single-precision%29)))

(event EventGrab
  (params (Character :type Skeletal%20Mesh%20Component%20Object%20Reference))
  (Transformation|AttachComponentToComponent (Variables|Default|GetCapsule) (Variables|Default|GetDefaultSceneRoot) "None" "SnapToTarget" "SnapToTarget" "KeepWorld" true)
  (Physics|SetSimulatePhysics (Variables|Default|GetCapsule) false)
  (bind _asbp_character (Utilities|Casting|CastToBP_Character (Game|GetPlayerCharacter 0)))
  (Variables|/Game/Blueprints/Bluperints/BP_Character.BP_Character_C|SetCaryObject _asbp_character true)
  (Variables|/Game/Blueprints/Bluperints/BP_Character.BP_Character_C|SetCarriedObject _asbp_character self)
  (Transformation|AttachComponentToComponent Character "AttachPoint" "SnapToTarget" "SnapToTarget" "KeepWorld" false)
  (Variables|Default|SetisGrabbed true))

(event EventInteract
  (if (Variables|Default|GetisGrabbed)
    (bind _asbp_character (Utilities|Casting|CastToBP_Character (Game|GetPlayerCharacter 0)))
    (Default|Throw _asbp_character (Variables|Default|GetCapsule))
    (bind _outactors (Actor|GetAllActorsOfClass "/Game/Blueprints/Bluperints/BP_LevelManager.BP_LevelManager_C"))
    (if (and (== (Variables|/Game/Blueprints/Bluperints/BP_LevelManager.BP_LevelManager_C|GetCurrentDay (Utilities|Array|Get(acopy) _outactors)) 2) (== (Variables|/Game/Blueprints/Bluperints/BP_LevelManager.BP_LevelManager_C|GetCurrentProblem (Utilities|Array|Get(acopy) _outactors)) 27))
      (Variables|/Game/Blueprints/Bluperints/BP_LevelManager.BP_LevelManager_C|SethasThrownTheArm (Utilities|Array|Get(acopy) _outactors) true))))

(event EventRelease
  (Transformation|DetachFromActor "KeepWorld" "KeepWorld" "KeepWorld")
  (bind _asbp_character (Utilities|Casting|CastToBP_Character (Game|GetPlayerCharacter 0)))
  (Variables|/Game/Blueprints/Bluperints/BP_Character.BP_Character_C|SetCaryObject _asbp_character false)
  (Variables|/Game/Blueprints/Bluperints/BP_Character.BP_Character_C|SetCarriedObject _asbp_character 0)
  (Physics|SetSimulatePhysics (Variables|Default|GetCapsule) true)
  (Variables|Default|SetisGrabbed false))

(event EventShowGrabInteraction
  (bind _asbp_character (Utilities|Casting|CastToBP_Character (Game|GetPlayerCharacter 0)))
  (Default|ChangeGrabHUD _asbp_character "Grab the arm" true))

(fn ConstructionScript)