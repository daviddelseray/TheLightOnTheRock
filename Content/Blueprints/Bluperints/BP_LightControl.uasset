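; Level lighting controller that fades, flickers and shuts down all point lights, plus referenced Spotlight and Lantern fixtures.
; TurnOn drives intensity with a timeline, then turns off the player character's light; ShutDown kills the lights and turns it on.
; Flickering re-calls itself after random delays, alternating on and off via FlipFlop while Flicker is set.
; With Shut true, it counts flickers and calls ShutDown once past the limit.
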(event Custom|ShutDown
  (Variables|Default|SetFlicker false)
  (for _array_element (Variables|Default|GetLights)
    (bind _aspoint_light (Utilities|Casting|CastToPointLight _array_element))
    (Rendering|Components|Light|SetIntensity (Variables|/Script/Engine.PointLight|GetPointLightComponent _aspoint_light) 0.0))
  (Default|TurnOff (Variables|Default|GetSpotlight))
  (Default|ShutDown (Variables|Default|GetLantern))
  (bind _asbp_character (Utilities|Casting|CastToBP_Character (Game|GetPlayerCharacter 0)))
  (Default|TurnonLight _asbp_character))

(event Custom|Flickering
  (params (Shut :type Boolean))
  ;[1 1 1] Flow Control
  (if Shut
    (if (<= (Variables|Default|GetFlickerOccur) 10)
      (if (Variables|Default|GetFlicker) :!label _label
        (bind _output_get (Variables|Default|SetFlickeringTime (Math|Random|RandomFloatinRange 0.03 0.15)))
        (Utilities|FlowControl|Delay _output_get)
        ;[1 1 1] Alternate Max Intensity and 0 with all the pointlight
        (bind _isa (Utilities|FlowControl|FlipFlop)
          (:A
            _)
          (:B
            _))
        (for _array_element (Variables|Default|GetLights)
          (bind _aspoint_light (Utilities|Casting|CastToPointLight _array_element))
          (if _isa
            (Rendering|Components|Light|SetIntensity (Variables|/Script/Engine.PointLight|GetPointLightComponent _aspoint_light) (Variables|Default|GetMaxIntensity))
            (else
              (Rendering|Components|Light|SetIntensity (Variables|/Script/Engine.PointLight|GetPointLightComponent _aspoint_light) 0.0))))
        (if _isa
          (Default|Turnon (Variables|Default|GetSpotlight))
          (Default|Turnon (Variables|Default|GetLantern))
          (else
            (Default|TurnOff (Variables|Default|GetSpotlight))
            (Default|ShutDown (Variables|Default|GetLantern))))
        (if Shut
          (Math|Integer|IncrementInt (Variables|Default|GetFlickerOccur)
            (:%20%20
              _)))
        (CallFunction|Flickering Shut))
      (else
        (Variables|Default|SetFlickerOccur 0)
        (CallFunction|ShutDown)))
    (else
      (goto _label))))

(event Custom|TurnOn
  (bind _currentintensity (Timeline|IntensityTurnOn Play)
    (:Update
      (for _array_element (Variables|Default|GetLights)
        (bind _aspoint_light (Utilities|Casting|CastToPointLight _array_element))
        (Rendering|Components|Light|SetIntensity (Variables|/Script/Engine.PointLight|GetPointLightComponent _aspoint_light) _currentintensity))
      (for _array_element_2 (Variables|Default|GetSpotlights)
        (Rendering|Components|Light|SetIntensity _array_element_2 _currentintensity)))
    (:Finished
      (bind _asbp_character (Utilities|Casting|CastToBP_Character (Game|GetPlayerCharacter 0)))
      (Default|TurnOffLight _asbp_character))))

(event EventBeginPlay
  (bind _outactors (Actor|GetAllActorsOfClass "/Script/Engine.PointLight"))
  (Variables|Default|SetLights _outactors)
  (Utilities|Array|Add (Variables|Default|GetSpotlights) (Variables|/Game/Blueprints/Bluperints/BP_WallWalkSpotlight.BP_WallWalkSpotlight_C|GetSpotLight (Variables|Default|GetSpotlight)))
  (Utilities|Array|Add (Variables|Default|GetSpotlights) (Variables|/Game/Blueprints/Bluperints/BP_Light.BP_Light_C|GetSpotLight (Variables|Default|GetLantern)))
  (Utilities|Array|Add (Variables|Default|GetSpotlights) (Variables|/Game/Blueprints/Bluperints/BP_Light.BP_Light_C|GetSpotLight1 (Variables|Default|GetLantern))))

(event Collision|EventActorBeginOverlap
  (params (OtherActor :type Actor%20Object%20Reference)))

(event EventTick
  (params (DeltaSeconds :type Float%20%28single-precision%29)))

(fn ConstructionScript)