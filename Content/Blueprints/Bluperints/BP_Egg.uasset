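; BP_Egg is a grabbable egg the player can carry, with intact and cracked states.
; The HUD prompt and the monolog played on first grab through BP_DialogManager depend on IsCracked, while Crack only swaps the mesh.
; Grab re-seats the physics mesh on the root, disables simulation, attaches to AttachPoint and registers as BP_Character's carried object.
; Release detaches it, clears that reference and restores physics.
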(event Custom|Crack
  (Components|StaticMesh|SetStaticMesh (Variables|Default|GetEgg) "/Game/DAvid3DAssets/CrackedEgg.CrackedEgg"))

(event EventBeginPlay)

(event Collision|EventActorBeginOverlap
  (params (OtherActor :type Actor%20Object%20Reference)))

(event EventTick
  (params (DeltaSeconds :type Float%20%28single-precision%29)))

(event EventRelease
  (Transformation|SetRelativeLocation (Variables|Default|GetEgg) "0, 0, 0" false false)
  (Transformation|DetachFromActor "KeepWorld" "KeepWorld" "KeepWorld")
  (bind _asbp_character (Utilities|Casting|CastToBP_Character (Game|GetPlayerCharacter 0)))
  (Variables|/Game/Blueprints/Bluperints/BP_Character.BP_Character_C|SetCaryObject _asbp_character false)
  (Variables|/Game/Blueprints/Bluperints/BP_Character.BP_Character_C|SetCarriedObject _asbp_character 0)
  (Physics|SetSimulatePhysics (Variables|Default|GetEgg) true))

(event EventGrab
  (params (Character :type Skeletal%20Mesh%20Component%20Object%20Reference))
  (Transformation|AttachComponentToComponent (Variables|Default|GetEgg) (Variables|Default|GetDefaultSceneRoot) "None" "SnapToTarget" "SnapToTarget" "KeepWorld" true)
  (Transformation|SetRelativeLocation (Variables|Default|GetEgg) "0, 0, 0" false false)
  (Physics|SetSimulatePhysics (Variables|Default|GetEgg) false)
  (bind _asbp_character (Utilities|Casting|CastToBP_Character (Game|GetPlayerCharacter 0)))
  (Variables|/Game/Blueprints/Bluperints/BP_Character.BP_Character_C|SetCaryObject _asbp_character true)
  (Variables|/Game/Blueprints/Bluperints/BP_Character.BP_Character_C|SetCarriedObject _asbp_character self)
  (Transformation|AttachComponentToComponent Character "AttachPoint" "SnapToTarget" "SnapToTarget" "KeepWorld" false)
  (if (Variables|Default|GetisFirstGrab)
    (Variables|Default|SetisFirstGrab false)
    (bind _outactors (Actor|GetAllActorsOfClass "/Game/Blueprints/Bluperints/BP_DialogManager.BP_DialogManager_C"))
    (if (Variables|Default|GetisCracked)
      (Default|PlayMonolog (Utilities|Array|Get(acopy) _outactors) 27)
      (else
        (Default|PlayMonolog (Utilities|Array|Get(acopy) _outactors) 28)))))

(event EventShowGrabInteraction
  (bind _asbp_character (Utilities|Casting|CastToBP_Character (Game|GetPlayerCharacter 0)))
  (if (Variables|Default|GetisCracked)
    (Default|ChangeGrabHUD _asbp_character "Grab the cracked egg" true)
    (else
      (Default|ChangeGrabHUD _asbp_character "Grab the egg" true))))

(fn ConstructionScript)