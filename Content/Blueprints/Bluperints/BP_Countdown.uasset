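; BP_Countdown is a "strange clock" prop that the player can grab, carry and look at to advance scripted problems.
; Grab and Release toggle physics on the Countdown component, attach or detach it at the character's AttachPoint, and update BP_Character's carry state.
; Interaction events drive the character's grab and look-at HUD prompts.
; LookedAt resolves specific day and problem steps through the BP_LevelManager found on BeginPlay.
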(event Custom|RevealLookAtInteraction
  (params (isVisible :type Boolean))
  (bind _asbp_character (Utilities|Casting|CastToBP_Character (Game|GetPlayerCharacter 0)))
  (Default|ChangeLookatHUD _asbp_character "Look at the strange clock" isVisible))

(event Custom|LookedAt
  (bind _levelmanager (Variables|Default|GetLevelManager))
  (bind _levelmanager_2 (Variables|Default|GetLevelManager))
  (if (and (== (Variables|/Game/Blueprints/Bluperints/BP_LevelManager.BP_LevelManager_C|GetCurrentDay _levelmanager_2) 1) (== (Variables|/Game/Blueprints/Bluperints/BP_LevelManager.BP_LevelManager_C|GetCurrentProblem _levelmanager_2) 14))
    (Default|ProblemResolution _levelmanager_2 15 0.0)
    (elif (and (== (Variables|/Game/Blueprints/Bluperints/BP_LevelManager.BP_LevelManager_C|GetCurrentDay _levelmanager) 2) (== (Variables|/Game/Blueprints/Bluperints/BP_LevelManager.BP_LevelManager_C|GetCurrentProblem _levelmanager) 12))
      (Default|ProblemResolution _levelmanager 13 0.0))))

(event EventBeginPlay
  (bind _outactors (Actor|GetAllActorsOfClass "/Game/Blueprints/Bluperints/BP_LevelManager.BP_LevelManager_C"))
  (Variables|Default|SetLevelManager (Utilities|Array|Get(acopy) _outactors)))

(event Collision|EventActorBeginOverlap
  (params (OtherActor :type Actor%20Object%20Reference)))

(event EventTick
  (params (DeltaSeconds :type Float%20%28single-precision%29)))

(event EventGrab
  (params (Character :type Skeletal%20Mesh%20Component%20Object%20Reference))
  (Transformation|AttachComponentToComponent (Variables|Default|Getcountdown) (Variables|Default|GetDefaultSceneRoot) "None" "SnapToTarget" "SnapToTarget" "KeepWorld" true)
  (Transformation|SetRelativeLocation (Variables|Default|Getcountdown) "-5.000000, 0, 0" false false)
  (Physics|SetSimulatePhysics (Variables|Default|Getcountdown) false)
  (bind _asbp_character (Utilities|Casting|CastToBP_Character (Game|GetPlayerCharacter 0)))
  (Variables|/Game/Blueprints/Bluperints/BP_Character.BP_Character_C|SetCaryObject _asbp_character true)
  (Variables|/Game/Blueprints/Bluperints/BP_Character.BP_Character_C|SetCarriedObject _asbp_character self)
  (Transformation|AttachComponentToComponent Character "AttachPoint" "SnapToTarget" "SnapToTarget" "KeepWorld" false)
  (CallFunction|RevealLookatInteraction true)
  (Transformation|SetRelativeRotation (Variables|Default|GetDefaultSceneRoot) "-50.000000,-50.000000,45.000000" false false)
  (Variables|Default|SetisGrabbed true))

(event EventRelease
  (Transformation|DetachFromActor "KeepWorld" "KeepWorld" "KeepWorld")
  (Transformation|AttachComponentToComponent (Variables|Default|Getcountdown) (Variables|Default|GetDefaultSceneRoot) "None" "SnapToTarget" "SnapToTarget" "KeepWorld" true)
  (bind _asbp_character (Utilities|Casting|CastToBP_Character (Game|GetPlayerCharacter 0)))
  (Variables|/Game/Blueprints/Bluperints/BP_Character.BP_Character_C|SetCaryObject _asbp_character false)
  (Variables|/Game/Blueprints/Bluperints/BP_Character.BP_Character_C|SetCarriedObject _asbp_character 0)
  (Physics|SetSimulatePhysics (Variables|Default|Getcountdown) true)
  (Variables|Default|SetisGrabbed false)
  (CallFunction|RevealLookatInteraction false))

(event EventShowGrabInteraction
  (bind _asbp_character (Utilities|Casting|CastToBP_Character (Game|GetPlayerCharacter 0)))
  (Default|ChangeGrabHUD _asbp_character "Grab the strange clock" true))

(fn ConstructionScript)