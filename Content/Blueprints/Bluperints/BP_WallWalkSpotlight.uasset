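; Carryable spotlight that the player can switch on or off while its linked generator is running.
; Activate and Interact share one toggle that sets light intensity, while tracking mode copies the first-person camera's rotation to the spotlight root each tick.
; Grab attaches it to the character's attach socket and records it as the carried object.
; Release re-docks it only at its own watch point, restoring rest transform and clearing the carry state.
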(event Custom|TurnOn
  ;[1 1 1] LightControl
  (Rendering|Components|Light|SetIntensity (Variables|Default|GetSpotLight) (Variables|Default|GetMaxIntensity))
  (Variables|Default|SetIsLightOn true))

(event Custom|Init
  (Transformation|AttachComponentToComponent (Variables|/Game/Blueprints/Bluperints/BP_SpotlightAttach.BP_SpotlightAttach_C|GetAttachPoint (Variables|Default|GetAttach)) "None" "KeepWorld" "KeepWorld" "KeepWorld" true))

(event Custom|TurnOff
  ;[1 1 1] LightControl
  (Rendering|Components|Light|SetIntensity (Variables|Default|GetSpotLight) 0.0)
  (Variables|Default|SetIsLightOn false))

(event Custom|StartTracking
  (Variables|Default|SetisTracking true))

(event Custom|StopTracking
  (Variables|Default|SetisTracking false))

(event EventBeginPlay)

(event Collision|EventActorBeginOverlap
  (params (OtherActor :type Actor%20Object%20Reference)))

(event EventAttachtoElement
  (params (Target :type Scene%20Component%20Object%20Reference))
  (Transformation|DetachFromActor "KeepWorld" "KeepWorld" "KeepWorld")
  (Transformation|AttachComponentToComponent Target "None" "SnapToTarget" "SnapToTarget" "KeepRelative" true)
  (Transformation|SetWorldTransform (Variables|Default|GetDefaultSceneRoot) (Variables|Default|GetRestSettings) false false)
  (bind _asbp_character (Utilities|Casting|CastToBP_Character (Game|GetPlayerCharacter 0)))
  (Variables|/Game/Blueprints/Bluperints/BP_Character.BP_Character_C|SetCaryObject _asbp_character false)
  (Variables|/Game/Blueprints/Bluperints/BP_Character.BP_Character_C|SetCarriedObject _asbp_character 0)
  (Variables|/Game/Blueprints/Bluperints/BP_SpotlightAttach.BP_SpotlightAttach_C|SetisLoaded (Variables|Default|GetAttach) true))

(event EventActivate
  ;[1 1 1] LightControl
  (if (Variables|/Game/Blueprints/Bluperints/BP_Generator.BP_Generator_C|GetisOn (Variables|Default|GetGenerator))
    (if (Variables|Default|GetIsLightOn)
      (CallFunction|TurnOff)
      (else
        (CallFunction|Turnon)))))

(event EventInteract
  ;[1 1 1] LightControl
  (if (Variables|/Game/Blueprints/Bluperints/BP_Generator.BP_Generator_C|GetisOn (Variables|Default|GetGenerator))
    (if (Variables|Default|GetIsLightOn)
      (CallFunction|TurnOff)
      (else
        (CallFunction|Turnon)))))

(event EventTick
  (params (DeltaSeconds :type Float%20%28single-precision%29))
  (if (Variables|Default|GetisTracking)
    (bind _asbp_character (Utilities|Casting|CastToBP_Character (Game|GetPlayerCharacter 0)))
    (Transformation|SetWorldRotation (Variables|Default|GetSpotlightRoot) (Transformation|GetWorldRotation (Variables|/Game/Blueprints/Bluperints/BP_Character.BP_Character_C|GetFirstPersonCamera _asbp_character)) false false)))

(event EventRelease
  (bind _asbp_character (Utilities|Casting|CastToBP_Character (Game|GetPlayerCharacter 0)))
  (if (and (Variables|/Game/Blueprints/Bluperints/BP_Character.BP_Character_C|GetatWatchPoint _asbp_character) (== (Variables|/Game/Blueprints/Bluperints/BP_Character.BP_Character_C|GetWatchPoint _asbp_character) (Variables|Default|GetAttach)))
    (CallFunction|AttachtoElement (Variables|/Game/Blueprints/Bluperints/BP_SpotlightAttach.BP_SpotlightAttach_C|GetAttachPoint (Variables|Default|GetAttach)))))

(event EventGrab
  (params (Character :type Skeletal%20Mesh%20Component%20Object%20Reference))
  (Transformation|DetachFromActor "KeepWorld" "KeepWorld" "KeepWorld")
  (Transformation|AttachComponentToComponent Character "AttachPoint" "SnapToTarget" "SnapToTarget" "KeepWorld" true)
  (bind _asbp_character (Utilities|Casting|CastToBP_Character (Game|GetPlayerCharacter 0)))
  (Variables|/Game/Blueprints/Bluperints/BP_Character.BP_Character_C|SetCaryObject _asbp_character true)
  (Variables|/Game/Blueprints/Bluperints/BP_Character.BP_Character_C|SetCarriedObject _asbp_character self))

(fn ConstructionScript)