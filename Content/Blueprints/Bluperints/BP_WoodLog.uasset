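; A carryable wood log the player can grab, throw, drop or attach to another component.
; Grab turns off physics, snaps the log to the character's AttachPoint socket and updates the player's carried-object state and HUD prompt.
; Interact hands the held log to BP_Character's Throw, Release detaches it with physics back on, and AttachtoElement snaps it onto a target.
; Each event re-parents or re-offsets the mesh and reaches the character by casting player 0.
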(event EventBeginPlay)

(event Collision|EventActorBeginOverlap
  (params (OtherActor :type Actor%20Object%20Reference)))

(event EventAttachtoElement
  (params (Target :type Scene%20Component%20Object%20Reference))
  (Transformation|DetachFromActor "KeepWorld" "KeepWorld" "KeepWorld")
  (Transformation|AttachComponentToComponent (Variables|Default|GetWoodLog) (Variables|Default|GetDefaultSceneRoot) "None" "SnapToTarget" "SnapToTarget" "KeepWorld" true)
  (Transformation|SetRelativeLocationAndRotation (Variables|Default|GetWoodLog) "0, 0, 0" "0, 0, 0" false false)
  (Transformation|AttachComponentToComponent Target "None" "SnapToTarget" "SnapToTarget" "KeepWorld" true)
  (bind _asbp_character (Utilities|Casting|CastToBP_Character (Game|GetPlayerCharacter 0)))
  (Variables|/Game/Blueprints/Bluperints/BP_Character.BP_Character_C|SetCaryObject _asbp_character false)
  (Variables|/Game/Blueprints/Bluperints/BP_Character.BP_Character_C|SetCarriedObject _asbp_character 0))

(event EventTick
  (params (DeltaSeconds :type Float%20%28single-precision%29)))

(event EventInteract
  (if (Variables|Default|GetisGrabbed)
    (Transformation|SetRelativeLocation (Variables|Default|GetWoodLog) "0, 0, 0" false false)
    (bind _asbp_character (Utilities|Casting|CastToBP_Character (Game|GetPlayerCharacter 0)))
    (Default|Throw _asbp_character (Variables|Default|GetWoodLog))
    (Variables|Default|SetisGrabbed false)))

(event EventRelease
  (Transformation|SetRelativeLocation (Variables|Default|GetWoodLog) "0, 0, 0" false false)
  (Transformation|DetachFromActor "KeepWorld" "KeepWorld" "KeepWorld")
  (bind _asbp_character (Utilities|Casting|CastToBP_Character (Game|GetPlayerCharacter 0)))
  (Variables|/Game/Blueprints/Bluperints/BP_Character.BP_Character_C|SetCaryObject _asbp_character false)
  (Variables|/Game/Blueprints/Bluperints/BP_Character.BP_Character_C|SetCarriedObject _asbp_character 0)
  (Physics|SetSimulatePhysics (Variables|Default|GetWoodLog) true)
  (Variables|Default|SetisGrabbed false))

(event EventGrab
  (params (Character :type Skeletal%20Mesh%20Component%20Object%20Reference))
  (Transformation|AttachComponentToComponent (Variables|Default|GetWoodLog) (Variables|Default|GetDefaultSceneRoot) "None" "SnapToTarget" "SnapToTarget" "KeepWorld" true)
  (Transformation|SetRelativeLocationAndRotation (Variables|Default|GetWoodLog) "15.000000,3.200000,2.000000" "0,30.000000,107.000000" false false)
  (Physics|SetSimulatePhysics (Variables|Default|GetWoodLog) false)
  (bind _asbp_character (Utilities|Casting|CastToBP_Character (Game|GetPlayerCharacter 0)))
  (Variables|/Game/Blueprints/Bluperints/BP_Character.BP_Character_C|SetCaryObject _asbp_character true)
  (Variables|/Game/Blueprints/Bluperints/BP_Character.BP_Character_C|SetCarriedObject _asbp_character self)
  (Transformation|AttachComponentToComponent Character "AttachPoint" "SnapToTarget" "SnapToTarget" "KeepWorld" false)
  (Variables|/Game/Blueprints/Bluperints/BP_Character.BP_Character_C|SetGrabbedInteraction _asbp_character "Throw away")
  (Variables|Default|SetisGrabbed true)
  (Default|ShowGrabbedInteraction _asbp_character))

(event EventShowGrabInteraction
  (bind _asbp_character (Utilities|Casting|CastToBP_Character (Game|GetPlayerCharacter 0)))
  (Default|ChangeGrabHUD _asbp_character "Grab the wood log" true))

(fn ConstructionScript)