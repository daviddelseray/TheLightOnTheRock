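; BP_Fusebox is a lever puzzle that uses audio feedback to signal how close the lever states are to a reference sequence.
; Activate starts the parasite noise and loops the ProperSequence Morse sound until StopPlaying.
; ReceiveInput stores each lever change, and Compare crossfades the noise down and the Morse up by the share of matching levers.
; A full match calls ProblemResolution on BP_LevelManager to move to the next problem.
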(event Custom|Activate
  (CallFunction|Compare)
  (Audio|Components|Audio|Play (Variables|Default|GetParasites) 0.0)
  (Variables|Default|SetshouldLoop? true)
  (CallFunction|LoopPlayMorse))

(event Custom|LoopPlayMorse
  (bind _propersequence (Variables|Default|GetProperSequence))
  (if (Variables|Default|GetshouldLoop?)
    (Audio|Components|Audio|Play _propersequence 0.0)
    (Utilities|FlowControl|Delay (+ (Variables|/Script/Engine.SoundBase|GetDuration (Variables|/Script/Engine.AudioComponent|GetSound _propersequence)) 1.0))
    (CallFunction|LoopPlayMorse)))

(event Custom|StopPlaying
  (Variables|Default|SetshouldLoop? false)
  (Audio|Components|Audio|Stop (Variables|Default|GetProperSequence))
  (Audio|Components|Audio|Stop (Variables|Default|GetParasites)))

(event EventBeginPlay
  (for _array_element (Variables|Default|GetLevers)
    (Utilities|Array|Add (Variables|Default|GetLeversState) (Variables|/Game/Blueprints/Bluperints/BP_FuseBoxLever.BP_FuseBoxLever_C|GetIsUp _array_element))))

(event Collision|EventActorBeginOverlap
  (params (OtherActor :type Actor%20Object%20Reference)))

(event EventTick
  (params (DeltaSeconds :type Float%20%28single-precision%29)))

(fn ConstructionScript)

(fn ReceiveInput
  (params (Index :type Integer) (LeverState :type Boolean))
  (Utilities|Array|SetArrayElem (Variables|Default|GetLeversState) Index LeverState)
  (CallFunction|Compare))

(fn Compare
  (bind _levers (Variables|Default|GetLevers))
  (bind _goodlevers (LocalVariables|GetgoodLevers))
  (bind _returnvalue (Utilities|Array|Length _levers))
  (bind _returnvalue_2 (Math|Conversions|ToFloat(Integer) _returnvalue))
  (bind _returnvalue_3 (/ _goodlevers _returnvalue_2))
  (for (_array_element _array_index) (Variables|Default|GetLeversState)
    (if (Math|Boolean|Equal(Boolean) _array_element (Utilities|Array|Get(acopy) (Variables|Default|GetReferenceSequence) _array_index))
      (Math|Float|IncrementFloat (LocalVariables|GetgoodLevers))))
  (Audio|Components|Audio|SetVolumeMultiplier (Variables|Default|GetParasites) (- 1.0 _returnvalue_3) :!class /Script/Engine.AudioComponent)
  (Audio|Components|Audio|SetVolumeMultiplier (Variables|Default|GetProperSequence) (/ _returnvalue_3 2.0) :!class /Script/Engine.AudioComponent)
  (if (== _returnvalue_3 1.0)
    (bind _outactors (Actor|GetAllActorsOfClass "/Game/Blueprints/Bluperints/BP_LevelManager.BP_LevelManager_C"))
    (Default|ProblemResolution (Utilities|Array|Get(acopy) _outactors) 9 3.0)))