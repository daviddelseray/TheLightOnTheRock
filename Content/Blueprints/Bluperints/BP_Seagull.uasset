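; BP_Seagull is a seagull that flies along a spline and can dive at the player.
; Activate shows its mesh and starts a timeline-driven spline flight, optionally looping.
; AttackPlayer halts the flight, and Tick then homes the mesh toward the player by a fixed per-frame step, unscaled by delta time.
; Overlapping BP_Character ends the attack, and a second timeline lerps it back to the spline start to resume flying.
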(event OnComponentBeginOverlap(Cube)
  (params (OverlappedComponent :type Primitive%20Component%20Object%20Reference) (OtherActor :type Actor%20Object%20Reference) (OtherComp :type Primitive%20Component%20Object%20Reference) (OtherBodyIndex :type Integer) (bFromSweep :type Boolean) (SweepResult :type Hit%20Result%20Structure%20%28by%20ref%29))
  (Utilities|Casting|CastToBP_Character OtherActor)
  (CallFunction|StopAttack))

(event Custom|FlyAlongSpline
  (Components|Timeline|SetPlayRate (Variables|Default|GetTrajectAlongSpline) (/ 1.0 (Variables|Default|GetFlyDuration)))
  (bind _progressalongspline (Timeline|TrajectAlongSpline PlayFromStart)
    (:Update
      (CallFunction|Fly _progressalongspline))
    (:Finished
      (if (Variables|Default|GetisLooping)
        (CallFunction|FlyAlongSpline)))))

(event Custom|AttackPlayer
  (CallFunction|BreakFlight)
  (Variables|Default|SetisAttacking true))

(event Custom|BreakFlight
  (bind _progressalongspline (Timeline|TrajectAlongSpline Stop)
    (:Update
      (CallFunction|Fly _progressalongspline))
    (:Finished
      (if (Variables|Default|GetisLooping)
        (CallFunction|FlyAlongSpline)))))

(event Custom|StopAttack
  (bind _cube (Variables|Default|GetCube))
  (bind _returnvalue (Transformation|GetWorldLocation _cube))
  (Variables|Default|SetisAttacking false)
  (Variables|Default|SetTempLocation _returnvalue)
  (Transformation|SetWorldRotation (Variables|Default|GetCube) (Math|Rotator|FindLookatRotation _returnvalue (Spline|GetLocationatSplinePoint (Variables|Default|GetSpline) 0 "World")) false false)
  (Components|Timeline|SetPlayRate (Variables|Default|GetBackToFlight) (/ 1.0 (Variables|Default|GetBackToFlightSpeed)))
  (bind _lerpprogress (Timeline|BackToFlight PlayFromStart)
    (:Update
      (Transformation|SetWorldLocation (Variables|Default|GetCube) (Math|Vector|Lerp(Vector) (Variables|Default|GetTempLocation) (Spline|GetLocationatSplinePoint (Variables|Default|GetSpline) 0 "World") _lerpprogress) false false))
    (:Finished
      (CallFunction|FlyAlongSpline))))

(event Custom|Activate
  (Rendering|SetVisibility (Variables|Default|GetCube) true false)
  (CallFunction|FlyAlongSpline))

(event EventBeginPlay)

(event Collision|EventActorBeginOverlap
  (params (OtherActor :type Actor%20Object%20Reference)))

(event EventTick
  (params (DeltaSeconds :type Float%20%28single-precision%29))
  (if (Variables|Default|GetisAttacking)
    (CallFunction|Attack)))

(fn ConstructionScript)

(fn Fly
  (params (Percent :type Float%20%28single-precision%29))
  (bind _spline (Variables|Default|GetSpline))
  (bind _returnvalue (Spline|GetSplineLength _spline))
  (bind _returnvalue_2 (* Percent _returnvalue))
  (Transformation|SetWorldLocationAndRotation (Variables|Default|GetCube) (Spline|GetLocationatDistanceAlongSpline _spline _returnvalue_2 "World") (Spline|GetRotationatDistanceAlongSpline _spline _returnvalue_2 "World") false false))

(fn Attack
  (bind _cube (Variables|Default|GetCube))
  (Transformation|SetWorldRotation (Variables|Default|GetCube) (Math|Rotator|FindLookatRotation (Transformation|GetWorldLocation (Variables|Default|GetCube)) (Transformation|GetWorldLocation (Variables|/Script/Engine.Character|GetCapsuleComponent (Game|GetPlayerCharacter 0)))) false false)
  (Transformation|SetWorldLocation (Variables|Default|GetCube) (+ (Transformation|GetWorldLocation _cube) (* (Math|Vector|GetForwardVector _cube) (Variables|Default|GetAttackSpeed))) false false))