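; Carryable bucket that the player can grab, fill with water, splash or throw away.
; Grab disables physics, attaches it to the character's AttachPoint socket and can advance a Day 1 problem in BP_LevelManager.
; Fill shows the water mesh, and Interact either splashes and empties a full bucket or throws an empty one, updating the character's interaction prompt.
; Release detaches it and restores physics.
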(event Custom|Fill
  (bind _character (Variables|Default|GetCharacter))
  (Rendering|SetVisibility (Variables|Default|GetWaterLevel) true false)
  (Variables|Default|SetisFull true)
  (Variables|/Game/Blueprints/Bluperints/BP_Character.BP_Character_C|SetGrabbedInteraction _character "Splash Water")
  (Default|ShowGrabbedInteraction _character))

(event EventBeginPlay
  (bind _asbp_character (Utilities|Casting|CastToBP_Character (Game|GetPlayerCharacter 0)))
  (Variables|Default|SetCharacter _asbp_character))

(event Collision|EventActorBeginOverlap
  (params (OtherActor :type Actor%20Object%20Reference)))

(event EventTick
  (params (DeltaSeconds :type Float%20%28single-precision%29)))

(event EventInteract
  (bind _character (Variables|Default|GetCharacter))
  (if (Variables|Default|GetisGrabbed)
    (if (Variables|Default|GetisFull)
      (Default|Projection (Variables|Default|GetCharacter) "NewEnumerator0")
      (Rendering|SetVisibility (Variables|Default|GetWaterLevel) false false)
      (Variables|Default|SetisFull false)
      (Default|Contraction _character)
      (Variables|/Game/Blueprints/Bluperints/BP_Character.BP_Character_C|SetGrabbedInteraction _character "Throw away")
      (Default|ShowGrabbedInteraction _character)
      (else
        (Default|Throw (Variables|Default|GetCharacter) (Variables|Default|GetBucket))))))

(event EventRelease
  (bind _character (Variables|Default|GetCharacter))
  (Transformation|DetachFromActor "KeepWorld" "KeepWorld" "KeepWorld")
  (Variables|/Game/Blueprints/Bluperints/BP_Character.BP_Character_C|SetCaryObject _character false)
  (Variables|/Game/Blueprints/Bluperints/BP_Character.BP_Character_C|SetCarriedObject _character 0)
  (Physics|SetSimulatePhysics (Variables|Default|GetBucket) true))

(event EventGrab
  (params (Character :type Skeletal%20Mesh%20Component%20Object%20Reference))
  (Transformation|AttachComponentToComponent (Variables|Default|GetBucket) (Variables|Default|GetScene) "None" "SnapToTarget" "SnapToTarget" "KeepWorld" true)
  (Transformation|SetRelativeLocation (Variables|Default|GetBucket) "0, 0,-27.000000" false false)
  (Physics|SetSimulatePhysics (Variables|Default|GetBucket) false)
  (Variables|/Game/Blueprints/Bluperints/BP_Character.BP_Character_C|SetCaryObject (Variables|Default|GetCharacter) true)
  (Variables|/Game/Blueprints/Bluperints/BP_Character.BP_Character_C|SetCarriedObject (Variables|Default|GetCharacter) self)
  (Transformation|AttachComponentToComponent Character "AttachPoint" "SnapToTarget" "SnapToTarget" "KeepWorld" false)
  (Variables|Default|SetisGrabbed true)
  (Variables|/Game/Blueprints/Bluperints/BP_Character.BP_Character_C|SetGrabbedInteraction (Variables|Default|GetCharacter) "Throw away")
  (Default|ShowGrabbedInteraction (Variables|Default|GetCharacter))
  ;[1 1 1] Resolution of the 6th problem of Day 1
  (bind _outactors (Actor|GetAllActorsOfClass "/Game/Blueprints/Bluperints/BP_LevelManager.BP_LevelManager_C"))
  (if (and (== (Variables|/Game/Blueprints/Bluperints/BP_LevelManager.BP_LevelManager_C|GetCurrentDay (Utilities|Array|Get(acopy) _outactors)) 1) (== (Variables|/Game/Blueprints/Bluperints/BP_LevelManager.BP_LevelManager_C|GetCurrentProblem (Utilities|Array|Get(acopy) _outactors)) 8))
    (Default|ProblemResolution (Utilities|Array|Get(acopy) _outactors) 9 0.0)))

(event EventShowGrabInteraction
  (Default|ChangeGrabHUD (Variables|Default|GetCharacter) "Grab the bucket" true))

(fn ConstructionScript)